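; Cash-out objective that runs a timed extraction point, reporting to GameState when it finishes.
; Server Tick holds the destroy timer near one second while busy, ends extraction once TotalBanked equals RoundCashValue, and flags busy from the occupant map.
; Clients swap the cone material from the busy state.
; Overlap, targeting, interaction and team banking logic is disconnected, so those events and StartExtractionFunction do nothing.
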(event OnComponentBeginOverlap(Box)
  (params (OverlappedComponent :type Primitive%20Component%20Object%20Reference) (OtherActor :type Actor%20Object%20Reference) (OtherComp :type Primitive%20Component%20Object%20Reference) (OtherBodyIndex :type Integer) (bFromSweep :type Boolean) (SweepResult :type Hit%20Result%20Structure%20%28by%20ref%29))
  ;[0.15 0.15 0.15 0.5] Add Character To List When Overlap
)

(event OnComponentEndOverlap(Box)
  (params (OverlappedComponent :type Primitive%20Component%20Object%20Reference) (OtherActor :type Actor%20Object%20Reference) (OtherComp :type Primitive%20Component%20Object%20Reference) (OtherBodyIndex :type Integer))
  ;[0.15 0.15 0.15 0.5] Remove Character To List When End Of Overlap
)

(event Custom|SetTimer
  (params (TimeBeforeEnd :type Float%20%28double-precision%29))
  ;[0.15 0.15 0.15 0.5] Destroying Timer
  (bind _returnvalue (Utilities|Time|SetTimerbyEvent (delegate Custom|DestroyExtraction) TimeBeforeEnd))
  (Variables|Default|SetDestroyTimerHandle _returnvalue))

(event Custom|DestroyExtraction
  ;[0.15 0.15 0.15 0.5] Destroying Timer
  (Default|CallFinishedExtraction (Variables|Default|GetGameState)))

(event Custom|FinishCashOut
  (params (Player :type BP%20First%20Person%20Character%20Object%20Reference))
  ;[0.15 0.15 0.15 0.5] Finished
  (CallFunction|StartExtractionFunction Player))

(event EventOnInteract
  (params (InteractingActor :type Actor%20Object%20Reference))
  ;[0.15 0.15 0.15 0.5] Start Extraction On Player
)

(event EventOnUntarget
  (params (TargetingActor :type Actor%20Object%20Reference))
  ;[0.15 0.15 0.15 0.5] Stop Looking
)

(event EventOnTarget
  (params (TargetingActor :type Actor%20Object%20Reference)))

(event EventTick
  (params (DeltaSeconds :type Float%20%28single-precision%29))
  ;[0.15 0.15 0.15 0.5] Logic For Adding Point Each Tick
  (Networking|SwitchHasAuthority
    (:Authority
      (bind _output_get (Variables|Default|SetTimeRemaining (Utilities|Time|GetTimerRemainingTimebyHandle (Variables|Default|GetDestroyTimerHandle))))
      (if (Math|Float|NearlyEqual(Float) _output_get 1.0 1e-06)
        (if (Variables|Default|GetBusyRn)
          (Utilities|Time|PauseTimerbyHandle (Variables|Default|GetDestroyTimerHandle))))
      (Networking|SwitchHasAuthority
        (:Authority
          (if (== (Variables|Default|GetRoundCashValue) (Variables|Default|GetTotalBanked))
            (Utilities|Time|ClearandInvalidateTimerbyHandle (Variables|Default|GetDestroyTimerHandle))
            (CallFunction|DestroyExtraction)
            (else
              (Networking|SwitchHasAuthority
                (:Authority
                  (bind _valuepin (Utilities|Map|ForEachLoop(Map) (Variables|Default|GetCharacterCurrentlyIn%20))
                    (:then
                      (if _valuepin
                        (Variables|Default|SetBusyRn true)))))))))))
    (:Remote
      (Variables|Default|GetBusyRn
        (:then
          (Rendering|Material|SetMaterial (Variables|Default|GetCone) 0 "/Game/Art/Materials/Inst/Blue_Inst.Blue_Inst"))
        (:else
          (Rendering|Material|SetMaterial (Variables|Default|GetCone) 0 "/Engine/BasicShapes/BasicShapeMaterial.BasicShapeMaterial"))))))

(fn ConstructionScript)

(fn StartExtractionFunction
  (params (Player :type BP%20First%20Person%20Character%20Object%20Reference)))