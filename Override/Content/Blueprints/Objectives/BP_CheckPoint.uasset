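; BP_CheckPoint is a replicated brazier checkpoint lit by a team's torch or flag carrier.
; On the server, overlap while enabled and unlit reports to BP_GameState and multicasts the flame effect.
; Clients tint flames relative to the local player's team and unpause FMOD ambience.
; RepNotifies drive the ping and visibility, with hiding resetting effects; ResetCheckpoint disables and hides it after a delay.
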(event OnComponentBeginOverlap(Box)
  (params (OverlappedComponent :type Primitive%20Component%20Object%20Reference) (OtherActor :type Actor%20Object%20Reference) (OtherComp :type Primitive%20Component%20Object%20Reference) (OtherBodyIndex :type Integer) (bFromSweep :type Boolean) (SweepResult :type Hit%20Result%20Structure%20%28by%20ref%29))
  (Networking|SwitchHasAuthority
    (:Authority
      (if (and (Variables|Default|GetEnable%20) (not (Variables|Default|GetLightUp)))
        (bind _asbp_torch (Utilities|Casting|CastToBP_Torch OtherActor)
          (:then
            (bind _flagcarrier (Variables|/Game/Blueprints/Objectives/BP_Torch.BP_Torch_C|GetFlagCarrier _asbp_torch)
              (:then
                (Variables|Default|SetLightUp true)
                (Variables|Default|SetAs%20BP%20First%20Person%20Character _flagcarrier)
                (bind _asbp_game_state (Utilities|Casting|CastToBP_GameState (Game|GetGameState)))
                (Default|CallCheckpointReached _asbp_game_state (Variables|/Game/Blueprints/Objectives/BP_Torch.BP_Torch_C|GetTeam%20Index _asbp_torch) (Variables|Default|GetAs%20BP%20First%20Person%20Character))
                (CallFunction|MultiCastBrasseroVFX (Variables|/Game/Blueprints/Objectives/BP_Torch.BP_Torch_C|GetTeam%20Index _asbp_torch)))
              (:else)))
          (:CastFailed
            (bind _asbp_first_person_character (Utilities|Casting|CastToBP_FirstPersonCharacter OtherActor))
            (Variables|/Game/Blueprints/Player/BP_FirstPersonCharacter.BP_FirstPersonCharacter_C|GetHasFlag _asbp_first_person_character
              (:then
                (Variables|Default|SetLightUp true)
                (Variables|Default|SetAs%20BP%20First%20Person%20Character _asbp_first_person_character)
                (bind _asbp_game_state_2 (Utilities|Casting|CastToBP_GameState (Game|GetGameState)))
                (Default|CallCheckpointReached _asbp_game_state_2 (Variables|/Game/Blueprints/Objectives/BP_Torch.BP_Torch_C|GetTeam%20Index (Variables|/Game/Blueprints/Player/BP_FirstPersonCharacter.BP_FirstPersonCharacter_C|GetFlag _asbp_first_person_character)) (Variables|Default|GetAs%20BP%20First%20Person%20Character))
                (CallFunction|MultiCastBrasseroVFX (Variables|/Game/Blueprints/Objectives/BP_Torch.BP_Torch_C|GetTeam%20Index (Variables|/Game/Blueprints/Player/BP_FirstPersonCharacter.BP_FirstPersonCharacter_C|GetFlag _asbp_first_person_character))))
              (:else))))))))

(event Custom|ResetVFX
  (bind _niagara (Variables|Default|GetNiagara))
  (Niagara|SetNiagaraVariable(Float) (Variables|Default|Getping) "PingOpacity" 0.0)
  (Niagara|SetNiagaraVariable(Float) _niagara "ColorID" 0.0)
  (Components|Activation|SetActive _niagara false true)
  ;[0.15 1 0.15 0.5] SFX Pause Ambience on Reset
  (Networking|SwitchHasAuthority
    (:Remote
      (Utilities|IsValid (Variables|Default|GetFMODSoundPoint)
        (:Is%20Valid
          _)
        (:Is%20Not%20Valid
          (bind _returnvalue (Class|FMODBlueprintStatics|PlayEventAttached "/Game/FMOD/Events/SFX_FOLDER/AMBIENCE/SoundPoint/Brazier.Brazier" (Variables|Default|GetPlane) "None" "0, 0, 0" "KeepRelativeOffset"))
          (bind _output_get (Variables|Default|SetFMODSoundPoint _returnvalue))))
      (Class|FMODAudioComponent|SetPaused _output_get true))))

(event Custom|ResetCheckpoint
  (Utilities|FlowControl|Delay 3.0)
  (Variables|Default|SetLightUp false)
  (Variables|Default|SetEnable%20 false)
  (CallFunction|SetVisible false))

(event Custom|MultiCast_BrasseroVFX
  (params (Team :type Integer))
  (Networking|SwitchHasAuthority
    (:Remote
      (Niagara|SetNiagaraVariable(Float) (Variables|Default|GetNiagara) "ColorID" (Utilities|Select :Index (Variables|/Game/Blueprints/Controller/BP_FirstPersonPlayerController.BP_FirstPersonPlayerController_C|GetTeamIndex (.AsBP%20First%20Person%20Player%20Controller (Utilities|Casting|CastToBP_FirstPersonPlayerController (Game|GetPlayerController 0)))) :Option%200 (Utilities|Select :Index Team :Option%200 1.0 :Option%201 2.0 :Option%202 3.0) :Option%201 (Utilities|Select :Index Team :Option%200 2.0 :Option%201 1.0 :Option%202 3.0) :Option%202 (Utilities|Select :Index Team :Option%200 2.0 :Option%201 3.0 :Option%202 1.0)))
      (Niagara|SetNiagaraVariable(Float) (Variables|Default|Getping) "PingOpacity" 0.0)
      (Components|Activation|SetActive (Variables|Default|GetNiagara) true true)
      ;[0.15 1 0.15 0.5] SFX Unpause Ambience
      (Class|FMODAudioComponent|SetPaused (Variables|Default|GetFMODSoundPoint) false))))

(event EventBeginPlay
  (Variables|Default|SetVisible false))

(fn ConstructionScript)

(fn OnRepVisible
  (Rendering|SetActorHiddenInGame (not (Variables|Default|GetVisible)))
  (if (not (Variables|Default|GetVisible))
    (CallFunction|ResetVFX)))

(fn SetVisible
  (params (Visible :type Boolean))
  (Variables|Default|SetVisible Visible)
  (Networking|ForceNetUpdate))

(fn OnRepEnable
  (Niagara|SetNiagaraVariable(Float) (Variables|Default|Getping) "PingOpacity" 1.0))