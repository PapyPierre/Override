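; Flag extraction point that starts for a possessing team, destroys the other point and awards points when its timer expires uncontested.
; Box overlaps maintain a player-to-team map, from which SetBooleanCheck derives ally, contest and duo flags.
; Server Tick uses those flags to scale extraction and steal timers: pairs speed them up, defenders freeze stealing, and completed steals transfer ownership.
; Older per-second data-scoring logic and debug prints remain as leftovers.
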(event OnComponentBeginOverlap(Box2)
  (params (OverlappedComponent :type Primitive%20Component%20Object%20Reference) (OtherActor :type Actor%20Object%20Reference) (OtherComp :type Primitive%20Component%20Object%20Reference) (OtherBodyIndex :type Integer) (bFromSweep :type Boolean) (SweepResult :type Hit%20Result%20Structure%20%28by%20ref%29))
  (bind _asbp_first_person_character (Utilities|Casting|CastToBP_FirstPersonCharacter OtherActor))
  ;[0.15 0.15 0.15 0.5] Add Character To List When Overlap
  (if (== (Utilities|GetClass OtherActor) "/Game/Blueprints/Player/BP_FirstPersonCharacter.BP_FirstPersonCharacter_C")
    (Utilities|Map|Add (Variables|Default|GetTeamAndPlayer) _asbp_first_person_character (Variables|/Game/Blueprints/Player/BP_FirstPersonCharacter.BP_FirstPersonCharacter_C|GetTeamIndex _asbp_first_person_character))
    (CallFunction|SetBooleanCheck _asbp_first_person_character true)))

(event Custom|ReceiveInfo
  (params (Character :type BP%20First%20Person%20Character%20Object%20Reference) (TeamIndex :type Integer))
  (Variables|Default|SetTeamIndex TeamIndex)
  (Variables|Default|SetCharacterPossessing Character)
  (CallFunction|StartTimer)
  (CallFunction|SetBooleanCheck Character true)
  (Networking|SwitchHasAuthority
    (:Authority
      (Default|DestroyOtherPoint (Variables|Default|GetGameState) self))))

(event Custom|StartTimer
  (Variables|Default|SetStart true)
  (Variables|Default|SetTime (Variables|Default|GetInitialTime))
  (Variables|Default|SetStealTime (Variables|Default|GetInitialStealTime))
  (Variables|/Script/Engine.PrimitiveComponent|SetbGenerateOverlapEvents (Variables|Default|GetBox2) true)
  (Rendering|SetVisibility (Variables|Default|GetContestZone) true false)
  (Rendering|SetVisibility (Variables|Default|GetFlagDropOut) false false))

(event Custom|Add%20Date%20Per%20Second
  (bind _datapertime (Variables|Default|GetDataPerTime))
  ;[1 0 0 0.5] OLD Again ?
  (for _array_element (Variables|Default|GetCharacterCurrentlyIn%20)
    (bind _output_get (Variables|/Game/Blueprints/Player/BP_FirstPersonCharacter.BP_FirstPersonCharacter_C|SetDataPossesed _array_element (Math|Float|Truncate (+ (Variables|/Game/Blueprints/Player/BP_FirstPersonCharacter.BP_FirstPersonCharacter_C|GetDataPossesed _array_element) _datapertime))))
    (Utilities|IsValid (Variables|/Game/Blueprints/Player/BP_FirstPersonCharacter.BP_FirstPersonCharacter_C|GetTeamMateRef _array_element)
      (:Is%20Valid
        (Default|RPCFeedDataEntry (Variables|/Game/Blueprints/Player/BP_FirstPersonCharacter.BP_FirstPersonCharacter_C|GetTeamMateRef _array_element) "[Ally] Holding point" _datapertime)
        (Variables|/Game/Blueprints/Player/BP_FirstPersonCharacter.BP_FirstPersonCharacter_C|SetDataPossesed (Variables|/Game/Blueprints/Player/BP_FirstPersonCharacter.BP_FirstPersonCharacter_C|GetTeamMateRef _array_element) _output_get))
      (:Is%20Not%20Valid
        _))
    (Variables|Default|SetCurrentData (- (Variables|Default|GetCurrentData) _datapertime))
    (Default|RPCFeedDataEntry _array_element "Holding point" _datapertime)))

(event Custom|ChangeOwnership
  (bind _output_get (Variables|Default|SetTeamIndex (Variables|Default|GetContestingPlayer)))
  (Variables|Default|SetStealTime (Variables|Default|GetInitialStealTime))
  (Variables|Default|SetContestingPlayer -1)
  (Variables|Default|SetContesting false)
  (bind _output_get_2 (Variables|Default|SetCharacterPossessing (Variables|/Game/Blueprints/Controller/BP_FirstPersonPlayerController.BP_FirstPersonPlayerController_C|GetPlayerOwning (Utilities|Array|Get(acopy) (.Player (Utilities|Struct|BreakS_PlayerArray (Utilities|Array|Get(acopy) (Variables|/Game/Blueprints/GameMode/GameState/BP_GameState.BP_GameState_C|GetTeams (Variables|Default|GetGameState)) _output_get)))))))
  (if (<= (Variables|Default|GetTime) 0.0)
    (CallFunction|FinishedExtraction)
    (else
      (CallFunction|SetBooleanCheck _output_get_2 false))))

(event Custom|FinishedExtraction
  (Variables|Default|GetStart
    (:then
      (Default|CallAddPoint (Variables|Default|GetCharacterPossessing) 25 "Flag secured")
      (Variables|Default|SetStart false)
      (Default|CallEmptyDataPoint (Variables|Default|GetGameState))
      (Variables|/Script/Engine.PrimitiveComponent|SetbGenerateOverlapEvents (Variables|Default|GetBox2) false))
    (:else)))

(event Custom|debug
  (Networking|SwitchHasAuthority
    (:Authority
      (Development|PrintString (Utilities|String|ToString(Float) (Variables|Default|GetStealTime)) true true "(R=0.000000,G=0.660000,B=1.000000,A=1.000000)" 2.0 "rafaaf"))))

(event Custom|Old
  (params (DeltaSeconds :type Float%20%28single-precision%29))
  ;[0.15 0.000664 0 0.5] OLD Logic For Adding Point Each Tick
  (Networking|SwitchHasAuthority
    (:Authority
      (if (<= (Variables|Default|GetCurrentData) 0.0)
        (Default|DataPointEmpty (Variables|Default|GetGameState))
        (elif (> (Utilities|Array|Length (Variables|Default|GetCharacterCurrentlyIn%20)) 0)
          (bind _output_get (Variables|Default|SetCurrentData (- (Variables|Default|GetCurrentData) (+ (* DeltaSeconds (Variables|Default|GetDataPerTime)) (Variables|Default|GetScoreAccumulator)))))
          (if (< _output_get 0.0)
            (Variables|Default|SetScoreAccumulator (/ (- (+ (* DeltaSeconds (Variables|Default|GetDataPerTime)) (Variables|Default|GetScoreAccumulator)) (Math|Float|Absolute(Float) _output_get)) (Utilities|Array|Length (Variables|Default|GetCharacterCurrentlyIn%20))))
            (else
              (Variables|Default|SetScoreAccumulator (/ (+ (* DeltaSeconds (Variables|Default|GetDataPerTime)) (Variables|Default|GetScoreAccumulator)) (Utilities|Array|Length (Variables|Default|GetCharacterCurrentlyIn%20))))))
          (for _array_element (Variables|Default|GetCharacterCurrentlyIn%20)
            (bind _output_get_2 (Variables|/Game/Blueprints/Player/BP_FirstPersonCharacter.BP_FirstPersonCharacter_C|SetDataPossesed _array_element (Math|Float|Truncate (* (+ (Variables|Default|GetScoreAccumulator) (Variables|/Game/Blueprints/Player/BP_FirstPersonCharacter.BP_FirstPersonCharacter_C|GetDataPossesed _array_element)) (Variables|Default|GetRoundMultiplier)))))
            (Variables|/Game/Blueprints/Player/BP_FirstPersonCharacter.BP_FirstPersonCharacter_C|SetDataPossesed (Variables|/Game/Blueprints/Player/BP_FirstPersonCharacter.BP_FirstPersonCharacter_C|GetTeamMateRef _array_element) _output_get_2))
          (Variables|Default|SetScoreAccumulator 0.0))))))

(event EventBeginPlay
  (bind _asbp_game_state (Utilities|Casting|CastToBP_GameState (Game|GetGameState)))
  (Variables|Default|SetGameState _asbp_game_state))

(event EventTick
  (params (DeltaSeconds :type Float%20%28single-precision%29))
  (Networking|SwitchHasAuthority
    (:Authority
      (CallFunction|SetTimerMultiplicator)
      (Variables|Default|GetStart
        (:then
          (Variables|Default|GetContesting
            (:then
              (Variables|Default|SetStealTime (- (Variables|Default|GetStealTime) (* DeltaSeconds (Variables|Default|GetTimerMultiplicatorSteal))))
              (if (<= (Variables|Default|GetStealTime) 0.0)
                (CallFunction|ChangeOwnership)))
            (:else
              _))
          (Variables|Default|SetTime (- (Variables|Default|GetTime) (* DeltaSeconds (Variables|Default|GetTimerMultiplicator))))
          (CallFunction|Debug)
          (if (Math|Boolean|ANDBoolean (== (Variables|Default|GetContesting) false) (== (Variables|Default|GetStealTime) (Variables|Default|GetInitialStealTime)) (<= (Variables|Default|GetTime) 0.0))
            (CallFunction|FinishedExtraction)))
        (:else)))))

(event Collision|EventActorEndOverlap
  (params (OtherActor :type Actor%20Object%20Reference))
  (bind _asbp_first_person_character (Utilities|Casting|CastToBP_FirstPersonCharacter OtherActor))
  ;[0.15 0.15 0.15 0.5] Remove Character To List When End Of Overlap
  (if (== (Utilities|GetClass OtherActor) "/Game/Blueprints/Player/BP_FirstPersonCharacter.BP_FirstPersonCharacter_C")
    (Utilities|Map|Remove (Variables|Default|GetTeamAndPlayer) _asbp_first_person_character)
    (CallFunction|SetBooleanCheck _asbp_first_person_character false)))

(fn ConstructionScript)

(fn SetTimerMultiplicator
  (Variables|Default|GetContesting
    (:then
      (Variables|Default|GetNoAllies
        (:then
          (Variables|Default|GetDuoContesting
            (:then
              (Variables|Default|SetTimerMultiplicatorSteal 2.0))
            (:else
              (Variables|Default|SetTimerMultiplicatorSteal 1.0))))
        (:else
          (Variables|Default|SetTimerMultiplicatorSteal 0.0))))
    (:else
      (Variables|Default|GetAllyInZone
        (:then
          (Variables|Default|SetTimerMultiplicator 2.0))
        (:else
          (Variables|Default|SetTimerMultiplicator 1.0))))))

(fn SetBooleanCheck
  (params (Player :type BP%20First%20Person%20Character%20Object%20Reference) (Add :type Boolean))
  (if (!= (Variables|Default|GetTeamIndex) -1)
    (LocalVariables|GetAdd
      (:then
        _)
      (:else
        (if (and (== (Variables|/Game/Blueprints/Player/BP_FirstPersonCharacter.BP_FirstPersonCharacter_C|GetTeamIndex Player) (Variables|Default|GetContestingPlayer)) (== (.ReturnValue (Utilities|Map|Find (Variables|Default|GetTeamAndPlayer) (Variables|/Game/Blueprints/Player/BP_FirstPersonCharacter.BP_FirstPersonCharacter_C|GetTeamMateRef Player))) false))
          (Variables|Default|SetContesting false))))
    (bind (_keypin _valuepin) (Utilities|Map|ForEachLoop(Map) (Variables|Default|GetTeamAndPlayer))
      (:then
        (if (== _valuepin (Variables|Default|GetTeamIndex))
          (bind _result (Math|Integer|IncrementInt (LocalVariables|GetNumberOfAllies))
            (:%20%20
              (if (>= _result 2)
                (Variables|Default|SetAllyInZone true)
                (else
                  (Variables|Default|SetAllyInZone false)))))
          (else
            (bind _result_2 (Math|Integer|IncrementInt (LocalVariables|GetNumberOfEnemies))
              (:%20%20
                (Variables|Default|GetContesting
                  (:then
                    _)
                  (:else
                    (Variables|Default|SetContestingPlayer (Variables|/Game/Blueprints/Player/BP_FirstPersonCharacter.BP_FirstPersonCharacter_C|GetTeamIndex (select Add Player _keypin)))
                    (Variables|Default|SetContesting true)))
                (if (>= _result_2 2)
                  (if (== _valuepin (Variables|Default|GetContestingPlayer))
                    (Variables|Default|SetDuoContesting true)
                    (Variables|Default|SetMutlipleTeam false)
                    (else
                      (Variables|Default|SetMutlipleTeam true)
                      (Variables|Default|SetDuoContesting false)))
                  (else
                    (Variables|Default|SetDuoContesting false)
                    (Variables|Default|SetMutlipleTeam false))))))))
      (:CompletedPin
        (if (== (LocalVariables|GetNumberOfEnemies) 0)
          (Variables|Default|SetContesting false)
          (Variables|Default|SetStealTime (Variables|Default|GetInitialStealTime))
          (Variables|Default|SetContestingPlayer -1))
        (if (== (LocalVariables|GetNumberOfAllies) 0)
          (Variables|Default|SetNoAllies true)
          (else
            (Variables|Default|SetNoAllies false)))
        (return)))
    (else
      (return))))