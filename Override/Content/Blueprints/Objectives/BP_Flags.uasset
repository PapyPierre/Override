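; BP_Flags is a carryable objective flag whose server-side sphere overlap handles pickup and planting.
; A free flag records the carrier and team, disables their shooting, hides weapons, awards points on first pickup and notifies the GameState.
; Overlapping a checkpoint passes carrier and team to the collect point, awards points and expires the flag.
; Separate events release it or launch it from the weapon socket with physics.
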(event OnComponentBeginOverlap(Sphere)
  (params (OverlappedComponent :type Primitive%20Component%20Object%20Reference) (OtherActor :type Actor%20Object%20Reference) (OtherComp :type Primitive%20Component%20Object%20Reference) (OtherBodyIndex :type Integer) (bFromSweep :type Boolean) (SweepResult :type Hit%20Result%20Structure%20%28by%20ref%29))
  (Networking|SwitchHasAuthority
    (:Authority
      (bind _asbp_first_person_character (Utilities|Casting|CastToBP_FirstPersonCharacter OtherActor)
        (:then
          (Variables|Default|GetFree
            (:then
              (Variables|Default|GetFirst
                (:then
                  (Default|CallAddPoint _asbp_first_person_character 5 "Flag taken"))
                (:else
                  _))
              (bind _output_get (Variables|Default|SetCharacter _asbp_first_person_character))
              (CallFunction|DisableShooting _output_get)
              (Variables|Default|SetFree false)
              (Variables|Default|SetTeam%20Index (Variables|/Game/Blueprints/Player/BP_FirstPersonCharacter.BP_FirstPersonCharacter_C|GetTeamIndex _asbp_first_person_character))
              (Variables|Default|SetFirst false)
              (Default|FlagPPM _asbp_first_person_character (Variables|Default|GetCharacter) true)
              (Default|RPCFlagAnimation (Variables|Default|GetCharacter) true)
              (Default|CallFinishedExtraction (Variables|Default|GetGameState))
              (Variables|/Game/Blueprints/Player/BP_FirstPersonCharacter.BP_FirstPersonCharacter_C|SetFlag (Variables|Default|GetCharacter) self))
            (:else)))
        (:CastFailed
          (if (== (Utilities|GetClass OtherActor) "/Game/Blueprints/Objectives/BP_CheckPoint.BP_CheckPoint_C")
            (bind _asbp_collect_point (Utilities|Casting|CastToBP_CollectPoint OtherActor))
            (Default|ReceiveInfo _asbp_collect_point (Variables|Default|GetCharacter) (Variables|Default|GetTeam%20Index))
            (Default|CallAddPoint (Variables|Default|GetCharacter) 10 "Flag plant")
            (Networking|SwitchHasAuthority
              (:Authority
                (Default|RPCFlagAnimation (Variables|Default|GetCharacter) false)
                (Actor|SetLifeSpan 0.2)
                (Variables|/Script/Engine.PrimitiveComponent|SetbGenerateOverlapEvents (Variables|Default|GetSphere) false)))))))))

(event Custom|RPC_LaunchFlag
  (Transformation|SetActorTransform (Transformation|GetBoneTransform (Variables|/Game/Blueprints/Player/BP_FirstPersonCharacter.BP_FirstPersonCharacter_C|GetFPSMesh (Variables|Default|GetCharacter)) "Weapon_Socket" "RTS_World"))
  (Physics|SetSimulatePhysics (Variables|Default|GetCylinder) true))

(event Custom|StopFlag
  (bind _character (Variables|Default|GetCharacter))
  (Variables|Default|SetFree true)
  (Variables|Default|SetTeam%20Index -1)
  (Default|RPCFlagAnimation _character false)
  (Variables|/Game/Blueprints/Player/BP_FirstPersonCharacter.BP_FirstPersonCharacter_C|SetFlag _character 0))

(event Custom|DisableShooting
  (params (Character :type BP%20First%20Person%20Character%20Object%20Reference))
  (Variables|/Game/Blueprints/Component/AC_Weapon.AC_Weapon_C|SetCanShoot (Variables|/Game/Blueprints/Player/BP_FirstPersonCharacter.BP_FirstPersonCharacter_C|GetAC_WeaponComponent Character) false)
  (Rendering|SetVisibility (Variables|/Game/Blueprints/Player/BP_FirstPersonCharacter.BP_FirstPersonCharacter_C|GetTPSWeapon Character) false false)
  (Rendering|SetVisibility (Variables|/Game/Blueprints/Player/BP_FirstPersonCharacter.BP_FirstPersonCharacter_C|GetFPSWeapon Character) false false)
  (Development|PrintString "Hello"))

(fn ConstructionScript)