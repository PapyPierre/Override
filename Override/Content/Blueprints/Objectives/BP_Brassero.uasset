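; BP_Brassero is a brazier checkpoint that a team lights by bringing a torch to it.
; The server checks box overlaps on begin and Tick, confirms line of sight by raycast, then notifies GameState.
; A multicast plays team-colored Niagara relative to the local team, HUD announcements and FMOD ambience.
; Clients drive a crowd build-up FMOD parameter from player distance, while RepNotifies handle visibility, reset and ping.
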(event OnComponentBeginOverlap(Box)
  (params (OverlappedComponent :type Primitive%20Component%20Object%20Reference) (OtherActor :type Actor%20Object%20Reference) (OtherComp :type Primitive%20Component%20Object%20Reference) (OtherBodyIndex :type Integer) (bFromSweep :type Boolean) (SweepResult :type Hit%20Result%20Structure%20%28by%20ref%29))
  (CallFunction|ManualCheck OtherActor))

(event Custom|ResetVFX
  (bind _niagara (Variables|Default|GetNiagara))
  (bind _durationafterbuildup (Variables|Default|GetDurationAfterBuildUp))
  (bind _returnvalue (/ _durationafterbuildup 2.0))
  (Niagara|SetNiagaraVariable(Float) (Variables|Default|Getping) "PingOpacity" 0.0)
  (Niagara|SetNiagaraVariable(Float) _niagara "ColorID" 0.0)
  (Components|Activation|SetActive _niagara false true)
  ;[0.15 1 0.15 0.5] SFX Pause Ambience on Reset
  (Networking|SwitchHasAuthority
    (:Remote
      (Utilities|IsValid (Variables|Default|GetFMODSoundPoint)
        (:Is%20Valid
          (Utilities|FlowControl|Sequence
            (:then_0
              (Class|FMODAudioComponent|SetPaused (stale _output_get) true :!label _label)
              (Variables|Default|SetLightUp false))
            (:then_1
              ;[0.15 1 0.15 0.5] EaseOut Crowd SFX BuildUp on last Brazier
              (Utilities|FlowControl|Delay _returnvalue)
              (Components|Timeline|SetPlayRate (Variables|Default|GetEaseOut) (/ 1.0 _returnvalue))
              (bind _alpha (Timeline|EaseOut PlayFromStart)
                (:Update
                  (Class|FMODBlueprintStatics|SetGlobalParameterbyName "DistanceFromBrazier" _alpha))
                (:Finished
                  (Variables|Default|SetBuildUpValue 0.0))))))
        (:Is%20Not%20Valid
          (bind _returnvalue_2 (Class|FMODBlueprintStatics|PlayEventAttached "/Game/FMOD/Events/SFX_FOLDER/AMBIENCE/SoundPoint/SP_Brazier.SP_Brazier" (Variables|Default|GetPlane) "None" "0, 0, 0" "KeepRelativeOffset"))
          (bind _output_get (Variables|Default|SetFMODSoundPoint _returnvalue_2))
          (goto _label))))))

(event Custom|ResetCheckpoint
  (params (Duration :type Float%20%28single-precision%29))
  (Utilities|FlowControl|Delay Duration)
  (Variables|Default|SetLightUp false)
  (Variables|Default|SetEnable%20 false)
  (CallFunction|SetVisible false))

(event Custom|MultiCast_BrasseroVFX
  (params (Team :type Integer))
  (bind _returnvalue (Game|GetPlayerController 0))
  (bind _returnvalue_2 (Utilities|Select :Index Team :Option%200 2.0 :Option%201 3.0 :Option%202 1.0))
  (bind _returnvalue_3 (Utilities|Select :Index Team :Option%200 1.0 :Option%201 2.0 :Option%202 3.0))
  (bind _returnvalue_4 (Utilities|Select :Index Team :Option%200 2.0 :Option%201 1.0 :Option%202 3.0))
  (bind _asbp_first_person_player_controller (Utilities|Casting|CastToBP_FirstPersonPlayerController _returnvalue))
  (bind _teamindex (Variables|/Game/Blueprints/Controller/BP_FirstPersonPlayerController.BP_FirstPersonPlayerController_C|GetTeamIndex _asbp_first_person_player_controller))
  (bind _returnvalue_5 (Utilities|Select :Index _teamindex :Option%200 _returnvalue_3 :Option%201 _returnvalue_4 :Option%202 _returnvalue_2))
  (Networking|SwitchHasAuthority
    (:Remote
      (Niagara|SetNiagaraVariable(Float) (Variables|Default|GetNiagara) "ColorID" _returnvalue_5)
      (bind _returnvalue_6 (Utilities|GetDataTableRow "/Game/Data/DataTable/DT_Teams.DT_Teams" (Utilities|String|StringToName (Utilities|String|ToString(Integer) (Math|Float|Truncate _returnvalue_5))))
        (:then
          (bind _asbp_first_person_player_controller_2 (Utilities|Casting|CastToBP_FirstPersonPlayerController (Game|GetPlayerController 0)))
          (Default|MessageSpawn (Variables|/Game/Blueprints/Widget/WBP_HUD.WBP_HUD_C|GetWBP_EventAnnoucement (Variables|/Game/Blueprints/Controller/BP_FirstPersonPlayerController.BP_FirstPersonPlayerController_C|GetHUD _asbp_first_person_player_controller_2)) (Utilities|Text|ToText(String) (Utilities|String|Append "Team " (Utilities|String|ToString(Integer) Team) " Scored !")) (Utilities|Struct|BreakS_Teams _returnvalue_6))
          (Default|ScoreChange (Utilities|Array|Get(acopy) (Variables|/Game/Blueprints/Widget/HUD/WBP_TeamsScore.WBP_TeamsScore_C|GetArrayTeamUI (Variables|/Game/Blueprints/Widget/WBP_HUD.WBP_HUD_C|GetWBP_TeamsScore (Variables|/Game/Blueprints/Controller/BP_FirstPersonPlayerController.BP_FirstPersonPlayerController_C|GetHUD _asbp_first_person_player_controller_2))) Team) (Utilities|Struct|BreakS_Teams _returnvalue_6))
          (Components|Activation|SetActive (Variables|Default|GetNiagara) true true)
          (Niagara|SetNiagaraVariable(Float) (Variables|Default|Getping) "PingOpacity" 0.0)
          ;[0.15 1 0.15 0.5] SFX Unpause Ambience
          (Class|FMODAudioComponent|SetPaused (Variables|Default|GetFMODSoundPoint) false)
          ;[0.15 1 0.15 0.5] Buffer on GameState before taking distance from next Brazier
          (bind _asbp_game_state (Utilities|Casting|CastToBP_GameState (Game|GetGameState)))
          (Variables|/Game/Blueprints/GameMode/GameState/BP_GameState.BP_GameState_C|SetBrazierHasBeenLit _asbp_game_state true)
          (Variables|Default|SetLightUp true)
          (Utilities|FlowControl|Delay (Variables|Default|GetDurationAfterBuildUp))
          (Variables|/Game/Blueprints/GameMode/GameState/BP_GameState.BP_GameState_C|SetBrazierHasBeenLit _asbp_game_state false))))))

(event Custom|ManualCheck
  (params (InputPin :type Object%20Object%20Reference))
  (Networking|SwitchHasAuthority
    (:Authority
      (if (and (Variables|Default|GetEnable%20) (not (Variables|Default|GetLightUp)))
        (bind _asbp_torch (Utilities|Casting|CastToBP_Torch InputPin)
          (:then
            (bind _flagcarrier (Variables|/Game/Blueprints/Objectives/BP_Torch.BP_Torch_C|GetFlagCarrier _asbp_torch)
              (:then
                (bind _output_get (Variables|Default|SetAs%20BP%20First%20Person%20Character _flagcarrier))
                (bind _confirm (CallFunction|RaycastConfirm self _asbp_torch _output_get))
                (if _confirm
                  (Default|ClientBrasseroPPIEffect _output_get)
                  (Variables|/Game/Blueprints/Objectives/BP_Torch.BP_Torch_C|GetThroughWall _asbp_torch
                    (:then)
                    (:else
                      (Variables|Default|SetLightUp true)
                      (CallFunction|MultiCastBrasseroVFX (Variables|/Game/Blueprints/Objectives/BP_Torch.BP_Torch_C|GetTeam%20Index _asbp_torch))
                      (bind _asbp_game_state (Utilities|Casting|CastToBP_GameState (Game|GetGameState)))
                      (Default|CallCheckpointReached _asbp_game_state (Variables|/Game/Blueprints/Objectives/BP_Torch.BP_Torch_C|GetTeam%20Index _asbp_torch) (Variables|Default|GetAs%20BP%20First%20Person%20Character))))))
              (:else)))
          (:CastFailed
            (bind _asbp_first_person_character (Utilities|Casting|CastToBP_FirstPersonCharacter InputPin))
            (Variables|/Game/Blueprints/Player/BP_FirstPersonCharacter.BP_FirstPersonCharacter_C|GetHasTorch _asbp_first_person_character
              (:then
                (bind _output_get_2 (Variables|Default|SetAs%20BP%20First%20Person%20Character _asbp_first_person_character))
                (bind _confirm_2 (CallFunction|RaycastConfirm _output_get_2 self (Variables|/Game/Blueprints/Player/BP_FirstPersonCharacter.BP_FirstPersonCharacter_C|GetFlag _asbp_first_person_character)))
                (if _confirm_2
                  (Default|ClientBrasseroPPIEffect _output_get_2)
                  (Variables|Default|SetLightUp true)
                  (CallFunction|MultiCastBrasseroVFX (Variables|/Game/Blueprints/Objectives/BP_Torch.BP_Torch_C|GetTeam%20Index (Variables|/Game/Blueprints/Player/BP_FirstPersonCharacter.BP_FirstPersonCharacter_C|GetFlag _asbp_first_person_character)))
                  (bind _asbp_game_state_2 (Utilities|Casting|CastToBP_GameState (Game|GetGameState)))
                  (Default|CallCheckpointReached _asbp_game_state_2 (Variables|/Game/Blueprints/Objectives/BP_Torch.BP_Torch_C|GetTeam%20Index (Variables|/Game/Blueprints/Player/BP_FirstPersonCharacter.BP_FirstPersonCharacter_C|GetFlag _asbp_first_person_character)) (Variables|Default|GetAs%20BP%20First%20Person%20Character))))
              (:else))))))))

(event EventBeginPlay
  (Variables|Default|SetVisible false))

(event EventTick
  (params (DeltaSeconds :type Float%20%28single-precision%29))
  (bind _returnvalue (Transformation|GetActorLocation))
  (bind _returnvalue_2 (Game|GetPlayerCharacter 0))
  (bind _distformaxbuildup (Variables|Default|GetDistForMaxBuildUp))
  (bind _distforminbuildup (Variables|Default|GetDistForMinBuildUp))
  (bind _box (Variables|Default|GetBox))
  (bind _returnvalue_3 (Transformation|GetActorLocation _returnvalue_2))
  (bind _overlappingactors (Collision|GetOverlappingActors _box 0 :!class /Script/Engine.PrimitiveComponent))
  (bind _returnvalue_4 (- _distforminbuildup _distformaxbuildup))
  (bind _returnvalue_5 (- _returnvalue_3 _returnvalue))
  (bind _returnvalue_6 (Math|Vector|VectorLength _returnvalue_5))
  (bind _returnvalue_7 (- _returnvalue_6 _distformaxbuildup))
  (bind _returnvalue_8 (/ _returnvalue_7 _returnvalue_4))
  (bind _returnvalue_9 (- 1.0 _returnvalue_8))
  (bind _returnvalue_10 (Math|Float|Clamp(Float) _returnvalue_9))
  (Utilities|FlowControl|Sequence
    (:then_0
      ;[0.15 1 0.15 0.5] Crowd SFX BuildUp with Brazier proximity
      (Networking|SwitchHasAuthority
        (:Remote
          (bind _asbp_game_state (Utilities|Casting|CastToBP_GameState (Game|GetGameState)))
          (if (Variables|/Game/Blueprints/GameMode/GameState/BP_GameState.BP_GameState_C|GetBrazierHasBeenLit _asbp_game_state)
            ;;[0 0 0 0.5] Register Current Value if not the FirstBrazier
            (Utilities|FlowControl|DoOnce false :!label _label
              (:Completed
                (bind _finalvalue (Class|FMODBlueprintStatics|GetGlobalParameterValuebyName "DistanceFromBrazier"))
                (Variables|Default|SetBuildUpValue _finalvalue)))
            (else
              (Utilities|FlowControl|Sequence
                (:then_0
                  (if (and (Variables|Default|GetEnable%20) (not (Variables|Default|GetLightUp)))
                    (bind _output_get (Variables|Default|SetBuildUpValue (select (> (Variables|Default|GetBuildUpValue) _returnvalue_10) (Math|Interpolation|FInterptoConstant (Variables|Default|GetBuildUpValue) _returnvalue_10 DeltaSeconds (Variables|Default|GetDecreaseInterpSpeed)) _returnvalue_10)))
                    (Class|FMODBlueprintStatics|SetGlobalParameterbyName "DistanceFromBrazier" _output_get)))
                (:then_1
                  (goto _label Reset))))))))
    (:then_1
      (if (and (Variables|Default|GetEnable%20) (not (Variables|Default|GetLightUp)))
        (if (Utilities|Array|IsNotEmpty _overlappingactors)
          (for _array_element _overlappingactors
            (CallFunction|ManualCheck _array_element)))))))

(fn ConstructionScript)

(fn OnRepVisible
  (Rendering|SetActorHiddenInGame (not (Variables|Default|GetVisible)))
  (if (not (Variables|Default|GetVisible))
    (CallFunction|ResetVFX)))

(fn SetVisible
  (params (Visible :type Boolean))
  (Variables|Default|SetVisible Visible)
  (Networking|ForceNetUpdate))

(fn OnRepEnable
  (Niagara|SetNiagaraVariable(Float) (Variables|Default|Getping) "PingOpacity" 1.0))

(fn RaycastConfirm
  (params (Actor1 :type Actor%20Object%20Reference) (Actor2 :type Actor%20Object%20Reference) (Actor3? :type Actor%20Object%20Reference))
  (bind _returnvalue (Collision|LineTraceByChannel (Transformation|GetActorLocation Actor1) (Transformation|GetActorLocation Actor2) "TraceTypeQuery1" false (Utilities|Array|MakeArray Actor1 Actor2 Actor3?) "ForOneFrame"))
  (return (not _returnvalue)))