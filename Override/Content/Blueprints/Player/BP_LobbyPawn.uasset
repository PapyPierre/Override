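; BP_LobbyPawn is a lobby pawn that animates the rotation of its root component.
; On BeginPlay it caches the root's starting pitch and yaw, then plays a Timeline at a configurable rate.
; Each update adds the Timeline's pitch and yaw values, scaled by target amounts, to that starting rotation while holding roll at zero.
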(event EventBeginPlay
  (bind _defaultsceneroot (Variables|Default|GetDefaultSceneRoot))
  (bind _relativerotation (Variables|/Script/Engine.SceneComponent|GetRelativeRotation _defaultsceneroot))
  (Variables|Default|SetDefaultPitch (.pitch _relativerotation))
  (Variables|Default|SetDefaultYaw (.yaw _relativerotation))
  (Components|Timeline|SetPlayRate (Variables|Default|GetTimeline) (Variables|Default|GetPlayRate))
  (bind (_direction _pitch _yaw) (Timeline|Timeline Play)
    (:Update
      (Transformation|SetRelativeRotation (Variables|Default|GetDefaultSceneRoot) (Math|Rotator|MakeRotator 0.0 (+ (Variables|Default|GetDefaultPitch) (* (Variables|Default|GetTargetPitch) _pitch)) (+ (Variables|Default|GetDefaultYaw) (* (Variables|Default|GetTargetYaw) _yaw))) false false))))

(fn ConstructionScript)