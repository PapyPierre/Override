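; BP_PlayerStart is a player spawn point that sits out for a cooldown when told to by a caller.
; StartSpawnCooldown stores the caller and starts a timer of SpawnCoolDown length.
; When the timer ends, it passes itself back to the caller through ReAddWhenFinished.
; Tick copies the timer's remaining time into TimeRemaining while the handle is valid.
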(event Custom|StartSpawnCooldown
  (params (Caller :type BP%20Player%20Spawn%20Zone%20Object%20Reference))
  (bind _returnvalue (Utilities|Time|SetTimerbyEvent (delegate Custom|FinishedCoolDown) (Variables|Default|GetSpawnCoolDown)))
  (Variables|Default|SetCaller Caller)
  (Variables|Default|SetTimer _returnvalue))

(event Custom|FinishedCoolDown
  (Default|ReAddwhenFinished (Variables|Default|GetCaller) self))

(event EventBeginPlay)

(event EventTick
  (params (DeltaSeconds :type Float%20%28single-precision%29))
  (bind _timer (Variables|Default|GetTimer))
  (if (Utilities|Time|IsValidTimerHandle _timer)
    (Variables|Default|SetTimeRemaining (Utilities|Time|GetTimerRemainingTimebyHandle _timer))))

(fn ConstructionScript)