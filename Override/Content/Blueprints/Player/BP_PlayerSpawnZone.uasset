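; Player spawn zone that holds a list of spawn points and tags itself with its default team.
; BeginPlay keeps a copy of the list, and events re-add spawns without duplicates when finished.
; When empty, it searches the copy for the spawn with an active timer and lowest time remaining, then re-adds it.
; The construction script places a billboard at each spawn's location.
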(event Custom|ReAddWhenFinished
  (params (NewItem :type BP%20Player%20Start%20Object%20Reference%20%28by%20ref%29))
  (if (== (Utilities|Array|FindItem (Variables|Default|GetPlayerSpawn) NewItem) -1)
    (Utilities|Array|Add (Variables|Default|GetPlayerSpawn) NewItem)))

(event Custom|GetClosestToFinish
  (for _array_element (Variables|Default|GetPlayerSpawnCopy)
    (if (Utilities|Time|IsValidTimerHandle (Variables|/Game/Blueprints/Player/BP_PlayerStart.BP_PlayerStart_C|GetTimer _array_element))
      (if (< (Variables|/Game/Blueprints/Player/BP_PlayerStart.BP_PlayerStart_C|GetTimeRemaining _array_element) (Variables|Default|GetLowestTimeRemaining))
        (bind _output_get (Variables|Default|SetReAddToTeam _array_element))
        (Variables|Default|SetLowestTimeRemaining (Variables|/Game/Blueprints/Player/BP_PlayerStart.BP_PlayerStart_C|GetTimeRemaining _output_get))))))

(event Custom|ReAddWhenEmpty
  (CallFunction|GetClosesttoFinish)
  (CallFunction|ReAddwhenFinished (Variables|Default|GetReAddToTeam)))

(event EventBeginPlay
  (Variables|Default|SetPlayerSpawnCopy (Variables|Default|GetPlayerSpawn))
  (Utilities|Array|Add (Variables|Actor|GetTags) (Utilities|String|StringToName (Utilities|String|ToString(Integer) (Variables|Default|GetDefaultTeamToSpawn)))))

(fn ConstructionScript
  (for _array_element (Variables|Default|GetPlayerSpawn)
    (AddComponent|AddBillboardComponent true (Math|Conversions|ToTransform(Vector) (Transformation|GetActorLocation _array_element)))))