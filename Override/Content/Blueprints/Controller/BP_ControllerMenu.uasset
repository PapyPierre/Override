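; Menu player controller that runs the front end: main menu, username entry, lobby screens, team choice and ability selection.
; It creates the widgets, saves the username through the GameInstance and reacts to lobby list, create (delayed auto-join) and join callbacks.
; RPC events pass team, ability and map requests to BP_GameStateMenu and BP_GameModeMenu, and relay teammate ability picks to the selection screen.
; K and L are debug shortcuts for play and map load.
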(event Custom|SetAbilitiesRPC
  (params (Abilities :type Array%20of%20GA%20Base%20Ability%20Class%20References))
  (Variables|Default|SetCharacter%20Abilities Abilities))

(event Custom|RPC_UpdateTextLobby
  (params (InputPin :type Integer) (B :type String) (Index :type Integer)))

(event Custom|Debug%20Load%20Map
  (Default|DebugLoadNewMap (Variables|Default|GetAs%20BP%20Game%20State%20Menu)))

(event Custom|RPC_CallNewMap
  (bind _asbp_game_mode_menu (Utilities|Casting|CastToBP_GameModeMenu (Game|GetGameMode)))
  (Default|CallNewMap _asbp_game_mode_menu self))

(event Custom|ShowSelection
  (bind _returnvalue (UserInterface|CreateWidget "/Game/Blueprints/Widget/Menu/WBP_SelectionScreen.WBP_SelectionScreen_C" self))
  (UserInterface|Viewport|AddtoViewport _returnvalue 0)
  (Variables|Default|SetSelectionScreen _returnvalue))

(event Custom|RPC_CallPlayButton
  (Default|CallWidget (Variables|Default|GetAs%20BP%20Game%20State%20Menu)))

(event Custom|StartSelection
  (Default|StartSelection (Variables|Default|GetAs%20BP%20Game%20State%20Menu)))

(event Custom|TeammateAbilitySelectNotifyRPC
  (params (SlotIndex :type Integer) (Abiliy :type GA%20Base%20Ability%20Class%20Reference))
  (Default|UpdateTeamateAbilitySlot (Variables|Default|GetSelectionScreen) SlotIndex Abiliy))

(event Custom|RPC_SaveUsername
  (params (UserName :type String))
  (Variables|Default|SetUserName UserName))

(event Custom|ServerNotifyAbilitySelect_RPC
  (params (Slot%20Index :type Integer) (Ability :type GA%20Base%20Ability%20Class%20Reference))
  (Default|AbilitySelectNotify (Variables|Default|GetAs%20BP%20Game%20State%20Menu) (Variables|Default|GetSelectedTeam) self Slot%20Index Ability))

(event Custom|RPC_UpdateText
  (params (Team%20Index :type Integer) (Player :type Integer))
  (Development|PrintString "0")
  (if (!= Team%20Index (Variables|Default|GetSelectedTeam))
    (Development|PrintString "1")
    (Default|RPCSetPlayerinNewTeam (Variables|Default|GetAs%20BP%20Game%20State%20Menu) (Variables|Default|GetUserName) Team%20Index (Variables|Default|GetSelectedTeam) Player)
    (Default|RPCCleanOldTeam (Variables|Default|GetAs%20BP%20Game%20State%20Menu) (Variables|Default|GetSelectedTeam) (Variables|Default|GetOldSlot))
    (Variables|Default|SetSelectedTeam Team%20Index)
    (Variables|Default|SetOldSlot Player)))

(event Custom|HUDMenu
  (params (Name :type String))
  (CallFunction|SaveUsername Name))

(event Custom|SaveUsername
  (params (UserName :type String))
  (Variables|/Game/Blueprints/GameMode/GameInstance/BP_SaveGame.BP_SaveGame_C|SetUserName (Variables|Default|GetAs%20BP%20Save%20Game) UserName)
  (Default|SaveGameData (Variables|Default|GetAs%20BP%20Game%20Instance))
  (CallFunction|RPCNewUIMenu)
  (CallFunction|RPCSaveUsername UserName)
  (Variables|Default|SetUserName UserName))

(event Custom|RPC_NewUIMenu
  (Widget|SetVisibility (Variables|Default|GetMenu%20Widget) "Visible"))

(event Custom|CreateMenu
  (bind _self self)
  ;[0.15 0.15 0.15 0.5] Create Menu
  (bind _returnvalue (UserInterface|CreateWidget "/Game/Blueprints/Widget/Menu/WBP_Menu.WBP_Menu_C" _self))
  (UserInterface|Viewport|AddtoViewport _returnvalue 0)
  (Variables|/Game/Blueprints/Widget/Menu/WBP_Menu.WBP_Menu_C|SetController _returnvalue _self)
  (Variables|Default|SetMenu%20Widget _returnvalue))

(event Custom|UpdateTeam
  (CallFunction|RPCCallUpdateTeam))

(event Custom|RPC_CallUpdateTeam
  (Default|UpdateTeam (Variables|Default|GetAs%20BP%20Game%20State%20Menu) self))

(event EventBeginPlay
  ;[0.15 0.15 0.15 0.5] Begin Play
  (|CallParentFunction)
  (bind _asbp_game_instance (Utilities|Casting|CastToBP_GameInstance (Game|GetGameInstance)))
  (bind _output_get (Variables|Default|SetAs%20BP%20Game%20Instance _asbp_game_instance))
  (Variables|Default|SetAs%20BP%20Save%20Game (Variables|/Game/Blueprints/GameMode/GameInstance/BP_GameInstance.BP_GameInstance_C|GetAs%20BP%20Save%20Game _output_get))
  (bind _asbp_game_state_menu (Utilities|Casting|CastToBP_GameStateMenu (Game|GetGameState)))
  (Variables|Default|SetAs%20BP%20Game%20State%20Menu _asbp_game_state_menu)
  (Networking|SwitchHasAuthority
    (:Remote
      (bind _returnvalue (Game|GetCurrentLevelName true))
      (if (Utilities|Enum|Equal(Enum) _returnvalue "Lvl_Menu")
        (Variables|/Script/Engine.PlayerController|SetbShowMouseCursor self true)
        (bind _returnvalue_2 (UserInterface|CreateWidget "/Game/Blueprints/Widget/Menu/WBP_MainMenu.WBP_MainMenu_C"))
        (UserInterface|Viewport|AddtoViewport _returnvalue_2 0)
        (Variables|/Script/UMG.TextBlock|SetText (Variables|/Game/Blueprints/Widget/Menu/WBP_MainMenu.WBP_MainMenu_C|GetVersion_Txt _returnvalue_2) (Utilities|Text|ToText(String) (Utilities|String|Append "Version: " (Class|BlueprintHelpers|GetProjectVersion))))))))

(event EventOnLobbyListReceived
  (params (Lobbies :type Array%20of%20Lobby%20Structures))
  ;[0.15 0.15 0.15 0.5] Lobby List Received
  (Default|UpdateList (Variables|Default|GetLobby%20List) Lobbies))

(event EventOnLobbyCreated
  (params (LobbyId :type String))
  ;[0.15 0.15 0.15 0.5] On Lobby Created
  (Utilities|FlowControl|Delay 4.0)
  (Class|CustomPlayerController|JoinLobby LobbyId))

(event EventOnLobbyJoined
  (params (LobbyId :type String))
  ;[0.15 0.15 0.15 0.5] On  Lobby Joined
  (CallFunction|ShowLobby LobbyId))

(event EventOnLobbyLeft)

(event Input|KeyboardEvents|DebugKeyL
  (params (Key :type Key%20Structure :default "None") (ActionValue :type Input%20Action%20Value%20Structure))
  (:Pressed
    (CallFunction|DebugLoadMap)))

(event Input|KeyboardEvents|DebugKeyK
  (params (Key :type Key%20Structure :default "None") (ActionValue :type Input%20Action%20Value%20Structure))
  (:Pressed
    (CallFunction|RPCCallPlayButton)))

(fn ConstructionScript)

(fn SetAbilities
  (params (Abilities :type Array%20of%20GA%20Base%20Ability%20Class%20References))
  (CallFunction|SetAbilitiesRPC Abilities))

(fn TeammateAbilitySelectNotify
  (params (Slot%20Index :type Integer) (Ability :type GA%20Base%20Ability%20Class%20Reference))
  (CallFunction|TeammateAbilitySelectNotifyRPC Slot%20Index Ability))

(fn NotifyStateAbilitySelect
  (params (Slot%20Index :type Integer) (Ability :type GA%20Base%20Ability%20Class%20Reference))
  (Development|PrintString (Utilities|GetClassDisplayName Ability))
  (CallFunction|ServerNotifyAbilitySelectRPC Slot%20Index Ability))

(fn ShowMenu
  (if (Utilities|Array|IsEmpty (Variables|/Game/Blueprints/GameMode/GameInstance/BP_SaveGame.BP_SaveGame_C|GetUserName (Variables|Default|GetAs%20BP%20Save%20Game)))
    (CallFunction|CreateMenu)
    (Widget|SetVisibility (Variables|Default|GetMenu%20Widget) "Collapsed")
    (Variables|/Script/Engine.PlayerController|SetbShowMouseCursor self true)
    (bind _returnvalue (UserInterface|CreateWidget "/Game/Blueprints/Widget/Menu/WBP_UserNameInput.WBP_UserNameInput_C" self))
    (UserInterface|Viewport|AddtoViewport _returnvalue 0)
    (else
      (bind _output_get (Variables|Default|SetUserName (Variables|/Game/Blueprints/GameMode/GameInstance/BP_SaveGame.BP_SaveGame_C|GetUserName (Variables|Default|GetAs%20BP%20Save%20Game))))
      (CallFunction|RPCSaveUsername _output_get)
      (Variables|/Script/Engine.PlayerController|SetbShowMouseCursor self true)
      (CallFunction|CreateMenu))))

(fn ShowLobbyList
  (bind _returnvalue (UserInterface|CreateWidget "/Game/Blueprints/Widget/Menu/WBP_Lobby_List.WBP_Lobby_List_C" self))
  (UserInterface|Viewport|AddtoViewport _returnvalue 0)
  (Variables|Default|SetLobby%20List _returnvalue)
  (Class|CustomPlayerController|FetchLobbyList))

(fn ShowLobby
  (params (Lobby%20ID :type String))
  (bind _returnvalue (UserInterface|CreateWidget "/Game/Blueprints/Widget/Menu/WBP_Lobby.WBP_Lobby_C"))
  (bind _output_get (Variables|Default|SetOpenedLobby _returnvalue))
  (UserInterface|Viewport|AddtoViewport _output_get 0)
  (bind _menu_widget (Variables|Default|GetMenu%20Widget)
    (:then
      (Widget|SetVisibility _menu_widget "Hidden"))
    (:else
      _))
  (Variables|/Game/Blueprints/Widget/Menu/WBP_Lobby.WBP_Lobby_C|SetCotrnoller _output_get self)
  (bind _output_get_2 (Variables|/Game/Blueprints/Widget/Menu/WBP_Lobby.WBP_Lobby_C|SetLobby%20ID _output_get Lobby%20ID))
  (Variables|/Script/UMG.TextBlock|SetText (Variables|/Game/Blueprints/Widget/Menu/WBP_Lobby.WBP_Lobby_C|GetLobbyName _output_get) (Utilities|Text|ToText(String) _output_get_2)))

(fn HideLobby)

(fn UpdateServerText
  (params (Team%20Index :type Integer) (Player%20Index :type Integer))
  (Development|PrintString "-1")
  (CallFunction|RPCUpdateText Team%20Index Player%20Index))