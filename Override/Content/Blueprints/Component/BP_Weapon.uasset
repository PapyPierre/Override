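; Weapon component for BP_FirstPersonCharacter that handles hitscan firing, ammo and reloading.
; While not sprinting, fire input runs RPM-limited camera traces that spend ammo, update the HUD and count shots, which decay on Tick.
; Hits on non-teammate characters scale base or long-range damage by a physical-material DataTable row, applied directly with authority or through a custom event on remotes.
; Reloading spins the weapon, refills ammo and blocks firing until shoot is pressed again.
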(event Custom|Reload
  (bind _weapon (Variables|Default|GetWeapon))
  (bind _relativelocation (Variables|/Script/Engine.SceneComponent|GetRelativeLocation _weapon))
  ;[0.15 0.15 0.15 0.5] Reload
  (Variables|Default|SetIsShooting false)
  (if (not (Variables|Default|GetReloading))
    (Variables|Default|SetReloading true)
    (Components|MoveComponentTo _weapon _relativelocation "0.000000,0.000000,180.000000" false false 0.3 false)
    (Components|MoveComponentTo _weapon _relativelocation "0.000000,0.000000,360.000000" false false 0.3 false)
    (Variables|Default|SetCurrentMunition (Variables|Default|GetMaxMunition%20))
    (Variables|Default|SetShootFired 0)
    (Variables|Default|SetReloading false)
    (CallFunction|UpdateHUD)
    (Variables|Default|SetDoReactivate true)))

(event Custom|UpdateHUD
  ;[0.15 0.15 0.15 0.5] Update Ammo HUD
  (Variables|/Script/UMG.TextBlock|SetText (Variables|/Game/Blueprints/Widget/WBP_HUD.WBP_HUD_C|GetMunitionCount (Variables|/Game/Blueprints/Player/BP_FirstPersonPlayerController.BP_FirstPersonPlayerController_C|GetHUD (Variables|/Game/Blueprints/Player/BP_FirstPersonCharacter.BP_FirstPersonCharacter_C|GetPlayer%20Controller (Variables|Default|GetAs%20BP%20First%20Person%20Character)))) (Utilities|Text|ToText(Integer) (Variables|Default|GetCurrentMunition))))

(event Custom|CancelShoot
  (bind _returnvalue (Game|GetPlayerCameraManager 0))
  (bind _as_bp_first_person_character (Variables|Default|GetAs%20BP%20First%20Person%20Character))
  (bind _transformcomponent (Variables|/Script/Engine.PlayerCameraManager|GetTransformComponent _returnvalue))
  (bind _returnvalue_2 (Transformation|GetWorldLocation _transformcomponent))
  ;[0.15 0.15 0.15 0.5] Shoot
  (Variables|Default|SetIsShooting false)
  (Utilities|FlowControl|Gate false) ; enters at Close
)

(event Custom|OpenShoot
  (bind _returnvalue (Game|GetPlayerCameraManager 0))
  (bind _as_bp_first_person_character (Variables|Default|GetAs%20BP%20First%20Person%20Character))
  (bind _transformcomponent (Variables|/Script/Engine.PlayerCameraManager|GetTransformComponent _returnvalue))
  (bind _returnvalue_2 (Transformation|GetWorldLocation _transformcomponent))
  ;[0.15 0.15 0.15 0.5] Shoot
  (Utilities|FlowControl|Gate false) ; enters at Open
)

(event Custom|ApplyDamage
  (params (Damaged%20Actor :type Actor%20Object%20Reference) (Damage :type Float%20%28double-precision%29) (Hit :type Hit%20Result%20Structure) (Damage%20Causer :type Actor%20Object%20Reference) (Direction :type Vector))
  (Game|Damage|ApplyPointDamage Damaged%20Actor Damage Direction Hit 0 Damage%20Causer "/Script/Engine.DamageType"))

(event Input|EnhancedActionEvents|EnhancedInputActionIA_Shoot
  (params (ActionValue :type Boolean) (ElapsedSeconds :type Float%20%28double-precision%29) (TriggeredSeconds :type Float%20%28double-precision%29) (InputAction :type Input%20Action%20Object%20Reference :default "/Game/Input/Actions/IA_Shoot.IA_Shoot"))
  (bind _returnvalue (Game|GetPlayerCameraManager 0))
  (bind _as_bp_first_person_character (Variables|Default|GetAs%20BP%20First%20Person%20Character))
  (bind _transformcomponent (Variables|/Script/Engine.PlayerCameraManager|GetTransformComponent _returnvalue))
  (bind _returnvalue_2 (Transformation|GetWorldLocation _transformcomponent))
  ;[0.15 0.15 0.15 0.5] Shoot
  (:Triggered
    (Utilities|FlowControl|Gate false :!label _label
      (:Exit
        (if (not (Variables|Default|GetDoReactivate))
          (if (not (Variables|/Script/Override.PlayerMovementComponent|GetbWantsToSprint (Variables|/Script/Override.PlayerCharacter|GetPlayerMovementComponent (Variables|Default|GetAs%20BP%20First%20Person%20Character))))
            (if (>= (Variables|Default|GetDelta%20Seconds) (/ 6e+01 (Variables|Default|GetRPM)))
              (Variables|Default|SetDelta%20Seconds 0.0)
              (if (> (Variables|Default|GetCurrentMunition) 0)
                (Variables|Default|SetIsShooting true)
                (bind (_outhit _returnvalue_3) (Collision|LineTraceForObjects _returnvalue_2 (+ _returnvalue_2 (* (Math|Vector|GetForwardVector _transformcomponent) 2e+04)) (Utilities|Array|MakeArray "ObjectTypeQuery3") false 0 "ForDuration"))
                (Math|Integer|DecrementInt (Variables|Default|GetCurrentMunition)
                  (:%20%20
                    (Math|Integer|IncrementInt (Variables|Default|GetShootFired)
                      (:%20%20
                        (CallFunction|UpdateHUD)
                        (if _returnvalue_3
                          (if (== (Utilities|GetClass (.HitActor (Collision|BreakHitResult _outhit))) "/Game/Blueprints/Player/BP_FirstPersonCharacter.BP_FirstPersonCharacter_C")
                            (if (== (Class|GameplayStatics|GetPlayerControllerfromID (Variables|/Game/Blueprints/Player/BP_FirstPersonPlayerController.BP_FirstPersonPlayerController_C|GetTeammate (Variables|/Game/Blueprints/Player/BP_FirstPersonCharacter.BP_FirstPersonCharacter_C|GetPlayer%20Controller (Variables|Default|GetAs%20BP%20First%20Person%20Character)))) (.AsBP%20First%20Person%20Character (Utilities|Casting|CastToBP_FirstPersonCharacter (.HitActor (Collision|BreakHitResult _outhit)))))
                              (Development|PrintString "Hello")
                              (else
                                (bind _returnvalue_4 (Utilities|GetDataTableRow "/Game/Blueprints/DataTable-Struct/DT_LocalizedDamage.DT_LocalizedDamage" (Utilities|String|StringToName (Utilities|GetObjectName (.PhysMat (Collision|BreakHitResult _outhit)))))
                                  (:then
                                    (Networking|SwitchHasAuthority
                                      (:Authority
                                        (Game|Damage|ApplyPointDamage (.AsBP%20First%20Person%20Character (Utilities|Casting|CastToBP_FirstPersonCharacter (.HitActor (Collision|BreakHitResult _outhit)))) (* (Utilities|Struct|BreakStruct_LocalizedDamage _returnvalue_4) (select (>= (Math|Vector|Distance(Vector) (Transformation|GetSocketLocation (Variables|Default|GetWeapon) "Muzzle") (.ImpactPoint (Collision|BreakHitResult _outhit))) (Variables|Default|GetMaxRange)) (Variables|Default|GetReducedDamage) (Variables|Default|GetBaseDamage))) (.Location (Collision|BreakHitResult _outhit)) _outhit 0 _as_bp_first_person_character "/Script/Engine.DamageType"))
                                      (:Remote
                                        (CallFunction|ApplyDamage (.AsBP%20First%20Person%20Character (Utilities|Casting|CastToBP_FirstPersonCharacter (.HitActor (Collision|BreakHitResult _outhit)))) (* (Utilities|Struct|BreakStruct_LocalizedDamage _returnvalue_4) (select (>= (Math|Vector|Distance(Vector) (Transformation|GetSocketLocation (Variables|Default|GetWeapon) "Muzzle") (.ImpactPoint (Collision|BreakHitResult _outhit))) (Variables|Default|GetMaxRange)) (Variables|Default|GetReducedDamage) (Variables|Default|GetBaseDamage))) _outhit _as_bp_first_person_character (.Location (Collision|BreakHitResult _outhit)))))))))))))))
                (else
                  (CallFunction|Reload)))))))))
  (:Started
    (Variables|Default|SetDoReactivate false)
    (goto _label Open))
  (:Canceled
    (Variables|Default|SetIsShooting false :!label _label_2))
  (:Completed
    (goto _label_2)))

(event Input|EnhancedActionEvents|EnhancedInputActionIA_Reload
  (params (ActionValue :type Boolean) (ElapsedSeconds :type Float%20%28double-precision%29) (TriggeredSeconds :type Float%20%28double-precision%29) (InputAction :type Input%20Action%20Object%20Reference :default "/Game/Input/Actions/IA_Reload.IA_Reload"))
  ;[0.15 0.15 0.15 0.5] Reload Input
  (:Started
    (if (not (== (Variables|Default|GetMaxMunition%20) (Variables|Default|GetCurrentMunition)))
      (CallFunction|Reload))))

(event EventBeginPlay
  ;[0.15 0.15 0.15 0.5] Begin
  (bind _asbp_first_person_character (Utilities|Casting|CastToBP_FirstPersonCharacter (Components|GetOwner)))
  (Variables|Default|SetAs%20BP%20First%20Person%20Character _asbp_first_person_character)
  (Variables|Default|SetCurrentMunition (Variables|Default|GetMaxMunition%20))
  (Variables|Default|SetWeapon (Variables|/Game/Blueprints/Player/BP_FirstPersonCharacter.BP_FirstPersonCharacter_C|GetWeapon (Variables|Default|GetAs%20BP%20First%20Person%20Character))))

(event EventTick
  (params (DeltaSeconds :type Float%20%28single-precision%29))
  ;[0.15 0.15 0.15 0.5] Tick
  (Variables|Default|SetDelta%20Seconds (+ DeltaSeconds (Variables|Default|GetDelta%20Seconds)))
  (if (not (Variables|Default|GetIsShooting))
    (if (> (Variables|Default|GetShootFired) 0)
      (Utilities|FlowControl|Delay (Variables|Default|GetMunitionRecallTime))
      (Math|Integer|DecrementInt (Variables|Default|GetShootFired)))))