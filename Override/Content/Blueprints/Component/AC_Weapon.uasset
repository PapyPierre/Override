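; Networked single-shot hitscan weapon component for BP_FirstPersonCharacter, configured by a DataAsset, with an automatic reload after each shot.
; Gated input sends camera traces to the server; the client retraces hits, requests team checks and sends damage RPCs, scaled by body part and range for players.
; A multicast plays Niagara and audio effects with colors relative to the viewer's team, while OnRep functions drive the fire gate and recoil recall.
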(event Custom|RPC_Reload
  ;[0.15 0.15 0.15 0.5] Reload
  (if (not (Variables|Default|GetReloading))
    (Variables|Default|SetReloading true)
    (Variables|Default|SetCanShoot false)
    (Networking|SwitchHasAuthority
      (:Authority
        (Utilities|FlowControl|Delay (Variables|Default|GetReloadDuration))
        (CallFunction|EndReload)))))

(event Custom|SetTeamOwning
  (params (Value :type Boolean))
  ;[0.15 0.15 0.15 0.5] Team Check
  (Variables|Default|SetIsOnTheSameTeam Value)
  (CallFunction|Continue))

(event Custom|SetCrosshairHit
  (params (HeadShot :type Boolean))
  (bind _as_bp_first_person_character (Variables|Default|GetAs%20BP%20First%20Person%20Character))
  (bind _player_controller (Variables|/Game/Blueprints/Player/BP_FirstPersonCharacter.BP_FirstPersonCharacter_C|GetPlayer%20Controller _as_bp_first_person_character))
  (bind _hud (Variables|/Game/Blueprints/Controller/BP_FirstPersonPlayerController.BP_FirstPersonPlayerController_C|GetHUD _player_controller))
  (bind _wbp_crosshair (Variables|/Game/Blueprints/Widget/WBP_HUD.WBP_HUD_C|GetWBP_Crosshair _hud))
  ;[0.15 0.15 0.15 0.5] CrossHair Visual
  (UserInterface|Animation|PlayAnimation _wbp_crosshair (select HeadShot (Variables|/Game/Blueprints/Widget/HUD/WBP_Crosshair.WBP_Crosshair_C|GetCriticalEnemyHit _wbp_crosshair) (Variables|/Game/Blueprints/Widget/HUD/WBP_Crosshair.WBP_Crosshair_C|GetEnemyHit _wbp_crosshair)) 0.0 1 "Forward" 1.0 false)
  ;[0.15 1 0.15 0.5] SFX Hitmarker
  (if HeadShot
    (Class|FMODBlueprintStatics|PlayEvent2D "/Game/FMOD/Events/SFX_FOLDER/SFX/SFX_UI/HitMarker_Headshot.HitMarker_Headshot")
    (else
      (Class|FMODBlueprintStatics|PlayEvent2D "/Game/FMOD/Events/SFX_FOLDER/SFX/SFX_UI/HitMarker.HitMarker"))))

(event Custom|Continue
  ;[0.15 0.15 0.15 0.5] Client Line Trace Result
  (if (not (Variables|Default|GetIsOnTheSameTeam))
    (bind _returnvalue (Utilities|GetDataTableRow "/Game/Data/DataTable/DT_LocalizedDamage.DT_LocalizedDamage" (Utilities|String|StringToName (Utilities|GetObjectName (.PhysMat (Collision|BreakHitResult (stale Custom|Client_LineTraceResult _outputpin))))))
      (:then
        _)
      (:RowNotFound
        _))
    (CallFunction|ApplyDamage (.HitActor (Collision|BreakHitResult (stale Custom|Client_LineTraceResult _outputpin))) (* (Utilities|Struct|BreakS_LocalizedDamage _returnvalue) (select (>= (Math|Vector|Distance(Vector) (Transformation|GetSocketLocation (Variables|Default|GetWeapon) "Muzzle") (.ImpactPoint (Collision|BreakHitResult (stale Custom|Client_LineTraceResult _outputpin)))) (Variables|PasTouche|GetMaxRange)) (Variables|PasTouche|GetReducedDamage) (Variables|PasTouche|GetBaseDamage))) (stale Custom|Client_LineTraceResult _outputpin) (Variables|Default|GetAs%20BP%20First%20Person%20Character) (.Location (Collision|BreakHitResult (stale Custom|Client_LineTraceResult _outputpin))))
    (CallFunction|SetCrosshairHit (== (.PhysMat (Collision|BreakHitResult (stale Custom|Client_LineTraceResult _outputpin))) "/Game/Art/Characters/Devs/PhysicsMaterial/PM_Head.PM_Head"))))

(event Custom|CancelAim
  ;[0.15 0.15 0.15 0.5] Reload
  (Default|CancelAim (Variables|Default|GetAs%20BP%20First%20Person%20Character)))

(event Custom|OpenAim
  (Default|OpenAim (Variables|Default|GetAs%20BP%20First%20Person%20Character)))

(event Custom|Multicast_Effect
  (params (HitResult :type Hit%20Result%20Structure) (RibbonColor :type Linear%20Color%20Structure%20%28by%20ref%29) (MuzzleColor :type Linear%20Color%20Structure%20%28by%20ref%29) (Team :type Integer))
  (bind (_bblockinghit _binitialoverlap _time _distance _location _impactpoint _normal _impactnormal _physmat _hitactor _hitcomponent _hitbonename _bonename _hititem _elementindex _faceindex _tracestart _traceend) (Collision|BreakHitResult HitResult))
  (bind _returnvalue (Game|GetPlayerController 0))
  (bind _returnvalue_2 (Utilities|Select :Index Team :Option%200 2.0 :Option%201 3.0 :Option%202 1.0))
  (bind _returnvalue_3 (Utilities|Select :Index Team :Option%200 1.0 :Option%201 2.0 :Option%202 3.0))
  (bind _returnvalue_4 (Utilities|Select :Index Team :Option%200 2.0 :Option%201 1.0 :Option%202 3.0))
  (bind _muzzle_socket_name (Variables|Default|GetMuzzle%20Socket%20Name))
  (bind _as_bp_first_person_character (Variables|Default|GetAs%20BP%20First%20Person%20Character))
  (bind _as_bp_first_person_character_2 (Variables|Default|GetAs%20BP%20First%20Person%20Character))
  (bind _returnvalue_5 (Collision|GetCollisionObjectType _hitcomponent))
  (bind _returnvalue_6 (Pawn|IsLocallyControlled _as_bp_first_person_character))
  (bind _asbp_first_person_player_controller (Utilities|Casting|CastToBP_FirstPersonPlayerController _returnvalue))
  (bind _tpsweapon (Variables|/Game/Blueprints/Player/BP_FirstPersonCharacter.BP_FirstPersonCharacter_C|GetTPSWeapon _as_bp_first_person_character_2))
  (bind _fpsweapon (Variables|/Game/Blueprints/Player/BP_FirstPersonCharacter.BP_FirstPersonCharacter_C|GetFPSWeapon _as_bp_first_person_character_2))
  (bind _teamindex (Variables|/Game/Blueprints/Controller/BP_FirstPersonPlayerController.BP_FirstPersonPlayerController_C|GetTeamIndex _asbp_first_person_player_controller))
  (bind _returnvalue_7 (Utilities|Select :Index _teamindex :Option%200 _returnvalue_3 :Option%201 _returnvalue_4 :Option%202 _returnvalue_2))
  ;[0.15 0.15 0.15 0.5] Shoot Effect
  (Networking|SwitchHasAuthority
    (:Remote
      (Rendering|Material|SetVectorParameterValue "/Game/Art/Niagara/Parameter/MPC_MuzzleFlash.MPC_MuzzleFlash" "ColorRibbon" RibbonColor :!class /Script/Engine.KismetMaterialLibrary)
      (Rendering|Material|SetVectorParameterValue "/Game/Art/Niagara/Parameter/MPC_MuzzleFlash.MPC_MuzzleFlash" "ColorMuzzle" MuzzleColor :!class /Script/Engine.KismetMaterialLibrary)
      (bind _returnvalue_8 (Niagara|SpawnSystematLocation "/Game/Art/Niagara/NS_BulletTrailHitscan.NS_BulletTrailHitscan" (select (Pawn|IsLocallyControlled (Variables|Default|GetAs%20BP%20First%20Person%20Character)) (Transformation|GetSocketLocation _fpsweapon _muzzle_socket_name) (Transformation|GetSocketLocation _tpsweapon _muzzle_socket_name))))
      (Class|NiagaraComponent|SetVariablePosition _returnvalue_8 "Position" (select _bblockinghit _impactpoint _traceend))
      (Niagara|SetNiagaraVariable(Float) _returnvalue_8 "ColorID" _returnvalue_7)
      (if (and (Variables|/Script/Override.PlayerCharacter|GetbIsAimingWeapon _as_bp_first_person_character) _returnvalue_6)
        _
        (else
          (bind _returnvalue_9 (Niagara|SpawnSystemAttached (select _returnvalue_6 "/Game/Art/Niagara/NS_MuzzleFlashTPV.NS_MuzzleFlashTPV" "/Game/Art/Niagara/NS_MuzzleFlash.NS_MuzzleFlash") (select _returnvalue_6 _fpsweapon _tpsweapon) "None" "0, 0, 0" "0, 0, 0" "KeepRelativeOffset" true))
          (if _returnvalue_6
            (Rendering|SetFirstPersonPrimitiveType _returnvalue_9 "FirstPerson")
            (else
              (Niagara|SetNiagaraVariable(Float) _returnvalue_9 "ColorID" _returnvalue_7)))))
      ;;[0.15 1 0.15 0.5] SFX Shoot
      (Class|FMODBlueprintStatics|PlayEventAttached "/Game/FMOD/Events/SFX_FOLDER/SFX/Gunplay/Shoot.Shoot" (Variables|/Game/Blueprints/Player/BP_FirstPersonCharacter.BP_FirstPersonCharacter_C|GetFPSWeapon (Variables|Default|GetAs%20BP%20First%20Person%20Character)) "None" "0, 0, 0" "KeepRelativeOffset")
      (if _bblockinghit
        (if (and (or (Utilities|Enum|Equal(Enum) _returnvalue_5 "ECC_GameTraceChannel1") (Utilities|Enum|Equal(Enum) _returnvalue_5 "ECC_WorldStatic")) (!= (Utilities|GetClass _hitactor) "/Game/Blueprints/Player/BP_FirstPersonCharacter.BP_FirstPersonCharacter_C"))
          (bind _returnvalue_10 (Niagara|SpawnSystematLocation "/Game/Art/Niagara/NS_BulletImpact.NS_BulletImpact" _impactpoint (Math|Rotator|MakeRotfromX (* _impactnormal -1.0))))
          (Niagara|SetNiagaraVariable(Float) _returnvalue_10 "ColorID" _returnvalue_7)
          ;;[0.15 1 0.15 0.5] SFX Shot Wall Hit
          (Class|FMODBlueprintStatics|PlayEventatLocation "/Game/FMOD/Events/SFX_FOLDER/SFX/Gunplay/Shot_Passby.Shot_Passby" (Math|Transform|MakeTransform _impactnormal)))))))

(event Custom|OpenShoot
  (bind _returnvalue (Game|GetPlayerCameraManager 0))
  (bind _transformcomponent (Variables|/Script/Engine.PlayerCameraManager|GetTransformComponent _returnvalue))
  (bind _returnvalue_2 (Transformation|GetWorldLocation _transformcomponent))
  (Utilities|FlowControl|Gate false) ; enters at Open
)

(event Custom|SetCrosshair
  (bind _as_bp_first_person_character (Variables|Default|GetAs%20BP%20First%20Person%20Character))
  (bind _player_controller (Variables|/Game/Blueprints/Player/BP_FirstPersonCharacter.BP_FirstPersonCharacter_C|GetPlayer%20Controller _as_bp_first_person_character))
  (bind _hud (Variables|/Game/Blueprints/Controller/BP_FirstPersonPlayerController.BP_FirstPersonPlayerController_C|GetHUD _player_controller))
  (bind _wbp_crosshair (Variables|/Game/Blueprints/Widget/WBP_HUD.WBP_HUD_C|GetWBP_Crosshair _hud))
  (UserInterface|Animation|PlayAnimation _wbp_crosshair (Variables|/Game/Blueprints/Widget/HUD/WBP_Crosshair.WBP_Crosshair_C|GetShoot _wbp_crosshair) 0.0 1 "Forward" 1.0 false)
  (Default|PlayerRunStop _wbp_crosshair)
  (Utilities|FlowControl|RetriggerableDelay 0.7)
  (Variables|/Game/Blueprints/Player/BP_FirstPersonCharacter.BP_FirstPersonCharacter_C|GetMovingInput (Variables|Default|GetAs%20BP%20First%20Person%20Character)
    (:then
      (Default|PlayerRunStart _wbp_crosshair))
    (:else)))

(event Custom|CancelShoot
  (bind _returnvalue (Game|GetPlayerCameraManager 0))
  (bind _transformcomponent (Variables|/Script/Engine.PlayerCameraManager|GetTransformComponent _returnvalue))
  (bind _returnvalue_2 (Transformation|GetWorldLocation _transformcomponent))
  (Utilities|FlowControl|Gate false) ; enters at Close
)

(event Custom|ShootLineTrace
  (params (NewParam :type Vector) (NewParam2 :type Vector))
  ;[0.15 0.15 0.15 0.5] Line Trace For Hit (then Sphere Trace for wider detection)
  (if (> (Variables|Default|GetCurrentMunition) 0)
    (Variables|Default|SetIsShooting true)
    (Variables|Default|SetCurrentMunition 0)
    (Math|Integer|IncrementInt (Variables|Default|GetShootFired)
      (:%20%20
        (bind (_outputpin _outputpin1) (CallFunction|LineTrace NewParam NewParam2))
        (CallFunction|ClientLineTraceResult _outputpin1 NewParam NewParam2)
        (CallFunction|MulticastEffect _outputpin (Variables|Default|GetRibbonColor) (Variables|Default|GetMuzzleColor) (Variables|/Game/Blueprints/Player/BP_FirstPersonCharacter.BP_FirstPersonCharacter_C|GetTeamIndex (Variables|Default|GetAs%20BP%20First%20Person%20Character)))))))

(event Custom|ApplyDamage
  (params (Damaged%20Actor :type Actor%20Object%20Reference) (Damage :type Float%20%28double-precision%29) (Hit :type Hit%20Result%20Structure) (Damage%20Causer :type Actor%20Object%20Reference) (Direction :type Vector))
  ;[0.15 0.15 0.15 0.5] Apply Damage RPC
  (Game|Damage|ApplyPointDamage Damaged%20Actor Damage Direction Hit 0 Damage%20Causer "/Script/Engine.DamageType"))

(event Custom|RPC_SetShooting
  (params (Value :type Boolean))
  ;[0.15 0.15 0.15 0.5] RPC Set Value
  (Variables|Default|SetIsShooting Value))

(event Custom|CheckTeamServer
  (params (Player1 :type BP%20First%20Person%20Character%20Object%20Reference) (Player2 :type BP%20First%20Person%20Character%20Object%20Reference))
  ;[0.15 0.15 0.15 0.5] Team Check
  (bind _value (Default|IsontheSameTeam? (Variables|/Game/Blueprints/Player/BP_FirstPersonCharacter.BP_FirstPersonCharacter_C|GetAs%20BP%20Game%20State Player1) Player1 Player2))
  (bind _output_get (Variables|Default|SetIsOnTheSameTeam _value))
  (CallFunction|SetTeamOwning _output_get))

(event Custom|EndReload
  ;[0.15 0.15 0.15 0.5] Reload
  (Variables|Default|SetIsShooting false)
  (Variables|Default|SetCurrentMunition 1)
  (Variables|Default|SetShootFired 0)
  (Variables|Default|SetReloading false)
  (CallFunction|OpenAim)
  (Variables|/Game/Blueprints/Player/BP_FirstPersonCharacter.BP_FirstPersonCharacter_C|GetHasFlag (Variables|Default|GetAs%20BP%20First%20Person%20Character)
    (:then)
    (:else
      (Variables|Default|SetCanShoot true))))

(event Custom|RPC_ShootLineTrace
  (params (Start :type Vector) (End :type Vector))
  (bind _as_bp_first_person_character (Variables|Default|GetAs%20BP%20First%20Person%20Character))
  (CallFunction|ShootLineTrace Start End)
  (Variables|/Game/Blueprints/Player/BP_FirstPersonCharacter.BP_FirstPersonCharacter_C|GetInCamouflage _as_bp_first_person_character
    (:then
      (Default|StopCamouflage _as_bp_first_person_character))
    (:else)))

(event Custom|Client_LineTraceResult
  (params (Value :type Boolean) (Start :type Vector) (End :type Vector))
  ;[0.15 0.15 0.15 0.5] Client Line Trace Result
  (bind _outputpin (CallFunction|LineTrace Start End))
  (if Value
    (bind _asbp_first_person_character (Utilities|Casting|CastToBP_FirstPersonCharacter (.HitActor (Collision|BreakHitResult _outputpin)))
      (:then
        (CallFunction|CheckTeamServer _asbp_first_person_character (Variables|Default|GetAs%20BP%20First%20Person%20Character)))
      (:CastFailed
        ;[0.15 0.15 0.15 0.5] Shoot on modulation
        (bind _asbp_modulation (Utilities|Casting|CastToBP_Modulation (.HitActor (Collision|BreakHitResult _outputpin))))
        (if (not (Variables|/Script/Override.Modulation|GetIsDemat _asbp_modulation))
          (CallFunction|ApplyDamage _asbp_modulation (Variables|Default|GetDamageOnModulations) _outputpin (Variables|Default|GetAs%20BP%20First%20Person%20Character) (.Location (Collision|BreakHitResult _outputpin))))))))

(event Input|EnhancedActionEvents|EnhancedInputActionIA_Shoot
  (params (ActionValue :type Boolean) (ElapsedSeconds :type Float%20%28double-precision%29) (TriggeredSeconds :type Float%20%28double-precision%29) (InputAction :type Input%20Action%20Object%20Reference :default "/Game/Input/Actions/IA_Shoot.IA_Shoot"))
  (bind _returnvalue (Game|GetPlayerCameraManager 0))
  (bind _transformcomponent (Variables|/Script/Engine.PlayerCameraManager|GetTransformComponent _returnvalue))
  (bind _returnvalue_2 (Transformation|GetWorldLocation _transformcomponent))
  (:Started
    (if (Variables|Default|GetCanShoot)
      _
      (else
        (Variables|/Game/Blueprints/Player/BP_FirstPersonCharacter.BP_FirstPersonCharacter_C|GetHasFlag (Variables|Default|GetAs%20BP%20First%20Person%20Character)
          (:then)
          (:else
            (Utilities|FlowControl|Delay (* (Variables|Default|GetReloadDuration) 0.75))
            (Variables|Default|GetCanShoot
              (:then
                _)
              (:else))))))
    (Utilities|FlowControl|Gate false
      (:Exit
        (if (not (Variables|Default|GetIsShooting))
          (CallFunction|RPCShootLineTrace _returnvalue_2 (+ _returnvalue_2 (* (Math|Vector|GetForwardVector _transformcomponent) 2e+04)))
          (CallFunction|RPCReload)
          (CallFunction|SetCrosshair)
          ;[0.15 1 0.15 0.5] CameraShake Shoot
          (CameraShakes|StartCameraShake (Variables|/Script/Engine.PlayerController|GetPlayerCameraManager (Game|GetPlayerController 0)) "/Game/Blueprints/Camera/CameraShake/CS_Shoot.CS_Shoot_C" 1.0 "CameraLocal" "0, 0, 0"))))))

(event EventBeginPlay
  ;[0.15 0.15 0.15 0.5] Begin
  (bind _asbp_first_person_character (Utilities|Casting|CastToBP_FirstPersonCharacter (Components|GetOwner)))
  (Variables|Default|SetAs%20BP%20First%20Person%20Character _asbp_first_person_character)
  (Variables|Default|SetEase%20Out%20Time%20Melee 0.15)
  (Variables|Default|SetWeapon (Variables|/Game/Blueprints/Player/BP_FirstPersonCharacter.BP_FirstPersonCharacter_C|GetFPSWeapon (Variables|Default|GetAs%20BP%20First%20Person%20Character)))
  (Utilities|IsValid (Variables|Default|GetDataAsset)
    (:Is%20Valid
      ;;[0.15 0.01867 0.02311 0.5] Le voilà votre DataAsset
      (CallFunction|ReadDataAsset)
      (Variables|Default|SetReloadDuration (Variables|PasTouche|GetReload)))))

(event EventTick
  (params (DeltaSeconds :type Float%20%28single-precision%29))
  ;[0.15 0.15 0.15 0.5] Tick
  (Variables|Default|SetDelta%20Seconds (+ DeltaSeconds (Variables|Default|GetDelta%20Seconds)))
  (Networking|SwitchHasAuthority
    (:Authority
      (if (not (Variables|Default|GetIsShooting))
        (if (> (Variables|Default|GetShootFired) 0)
          (Utilities|FlowControl|Delay (Variables|PasTouche|GetMunitionRecallTime))
          (Math|Integer|DecrementInt (Variables|Default|GetShootFired)))))))

(fn RPCShoot
  (return))

(fn OnRepCanShoot
  (if (Pawn|IsLocallyControlled (Variables|Default|GetAs%20BP%20First%20Person%20Character))
    (Networking|SwitchHasAuthority
      (:Remote
        (if (Variables|Default|GetCanShoot)
          (CallFunction|OpenShoot)
          (else
            (CallFunction|CancelShoot)))))))

(fn OnRepIsShooting
  (bind _as_bp_first_person_character (Variables|Default|GetAs%20BP%20First%20Person%20Character))
  (Variables|/Script/Override.PlayerMovementComponent|SetbIsShooting (Variables|/Game/Blueprints/Player/BP_FirstPersonCharacter.BP_FirstPersonCharacter_C|GetAs%20Player%20Movement%20Component (Variables|Default|GetAs%20BP%20First%20Person%20Character)) (Variables|Default|GetIsShooting))
  (Variables|Default|GetIsShooting
    (:then
      (Networking|SwitchHasAuthority
        (:Remote
          (if (Pawn|IsLocallyControlled _as_bp_first_person_character)
            (Default|StartRecall _as_bp_first_person_character (Variables|Default|GetShootFired))))))
    (:else)))

(fn ReadDataAsset
  (bind _dataasset (Variables|Default|GetDataAsset))
  (Variables|PasTouche|SetBaseDamage (Variables|/Script/Override.WeaponComponentStats|GetBaseDamage _dataasset))
  (Variables|PasTouche|SetReducedDamage (Variables|/Script/Override.WeaponComponentStats|GetReducedDamage _dataasset))
  (Variables|PasTouche|SetMunitionRecallTime (Variables|/Script/Override.WeaponComponentStats|GetMunitionRecallTime _dataasset))
  (Variables|PasTouche|SetMaxMunition%20 (Variables|/Script/Override.WeaponComponentStats|GetMaxMunition _dataasset))
  (Variables|PasTouche|SetMaxRange (Variables|/Script/Override.WeaponComponentStats|GetMaxRange _dataasset))
  (Variables|PasTouche|SetRPM (Variables|/Script/Override.WeaponComponentStats|GetRPM _dataasset))
  (Variables|Default|SetCurrentMunition 1)
  (Variables|PasTouche|SetReload (Variables|/Script/Override.WeaponComponentStats|GetReload _dataasset)))

(fn LineTrace
  (params (Start :type Vector) (End :type Vector))
  (bind (_outhit _returnvalue) (Collision|LineTraceForObjects Start End (Utilities|Array|MakeArray "ObjectTypeQuery1" "ObjectTypeQuery7") false 0 "None"))
  (return _outhit _returnvalue))