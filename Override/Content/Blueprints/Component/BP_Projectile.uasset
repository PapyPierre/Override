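; BP_Projectile is a weapon projectile actor that detects hits on the server.
; BeginPlay sets a lifespan and seeds the last position from the weapon's start point.
; Each tick traces between last and current positions, ignoring the shooter, to cover the gap between frames.
; A sphere trace decides the hit, but a separate line trace supplies the result to CallPlayerHit, after which ticking stops and the projectile soon expires.
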(event EventBeginPlay
  (Networking|SwitchHasAuthority
    (:Authority
      (Actor|SetLifeSpan 7.0)
      (Variables|Default|SetLastPosition (Variables|/Game/Blueprints/Component/AC_Weapon.AC_Weapon_C|GetStartProjectile (Variables|Default|GetWeapon))))))

(event EventTick
  (params (DeltaSeconds :type Float%20%28single-precision%29))
  (bind _array (Utilities|Array|MakeArray "ObjectTypeQuery7" "ObjectTypeQuery1"))
  (bind _weapon (Variables|Default|GetWeapon))
  (bind _as_bp_first_person_character (Variables|/Game/Blueprints/Component/AC_Weapon.AC_Weapon_C|GetAs%20BP%20First%20Person%20Character _weapon))
  (bind _array_2 (Utilities|Array|MakeArray _as_bp_first_person_character))
  (Networking|SwitchHasAuthority
    (:Authority
      (bind _output_get (Variables|Default|SetCurrentPosition (Transformation|GetActorLocation)))
      (bind _returnvalue (Collision|SphereTraceForObjects _output_get (Variables|Default|GetLastPosition) 1e+01 _array false _array_2 "None"))
      (bind _outhit (Collision|LineTraceForObjects (Variables|Default|GetLastPosition) _output_get _array false _array_2 "None" true "(R=1.000000,G=0.000000,B=0.000000,A=1.000000)" "(R=0.000000,G=0.192623,B=1.000000,A=1.000000)"))
      (if _returnvalue
        (Default|CallPlayerHit _outhit)
        (Actor|Tick|SetActorTickEnabled false)
        (Actor|SetLifeSpan 0.1)
        (else
          (Variables|Default|SetLastPosition (Transformation|GetActorLocation)))))))

(fn ConstructionScript)