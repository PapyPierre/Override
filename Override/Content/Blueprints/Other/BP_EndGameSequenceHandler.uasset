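; BP_EndGameSequenceHandler dresses the end-game scene in the winning team's look, driven by WinnerID.
; InitializeSequence recolors lights, swaps poster and tatami materials, sets the Niagara flame's ColorID, blacks out neons, stops the flame and shows the end-game widget.
; Separate functions relight neons individually or all at once, activate the flame and remove the UI.
; The event graph is empty, so nothing here calls these functions.
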(event EventBeginPlay)

(event Collision|EventActorBeginOverlap
  (params (OtherActor :type Actor%20Object%20Reference)))

(event EventTick
  (params (DeltaSeconds :type Float%20%28single-precision%29)))

(fn ConstructionScript)

(fn GetWinnerColor
  (return (Utilities|Array|Get(acopy) (Variables|Default|GetTeamColors) (Variables|Default|GetWinnerID))))

(fn InitializeSequence
  (Neons|ChangeLightsColors)
  (Neons|TurnOffNeons)
  (Poster|ChangePosterMat)
  (Tatami|ChangeTatamiMat)
  (Flame|ChangeFlameColor)
  (Flame|DeactivateFlame)
  (UI|DisplayUI))

(fn ChangeLightsColors
  (for _array_element (Variables|Default|GetLights)
    (bind _winnercolor (Helpers|GetWinnerColor))
    (Rendering|Components|Light|SetLightColor (Variables|/Script/Engine.Light|GetLightComponent _array_element) (Math|Conversions|ToLinearColor(Color) _winnercolor) true)))

(fn LightAllNeons
  (for _array_element (Variables|Default|GetNeons)
    (Rendering|Material|SetMaterial (Variables|/Script/Engine.StaticMeshActor|GetStaticMeshComponent _array_element) 0 (Utilities|Array|Get(acopy) (Variables|Default|GetNeonMaterials) (Variables|Default|GetWinnerID)))))

(fn TurnOffNeons
  (for _array_element (Variables|Default|GetNeons)
    (Rendering|Material|SetMaterial (Variables|/Script/Engine.StaticMeshActor|GetStaticMeshComponent _array_element) 0 "/Game/Art/Materials/Inst/MI_T_EmissiveNeon_Black.MI_T_EmissiveNeon_Black")))

(fn ChangeTatamiMat
  (Rendering|Material|SetMaterial (Variables|/Script/Engine.StaticMeshActor|GetStaticMeshComponent (Variables|Default|GetTatami)) 1 (Utilities|Array|Get(acopy) (Variables|Default|GetTatamiMaterials) (Variables|Default|GetWinnerID))))

(fn ChangePosterMat
  (Rendering|Material|SetMaterial (Variables|/Script/Engine.StaticMeshActor|GetStaticMeshComponent (Variables|Default|GetPoster)) 2 (Utilities|Array|Get(acopy) (Variables|Default|GetPosterMaterials) (Variables|Default|GetWinnerID))))

(fn ChangeFlameColor
  (Effects|Components|ParticleSystem|SetFloatParameter (Variables|/Script/Niagara.NiagaraActor|GetNiagaraComponent (Variables|Default|GetFlameNiagara)) "ColorID" (Math|Conversions|ToFloat(Integer) (+ (Variables|Default|GetWinnerID) 1))))

(fn ActivateFlame
  (bind _flameniagara (Variables|Default|GetFlameNiagara))
  (bind _niagaracomponent (Variables|/Script/Niagara.NiagaraActor|GetNiagaraComponent _flameniagara))
  (Components|Activation|SetAutoActivate _niagaracomponent true)
  (Components|Activation|Activate _niagaracomponent true))

(fn DeactivateFlame
  (bind _flameniagara (Variables|Default|GetFlameNiagara))
  (bind _niagaracomponent (Variables|/Script/Niagara.NiagaraActor|GetNiagaraComponent _flameniagara))
  (Components|Activation|SetAutoActivate _niagaracomponent false)
  (Components|Activation|Deactivate _niagaracomponent))

(fn LightNeonbyIndex
  (params (Index :type Integer))
  (Rendering|Material|SetMaterial (Variables|/Script/Engine.StaticMeshActor|GetStaticMeshComponent (Utilities|Array|Get(acopy) (Variables|Default|GetNeons) Index)) 0 (Utilities|Array|Get(acopy) (Variables|Default|GetNeonMaterials) (Variables|Default|GetWinnerID))))

(fn DisplayUI
  (bind _returnvalue (UserInterface|CreateWidget (Variables|Default|GetEndGameWidgetClass)))
  (bind _output_get (Variables|Default|SetEndGameWidget _returnvalue))
  (UserInterface|Viewport|AddtoViewport _output_get 0))

(fn RemoveUI
  (Widget|RemovefromParent (Variables|Default|GetEndGameWidget)))