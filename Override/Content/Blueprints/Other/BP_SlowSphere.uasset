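; BP_SlowSphere is a timed slow-bubble skill area that slows first-person characters inside it, except those in IgnoredActors.
; Overlap begin and end toggle the movement component's IsSlowed flag and the slowed HUD effect.
; StartLife sets the Niagara lifetime, enables overlaps a tick later, and plays start and end sounds via RPC before destroying the actor.
; On remotes, Niagara color depends on the first ignored character's team relative to the local player's.
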(event Custom|StartLife
  (params (Lifetime :type Float%20%28double-precision%29))
  (Niagara|SetNiagaraVariable(Float) (Variables|Default|GetNiagara) "Lifetime" (- Lifetime 0.5))
  ;[0.15 1 0.15 0.5] SFX Slow Start
  (CallFunction|RPCSoundSlow false)
  (Utilities|FlowControl|DelayUntilNextTick)
  (Variables|/Script/Engine.PrimitiveComponent|SetbGenerateOverlapEvents (Variables|Default|GetSphere1) true)
  (Utilities|FlowControl|Delay Lifetime)
  ;[0.15 1 0.15 0.5] SFX Slow End
  (CallFunction|RPCSoundSlow true))

(event Custom|RPC_SoundSlow
  (params (End :type Boolean))
  ;[0.15 1 0.15 0.5] SFX Slow Cast + End
  (Networking|SwitchHasAuthority
    (:Authority
      _)
    (:Remote
      (Class|FMODBlueprintStatics|PlayEventatLocation (select End "/Game/FMOD/Events/SFX_FOLDER/SFX/Skills/Bubble/SKILLS_SlowBubbleEnd.SKILLS_SlowBubbleEnd" "/Game/FMOD/Events/SFX_FOLDER/SFX/Skills/Bubble/SKILLS_SlowBubbleStart.SKILLS_SlowBubbleStart") (Transformation|GetActorTransform))))
  (if End
    (Utilities|FlowControl|DelayUntilNextTick)
    (Actor|DestroyActor)))

(event EventBeginPlay
  (bind _ignoredactors (Variables|Default|GetIgnoredActors))
  (bind _output (Utilities|Array|Get(acopy) _ignoredactors))
  (bind _asbp_first_person_character (Utilities|Casting|CastToBP_FirstPersonCharacter _output))
  (bind _playerstate (Variables|/Script/Engine.Pawn|GetPlayerState _asbp_first_person_character))
  (bind _asbp_custom_player_state (Utilities|Casting|CastToBP_CustomPlayerState _playerstate))
  (bind _teamindex (Variables|/Game/Blueprints/Player/BP_CustomPlayerState.BP_CustomPlayerState_C|GetTeamIndex _asbp_custom_player_state))
  (Networking|SwitchHasAuthority
    (:Remote
      (Niagara|SetNiagaraVariable(Float) (Variables|Default|GetNiagara) "ColorID" (Utilities|Select :Index (Variables|/Game/Blueprints/Controller/BP_FirstPersonPlayerController.BP_FirstPersonPlayerController_C|GetTeamIndex (.AsBP%20First%20Person%20Player%20Controller (Utilities|Casting|CastToBP_FirstPersonPlayerController (Game|GetPlayerController 0)))) :Option%200 (Utilities|Select :Index _teamindex :Option%200 1.0 :Option%201 2.0 :Option%202 3.0) :Option%201 (Utilities|Select :Index _teamindex :Option%200 2.0 :Option%201 1.0 :Option%202 3.0) :Option%202 (Utilities|Select :Index _teamindex :Option%200 2.0 :Option%201 3.0 :Option%202 1.0)))
      (Niagara|SetNiagaraVariable(Float) (Variables|Default|GetNiagara) "Scale" (* 0.2 (.x (Transformation|GetWorldScale (Variables|Default|GetDefaultSceneRoot))))))))

(event Collision|EventActorBeginOverlap
  (params (OtherActor :type Actor%20Object%20Reference))
  (bind _asbp_first_person_character (Utilities|Casting|CastToBP_FirstPersonCharacter OtherActor))
  (if (not (Utilities|Array|ContainsItem (Variables|Default|GetIgnoredActors) _asbp_first_person_character))
    (Variables|/Script/Override.PlayerMovementComponent|SetIsSlowed (Variables|/Script/Override.PlayerCharacter|GetPlayerMovementComponent _asbp_first_person_character) true)
    (Default|AddVFXHUD _asbp_first_person_character 0.0 1.0 1.0 true (Utilities|Name|MakeLiteralName "PPI_HudSlowed"))))

(event Collision|EventActorEndOverlap
  (params (OtherActor :type Actor%20Object%20Reference))
  (bind _asbp_first_person_character (Utilities|Casting|CastToBP_FirstPersonCharacter OtherActor))
  (if (not (Utilities|Array|ContainsItem (Variables|Default|GetIgnoredActors) _asbp_first_person_character))
    (Variables|/Script/Override.PlayerMovementComponent|SetIsSlowed (Variables|/Script/Override.PlayerCharacter|GetPlayerMovementComponent _asbp_first_person_character) false)
    (Default|AddVFXHUD _asbp_first_person_character 1.0 0.0 1.0 false (Utilities|Name|MakeLiteralName "PPI_HudSlowed"))))

(fn ConstructionScript)