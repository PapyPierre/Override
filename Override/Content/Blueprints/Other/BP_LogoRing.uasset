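; BP_LogoRing is a logo ring Blueprint that gives its three static meshes a shared logo material at runtime.
; On BeginPlay it collects the meshes into an array and loops over them.
; The first pass creates a dynamic instance of MI_LOGO when none is valid, and later passes assign that same instance to material slot 0.
; The construction script is empty, and no material parameters are changed.
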(event EventBeginPlay
  (bind _meshes (Variables|Default|GetMeshes))
  (Utilities|Array|Add _meshes (Variables|Default|GetStaticMesh))
  (Utilities|Array|Add _meshes (Variables|Default|GetStaticMesh1))
  (Utilities|Array|Add _meshes (Variables|Default|GetStaticMesh2))
  (for _array_element (Variables|Default|GetMeshes)
    (bind _mid (Variables|Default|GetMID)
      (:then
        (Rendering|Material|SetMaterial _array_element 0 _mid))
      (:else
        (bind _returnvalue (Rendering|Material|CreateDynamicMaterialInstance _array_element 0 "/Game/Art/Materials/VFX/Skybox/ToCode/MI_LOGO.MI_LOGO" "None" :!class /Script/Engine.PrimitiveComponent))
        (Variables|Default|SetMID _returnvalue)))))

(fn ConstructionScript)