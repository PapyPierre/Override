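; BP_DeathZone is a trigger volume that kills any player character entering its box.
; On server-side overlap with a BP_FirstPersonCharacter, it gets the ability system component from the character's custom player state.
; It applies GE_Health_SetByCallerDamage to that component with a huge Data.Damage set-by-caller magnitude, so death comes through GAS damage rather than a direct kill call.
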(event OnComponentBeginOverlap(Box)
  (params (OverlappedComponent :type Primitive%20Component%20Object%20Reference) (OtherActor :type Actor%20Object%20Reference) (OtherComp :type Primitive%20Component%20Object%20Reference) (OtherBodyIndex :type Integer) (bFromSweep :type Boolean) (SweepResult :type Hit%20Result%20Structure%20%28by%20ref%29))
  (Networking|SwitchHasAuthority
    (:Authority
      (if (== (Utilities|GetClass OtherActor) "/Game/Blueprints/Player/BP_FirstPersonCharacter.BP_FirstPersonCharacter_C")
        (bind _asbp_first_person_character (Utilities|Casting|CastToBP_FirstPersonCharacter OtherActor))
        (bind _returnvalue (Ability|GameplayEffect|AssignTagSetbyCallerMagnitude (GameplayEffects|MakeOutgoingSpec :self (Variables|/Script/Override.CustomPlayerState|GetAsc (Class|PlayerCharacter|GetCustomPlayerState _asbp_first_person_character)) :GameplayEffectClass "/Game/Blueprints/GAS/GameplayEffects/GE_Health_SetByCallerDamage.GE_Health_SetByCallerDamage_C" :Level 1.0) "(TagName=\"Data.Damage\")" 1e+10))
        (GameplayEffects|ApplyGameplayEffectSpecToSelf (Variables|/Script/Override.CustomPlayerState|GetAsc (Class|PlayerCharacter|GetCustomPlayerState _asbp_first_person_character)) _returnvalue)
        (GameplayAttributes|GetAttributeSet (Variables|/Script/Override.CustomPlayerState|GetAsc (Class|PlayerCharacter|GetCustomPlayerState _asbp_first_person_character)) "/Script/Override.HealthAttributeSet")))))

(event EventBeginPlay)

(event Collision|EventActorBeginOverlap
  (params (OtherActor :type Actor%20Object%20Reference)))

(event EventTick
  (params (DeltaSeconds :type Float%20%28single-precision%29)))

(fn ConstructionScript)