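; Arena crowd manager that drives the audience ring's visuals and sound from replicated state.
; Hype, Ola and Pulse RepNotifies set ring material parameters and fire crowd cheers at sound sources, then fade via timelines after a retriggerable delay.
; Team color is multicast and remapped relative to each client's local team.
; Alert lights the logo ring and plays last-minute announcer lines, while state-based crowd ambience runs on clients only.
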(event Custom|DecreasePulse
  (Rendering|Material|SetScalarParameterValue (Variables|/Game/Blueprints/Other/BP_PublicRing.BP_PublicRing_C|GetMID (Variables|Default|GetPublic%20Ring)) "Pulse" (Variables|Default|GetPulse) :!class /Script/Engine.MaterialInstanceDynamic)
  (CallFunction|CrowdCheers)
  (Utilities|FlowControl|RetriggerableDelay 3.0)
  (bind _slowdecrease (Timeline|Timeline_0 PlayFromStart)
    (:Update
      (Rendering|Material|SetScalarParameterValue (Variables|/Game/Blueprints/Other/BP_PublicRing.BP_PublicRing_C|GetMID (Variables|Default|GetPublic%20Ring)) "Pulse" (* (Variables|Default|GetPulse) _slowdecrease) :!class /Script/Engine.MaterialInstanceDynamic))
    (:Finished
      (Variables|Default|SetPulse 0.0))))

(event Custom|Multicast_TeamColor
  (params (Team :type Integer))
  (bind _public_ring (Variables|Default|GetPublic%20Ring))
  (bind _public_ring_2 (Variables|Default|GetPublic%20Ring))
  (bind _mid (Variables|/Game/Blueprints/Other/BP_PublicRing.BP_PublicRing_C|GetMID _public_ring))
  (bind _mid_2 (Variables|/Game/Blueprints/Other/BP_PublicRing.BP_PublicRing_C|GetMID _public_ring_2))
  (Networking|SwitchHasAuthority
    (:Remote
      (Rendering|Material|SetScalarParameterValue _mid "BlueTeamColor" 0.0 :!class /Script/Engine.MaterialInstanceDynamic)
      (Rendering|Material|SetScalarParameterValue _mid "RedTeamColor" 0.0 :!class /Script/Engine.MaterialInstanceDynamic)
      (Rendering|Material|SetScalarParameterValue _mid "OrangeTeamColor" 0.0 :!class /Script/Engine.MaterialInstanceDynamic)
      (if (!= Team -1)
        (bind _asbp_first_person_player_controller (Utilities|Casting|CastToBP_FirstPersonPlayerController (Game|GetPlayerController 0)))
        (switch int (Utilities|Select :Index (Variables|/Game/Blueprints/Controller/BP_FirstPersonPlayerController.BP_FirstPersonPlayerController_C|GetTeamIndex _asbp_first_person_player_controller) :Option%200 (Utilities|Select :Index Team :Option%200 0 :Option%201 1 :Option%202 2) :Option%201 (Utilities|Select :Index Team :Option%200 1 :Option%201 0 :Option%202 2) :Option%202 (Utilities|Select :Index Team :Option%200 1 :Option%201 2 :Option%202 0))
          (:0
            (Rendering|Material|SetScalarParameterValue _mid_2 "BlueTeamColor" 1.0 :!class /Script/Engine.MaterialInstanceDynamic))
          (:1
            (Rendering|Material|SetScalarParameterValue _mid_2 "RedTeamColor" 1.0 :!class /Script/Engine.MaterialInstanceDynamic))
          (:2
            (Rendering|Material|SetScalarParameterValue _mid_2 "OrangeTeamColor" 1.0 :!class /Script/Engine.MaterialInstanceDynamic)))))))

(event Custom|HypeDecrease
  (Rendering|Material|SetScalarParameterValue (Variables|/Game/Blueprints/Other/BP_PublicRing.BP_PublicRing_C|GetMID (Variables|Default|GetPublic%20Ring)) "Hype" (Variables|Default|GetHype) :!class /Script/Engine.MaterialInstanceDynamic)
  (CallFunction|CrowdCheers)
  (Utilities|FlowControl|RetriggerableDelay 3.0)
  (bind _slowdecrease (Timeline|SlowDecrease PlayFromStart)
    (:Update
      (Rendering|Material|SetScalarParameterValue (Variables|/Game/Blueprints/Other/BP_PublicRing.BP_PublicRing_C|GetMID (Variables|Default|GetPublic%20Ring)) "Hype" (* (Variables|Default|GetHype) _slowdecrease) :!class /Script/Engine.MaterialInstanceDynamic))
    (:Finished
      (Variables|Default|SetHype 0.0))))

(event Custom|RPC_AMB_Crowd
  (params (NewState :type Integer))
  ;[0.15 1 0.15 0.5] SFX Crowd Ambience
  (Networking|SwitchHasAuthority
    (:Remote
      (CallFunction|StartCrowdAmbience NewState))))

(event Custom|HolaDecrease
  (Rendering|Material|SetScalarParameterValue (Variables|/Game/Blueprints/Other/BP_PublicRing.BP_PublicRing_C|GetMID (Variables|Default|GetPublic%20Ring)) "Hola" (Variables|Default|GetOla) :!class /Script/Engine.MaterialInstanceDynamic)
  (CallFunction|CrowdCheers)
  (Utilities|FlowControl|RetriggerableDelay 3.0)
  (bind _slowdecrease (Timeline|Timeline PlayFromStart)
    (:Update
      (Rendering|Material|SetScalarParameterValue (Variables|/Game/Blueprints/Other/BP_PublicRing.BP_PublicRing_C|GetMID (Variables|Default|GetPublic%20Ring)) "Hola" (* (Variables|Default|GetOla) _slowdecrease) :!class /Script/Engine.MaterialInstanceDynamic))
    (:Finished
      (Variables|Default|SetOla 0.0))))

(event EventBeginPlay
  ;[0.15 1 0.15 0.5] SFX Crowd Ambience
  (Networking|SwitchHasAuthority
    (:Remote
      (bind _outactors (Actor|GetAllActorsOfClass "/Game/Blueprints/Other/PublicSoundSource.PublicSoundSource_C"))
      (Variables|Default|SetPublicSoundSources _outactors)
      (CallFunction|StartCrowdAmbience))))

(event EventEndPlay
  (params (EndPlayReason :type EEndPlayReason%20Enum :default "Destroyed"))
  ;[0.15 0.15 0.15 0.5] Ambience Stop On Destroy
  (Class|FMODBlueprintStatics|EventInstanceStop (Variables|Default|GetPublicAmbience) true))

(fn ConstructionScript)

(fn SetHype
  (params (NewHype :type Float%20%28double-precision%29))
  (Variables|Default|SetHype NewHype))

(fn SetOla
  (params (Value :type Float%20%28double-precision%29))
  (Variables|Default|SetOla Value))

(fn SetColor
  (params (Team :type Integer))
  (CallFunction|MulticastTeamColor Team))

(fn SetAlert
  (params (Value :type Float%20%28double-precision%29))
  (Variables|Default|GetInAlert
    (:then)
    (:else
      (Variables|Default|SetAlert Value)
      (Variables|Default|SetInAlert true))))

(fn SetPulse
  (params (Value :type Float%20%28double-precision%29))
  (Variables|Default|SetPulse Value))

(fn OnRepHype
  (if (!= (Variables|Default|GetHype) 0.0)
    (CallFunction|HypeDecrease)))

(fn OnRepOla
  (if (!= (Variables|Default|GetOla) 0.0)
    (CallFunction|HolaDecrease)))

(fn OnRepPulse
  (if (!= (Variables|Default|GetPulse) 0.0)
    (CallFunction|DecreasePulse)))

(fn OnRepAlert
  (Rendering|Material|SetScalarParameterValue (Variables|/Game/Blueprints/Other/BP_LogoRing.BP_LogoRing_C|GetMID (Variables|Default|GetLogo%20Ring)) "AlertLerp" 1.0 :!class /Script/Engine.MaterialInstanceDynamic)
  (Networking|SwitchHasAuthority
    (:Remote
      ;[0.15 1 0.15 0.5] SFX Announcer LastMinuteRemaining
      (bind _asbp_game_state (Utilities|Casting|CastToBP_GameState (Game|GetGameState)))
      (bind _teamsorted1 (Default|GetWinner _asbp_game_state))
      (Default|PlayAnnouncerEvent _asbp_game_state (select (== (.databanked (Utilities|Array|Get(acopy) _teamsorted1)) (.databanked (Utilities|Array|Get(acopy) _teamsorted1 1))) "/Game/FMOD/Events/SFX_FOLDER/VOICES/VOC_LastMinuteEquity.VOC_LastMinuteEquity" "/Game/FMOD/Events/SFX_FOLDER/VOICES/VOC_LastMinuteLead.VOC_LastMinuteLead") true true (Variables|/Game/Blueprints/Controller/BP_FirstPersonPlayerController.BP_FirstPersonPlayerController_C|GetTeamIndex (Utilities|Array|Get(acopy) (.player (Utilities|Array|Get(acopy) _teamsorted1))))))))

(fn CrowdCheers
  (for _array_element (Variables|Default|GetPublicSoundSources)
    (Class|FMODBlueprintStatics|PlayEventAttached "/Game/FMOD/Events/SFX_FOLDER/AMBIENCE/Rfx/RFX_CrowdImpact.RFX_CrowdImpact" (Variables|/Game/Blueprints/Other/PublicSoundSource.PublicSoundSource_C|GetDefaultSceneRoot _array_element) "None" "0, 0, 0" "KeepRelativeOffset")
    (Class|FMODBlueprintStatics|PlayEventAttached "/Game/FMOD/Events/SFX_FOLDER/SFX/Gamemode/SFX_Crowd_Cheer_Gun.SFX_Crowd_Cheer_Gun" (Variables|/Game/Blueprints/Other/PublicSoundSource.PublicSoundSource_C|GetDefaultSceneRoot _array_element) "None" "0, 0, 0" "KeepRelativeOffset")))

(fn StartCrowdAmbience
  (params (NewState :type Integer))
  (bind _returnvalue (Class|FMODBlueprintStatics|EventInstanceIsValid (Variables|Default|GetPublicAmbience)))
  (if _returnvalue
    (Class|FMODBlueprintStatics|EventInstanceStop (Variables|Default|GetPublicAmbience) true))
  (bind _returnvalue_2 (Class|FMODBlueprintStatics|PlayEvent2D (Utilities|Select :Index NewState :Option%200 "/Game/FMOD/Events/SFX_FOLDER/AMBIENCE/Beds/BEDS_Enter_Players.BEDS_Enter_Players" :Option%201 "/Game/FMOD/Events/SFX_FOLDER/AMBIENCE/Beds/BEDS_Crowd_General.BEDS_Crowd_General" :Option%202 "/Game/FMOD/Events/SFX_FOLDER/AMBIENCE/Beds/BEDS_Finish_Game.BEDS_Finish_Game")))
  (Variables|Default|SetPublicAmbience _returnvalue_2))