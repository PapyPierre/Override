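; BP_Critical is an interactable trigger that fires sample HUD feedback when the first-person character overlaps its Collision component, apparently for testing.
; It reaches the HUD through the character's PlayerController and pushes hardcoded penalty and bonus entries, one with placeholder text, to the score feed.
; It also plays the crosshair's critical-hit animation and changes the Flamme gamemode widget's B and C states.
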(event OnComponentBeginOverlap(Collision)
  (params (OverlappedComponent :type Primitive%20Component%20Object%20Reference) (OtherActor :type Actor%20Object%20Reference) (OtherComp :type Primitive%20Component%20Object%20Reference) (OtherBodyIndex :type Integer) (bFromSweep :type Boolean) (SweepResult :type Hit%20Result%20Structure%20%28by%20ref%29))
  (bind _asbp_first_person_character (Utilities|Casting|CastToBP_FirstPersonCharacter OtherActor))
  (Default|ScoreEntrySpawn (Variables|/Game/Blueprints/Widget/WBP_HUD.WBP_HUD_C|GetWBP_ScoreFeedContainer (Variables|/Game/Blueprints/Controller/BP_FirstPersonPlayerController.BP_FirstPersonPlayerController_C|GetHUD (Variables|/Game/Blueprints/Player/BP_FirstPersonCharacter.BP_FirstPersonCharacter_C|GetPlayer%20Controller _asbp_first_person_character))) "Player Killed" -2.5e+02)
  (Default|ScoreEntrySpawn (Variables|/Game/Blueprints/Widget/WBP_HUD.WBP_HUD_C|GetWBP_ScoreFeedContainer (Variables|/Game/Blueprints/Controller/BP_FirstPersonPlayerController.BP_FirstPersonPlayerController_C|GetHUD (Variables|/Game/Blueprints/Player/BP_FirstPersonCharacter.BP_FirstPersonCharacter_C|GetPlayer%20Controller _asbp_first_person_character))) "dgrdgrdgr" 1.2e+02)
  (UserInterface|Animation|PlayAnimation (Variables|/Game/Blueprints/Widget/WBP_HUD.WBP_HUD_C|GetWBP_Crosshair (Variables|/Game/Blueprints/Controller/BP_FirstPersonPlayerController.BP_FirstPersonPlayerController_C|GetHUD (Variables|/Game/Blueprints/Player/BP_FirstPersonCharacter.BP_FirstPersonCharacter_C|GetPlayer%20Controller _asbp_first_person_character))) (Variables|/Game/Blueprints/Widget/HUD/WBP_Crosshair.WBP_Crosshair_C|GetCriticalEnemyHit (Variables|/Game/Blueprints/Widget/WBP_HUD.WBP_HUD_C|GetWBP_Crosshair (Variables|/Game/Blueprints/Controller/BP_FirstPersonPlayerController.BP_FirstPersonPlayerController_C|GetHUD (Variables|/Game/Blueprints/Player/BP_FirstPersonCharacter.BP_FirstPersonCharacter_C|GetPlayer%20Controller _asbp_first_person_character)))) 0.0 1 "Forward" 1.0 false)
  (Default|SetInactiveB (Variables|/Game/Blueprints/Widget/WBP_HUD.WBP_HUD_C|GetWBP_GamemodeFlamme (Variables|/Game/Blueprints/Controller/BP_FirstPersonPlayerController.BP_FirstPersonPlayerController_C|GetHUD (Variables|/Game/Blueprints/Player/BP_FirstPersonCharacter.BP_FirstPersonCharacter_C|GetPlayer%20Controller _asbp_first_person_character))) (Math|Color|MakeColor 226 122 52 255))
  (Default|SetActiveC (Variables|/Game/Blueprints/Widget/WBP_HUD.WBP_HUD_C|GetWBP_GamemodeFlamme (Variables|/Game/Blueprints/Controller/BP_FirstPersonPlayerController.BP_FirstPersonPlayerController_C|GetHUD (Variables|/Game/Blueprints/Player/BP_FirstPersonCharacter.BP_FirstPersonCharacter_C|GetPlayer%20Controller _asbp_first_person_character))) 15.0))

(event EventBeginPlay)

(event Collision|EventActorBeginOverlap
  (params (OtherActor :type Actor%20Object%20Reference)))

(event EventTick
  (params (DeltaSeconds :type Float%20%28single-precision%29)))

(fn ConstructionScript)