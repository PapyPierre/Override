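; BP_Launcher is an interactable launch pad that throws the first-person character straight upward.
; Entering its Box trigger immediately launches the character with a fixed vertical velocity, overriding existing velocity.
; OnInteract gives a much weaker launch to everyone in PlayerInZone and prints a debug string.
; End overlap removes characters from that array, but nothing in these graphs adds to it.
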(event OnComponentBeginOverlap(Box)
  (params (OverlappedComponent :type Primitive%20Component%20Object%20Reference) (OtherActor :type Actor%20Object%20Reference) (OtherComp :type Primitive%20Component%20Object%20Reference) (OtherBodyIndex :type Integer) (bFromSweep :type Boolean) (SweepResult :type Hit%20Result%20Structure%20%28by%20ref%29))
  (bind _asbp_first_person_character (Utilities|Casting|CastToBP_FirstPersonCharacter OtherActor))
  (Character|LaunchCharacter _asbp_first_person_character "0.000000,0.000000,1000.000000" true true))

(event OnComponentEndOverlap(Box)
  (params (OverlappedComponent :type Primitive%20Component%20Object%20Reference) (OtherActor :type Actor%20Object%20Reference) (OtherComp :type Primitive%20Component%20Object%20Reference) (OtherBodyIndex :type Integer))
  (bind _asbp_first_person_character (Utilities|Casting|CastToBP_FirstPersonCharacter OtherActor))
  (Utilities|Array|RemoveItem (Variables|Default|GetPlayerInZone) _asbp_first_person_character))

(event EventBeginPlay)

(event Collision|EventActorBeginOverlap
  (params (OtherActor :type Actor%20Object%20Reference)))

(event EventTick
  (params (DeltaSeconds :type Float%20%28single-precision%29)))

(event EventOnInteract
  (params (InteractingActor :type Actor%20Object%20Reference))
  (for _array_element (Variables|Default|GetPlayerInZone)
    (Character|LaunchCharacter _array_element "0.000000,0.000000,100.000000" true true)
    (Development|PrintString "Hello")))

(fn ConstructionScript)