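; BP_Modulation is an interactable world object that applies its currently cast gameplay effect to players entering its box areas.
; Damage feeds a GAS health attribute with heal-over-time, and the object locks at zero health.
; Materials reflect targeting (shared across its group), locked or cooldown state, and a dematerialize hack that disables collision.
; A timed ping outlines the mesh through custom depth and a material parameter collection.
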(event Custom|BeginOverlap
  (params (OverlappedComponent :type Primitive%20Component%20Object%20Reference) (OtherActor :type Actor%20Object%20Reference) (OtherComp :type Primitive%20Component%20Object%20Reference) (OtherBodyIndex :type Integer) (bFromSweep :type Boolean) (SweepResult :type Hit%20Result%20Structure%20%28by%20ref%29))
  (bind _asbp_first_person_character (Utilities|Casting|CastToBP_FirstPersonCharacter OtherActor))
  (bind _currentlycastedge (Variables|Default|GetCurrentlyCastedGE))
  ;[0.15 0.15 0.15 0.5] Area Overlap Events
  (if (== (Utilities|GetClass OtherActor) "/Game/Blueprints/Player/BP_FirstPersonCharacter.BP_FirstPersonCharacter_C")
    (Utilities|Array|AddUnique (Variables|Default|GetPlayerInZone) _asbp_first_person_character)
    ;[0.15 0.15 0.15 0.5] Cast current GE on player enterting the area
    (if (Utilities|IsValidClass _currentlycastedge)
      (GameplayEffects|ApplyGameplayEffectToTarget :self (Variables|Default|GetAsc) :GameplayEffectClass _currentlycastedge :Target (Ability|GetAbilitySystemComponent _asbp_first_person_character)))))

(event Custom|OnTakeAnyDamage_Event
  (params (DamagedActor :type Actor%20Object%20Reference) (Damage :type Float%20%28single-precision%29) (DamageType :type Damage%20Type%20Object%20Reference) (InstigatedBy :type Controller%20Object%20Reference) (DamageCauser :type Actor%20Object%20Reference))
  (bind _asc (Variables|Default|GetAsc))
  ;[0.15 0.15 0.15 0.5] Take Damage
  (if (not (Utilities|Enum|Equal(Enum) (Variables|Default|GetCurrentState) "InCD"))
    (bind _returnvalue (Ability|GameplayEffect|AssignTagSetbyCallerMagnitude (GameplayEffects|MakeOutgoingSpec :self _asc :GameplayEffectClass "/Game/Blueprints/GAS/GameplayEffects/GE_Health_SetByCallerDamage.GE_Health_SetByCallerDamage_C" :Level 1.0) "(TagName=\"Data.Damage\")" Damage))
    (GameplayEffects|ApplyGameplayEffectSpecToSelf _asc _returnvalue)
    ;[0.15 0.15 0.15 0.5] Auto Heal Over Time
    (GameplayEffects|ApplyGameplayEffectToSelf :self _asc :GameplayEffectClass "/Game/Blueprints/GAS/GameplayEffects/GE_Health_Mod_HealOverTime.GE_Health_Mod_HealOverTime_C" :Level 1.0)))

(event Custom|CancelPing
  (bind _staticmesh (Variables|Default|GetStaticMesh))
  ;[0.15 0.15 0.15 0.5] Ping
  (Rendering|SetRenderCustomDepth _staticmesh false)
  (Rendering|SetCustomDepthStencilValue _staticmesh 0))

(event Custom|EndOverlap
  (params (OverlappedComponent :type Primitive%20Component%20Object%20Reference) (OtherActor :type Actor%20Object%20Reference) (OtherComp :type Primitive%20Component%20Object%20Reference) (OtherBodyIndex :type Integer))
  ;[0.15 0.15 0.15 0.5] Area Overlap Events
  (if (== (Utilities|GetClass OtherActor) "/Game/Blueprints/Player/BP_FirstPersonCharacter.BP_FirstPersonCharacter_C")
    (Utilities|Array|RemoveItem (Variables|Default|GetPlayerInZone) (.AsBP%20First%20Person%20Character (Utilities|Casting|CastToBP_FirstPersonCharacter OtherActor)))))

(event Custom|OnHealthChanged_Event
  (params (AttributeSet :type Attribute%20Set%20Object%20Reference) (OldValue :type Float%20%28single-precision%29) (NewValue :type Float%20%28single-precision%29))
  (if (<= NewValue 0.0)
    (Class|Modulation|Lock)))

(event Custom|Demat
  ;[0.15 0.15 0.15 0.5] Demat Hack
  (Collision|SetCollisionEnabled (Variables|Default|GetStaticMesh) "NoCollision")
  (Variables|Default|SetIsDemat true)
  (Development|PrintString "Demats")
  (CallFunction|SetMat (Variables|Default|GetDemat%20mat)))

(event Custom|Set%20Mat
  (params (Mat :type Material%20Object%20Reference))
  (Rendering|Material|SetMaterial (Variables|Default|GetStaticMesh) 0 Mat))

(event Custom|Remat
  ;[0.15 0.15 0.15 0.5] Demat Hack
  (Collision|SetCollisionEnabled (Variables|Default|GetStaticMesh) "QueryAndPhysics")
  (Variables|Default|SetIsDemat false)
  (Development|PrintString "remat")
  (CallFunction|SetMat (Variables|Default|GetDefault%20mat)))

(event EventStopPing
  (bind _staticmesh (Variables|Default|GetStaticMesh))
  ;[0.15 0.15 0.15 0.5] Ping
  (Rendering|SetRenderCustomDepth _staticmesh false)
  (Rendering|SetCustomDepthStencilValue _staticmesh 0))

(event EventPing
  (params (LifeTime :type Float%20%28single-precision%29))
  (bind _staticmesh (Variables|Default|GetStaticMesh))
  ;[0.15 0.15 0.15 0.5] Ping
  (Rendering|Material|SetVectorParameterValue "/Game/Art/Shader/Devs/PP_OutlineCollector.PP_OutlineCollector" "Color" (Math|Color|MakeColor 0.0 1.0 0.0) :!class /Script/Engine.KismetMaterialLibrary)
  (Rendering|SetRenderCustomDepth _staticmesh true)
  (Rendering|SetCustomDepthStencilValue _staticmesh 1)
  (Utilities|Time|SetTimerbyEvent (delegate Custom|CancelPing) LifeTime))

(event EventOnTarget
  (params (TargetingActor :type Actor%20Object%20Reference))
  (bind _group (Variables|Default|GetGroup))
  (bind _currentstate (Variables|Default|GetCurrentState))
  ;[0.15 0.15 0.15 0.5] Targeting
  (if (not (Variables|Default|GetIsDemat))
    (if (not (or (Utilities|Enum|Equal(Enum) _currentstate "Locked") (Utilities|Enum|Equal(Enum) _currentstate "InCD")))
      (Utilities|IsValid _group
        (:Is%20Valid
          (for _array_element (Variables|/Script/Override.ModulationGroup|GetModulationsInGroup _group)
            (bind _asbp_modulation (Utilities|Casting|CastToBP_Modulation _array_element))
            (CallFunction|SetMat _asbp_modulation (Variables|Default|GetTarget%20mat))))
        (:Is%20Not%20Valid
          (CallFunction|SetMat (Variables|Default|GetTarget%20mat)))))))

(event EventOnUntarget
  (bind _group (Variables|Default|GetGroup))
  (bind _currentstate (Variables|Default|GetCurrentState))
  ;[0.15 0.15 0.15 0.5] Targeting
  (if (not (Variables|Default|GetIsDemat))
    (if (not (or (Utilities|Enum|Equal(Enum) _currentstate "Locked") (Utilities|Enum|Equal(Enum) _currentstate "InCD")))
      (Utilities|IsValid _group
        (:Is%20Valid
          (for _array_element (Variables|/Script/Override.ModulationGroup|GetModulationsInGroup _group)
            (bind _asbp_modulation (Utilities|Casting|CastToBP_Modulation _array_element))
            (CallFunction|SetMat _asbp_modulation (Variables|Default|GetDefault%20mat))))
        (:Is%20Not%20Valid
          (CallFunction|SetMat (Variables|Default|GetDefault%20mat)))))))

(event EventOnStateChanged
  (params (NewState :type ModState%20Enum :default "Stopped"))
  (if (not (Variables|Default|GetIsDemat))
    (if (or (Utilities|Enum|Equal(Enum) NewState "Locked") (Utilities|Enum|Equal(Enum) NewState "InCD"))
      (CallFunction|SetMat (Variables|Default|GetLocked%20mat))
      (else
        (CallFunction|SetMat (Variables|Default|GetDefault%20mat))))))

(event EventBeginPlay
  ;[0.15 0.15 0.15 0.5] Area Overlap Events
  (for _array_element (Variables|Default|GetModulationsEffectMeshes)
    (Collision|BindEventtoOnComponentBeginOverlap _array_element (delegate Custom|BeginOverlap))
    (Collision|BindEventtoOnComponentEndOverlap _array_element (delegate Custom|EndOverlap))
    ;[0.15 0.15 0.15 0.5] Take Damage
    (EventDispatchers|AssignOnTakeAnyDamage (delegate Custom|OnTakeAnyDamage_Event))
    (bind _returnvalue (GameplayAttributes|GetAttributeSet (Variables|Default|GetAsc) "/Script/Override.HealthAttributeSet"))
    (EventDispatchers|AssignOnHealthChanged _returnvalue (delegate Custom|OnHealthChanged_Event))))

(fn ConstructionScript
  (|CallParentFunction)
  (Utilities|Array|Clear (Variables|Default|GetModulationsEffectMeshes))
  (for _array_element (Actor|GetComponentsByClass "/Script/Engine.BoxComponent")
    (Utilities|Array|AddUnique (Variables|Default|GetModulationsEffectMeshes) _array_element)))