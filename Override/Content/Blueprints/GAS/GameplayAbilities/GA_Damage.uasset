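; Gameplay ability that applies an AoE damage-over-time health effect to players through three targeting modes: free placement, modulation or single player.
; Free placement spawns a radius-scaled sphere with its own material, then applies the effect server-side to overlapped first-person characters.
; Modulation targeting hits players in the zone, calling EndAbility inside the loop; player targeting hits one.
; All modes target the character's custom PlayerState.
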(event EventOnFreePlacement
  (params (Point :type Vector :default "0, 0, 0"))
  (bind _free_placement_aoe_radius (Variables|Default|GetFree%20Placement%20Aoe%20Radius))
  (bind _returnvalue (Game|SpawnActorfromClass "/Game/Debug/UnitSphere.UnitSphere_C" (Math|Transform|MakeTransform Point "0, 0, 0" (Math|Conversions|ToVector(Float) (/ _free_placement_aoe_radius 5e+01))) "Undefined" "MultiplyWithRoot" 0 0))
  (Default|SetMat _returnvalue (Variables|Default|GetFree%20Placement%20Material))
  (bind _outactors (Collision|SphereOverlapActors Point _free_placement_aoe_radius (Utilities|Array|MakeArray "ObjectTypeQuery7") 0))
  (for _array_element _outactors
    (Ability|HasAuthority
      (:True
        (bind _asbp_first_person_character (Utilities|Casting|CastToBP_FirstPersonCharacter _array_element))
        (GameplayEffects|ApplyGameplayEffectToTarget (Ability|TargetData|AbilityTargetDatafromActor (Class|PlayerCharacter|GetCustomPlayerState _asbp_first_person_character)) "/Game/Blueprints/GAS/GameplayEffects/GE_Health_AoeDamageOverTime.GE_Health_AoeDamageOverTime_C" 1 1))))
  (Ability|EndAbility))

(event EventOnTargetModulation
  (params (Modulations :type BP%20Modulation%20Object%20Reference%20%28by%20ref%29))
  (for _array_element (Utilities|Array|MakeArray Modulations)
    (bind _asbp_modulation (Utilities|Casting|CastToBP_Modulation _array_element))
    (for _array_element_2 (Variables|/Game/Blueprints/Interactable/BP_Modulation.BP_Modulation_C|GetPlayerInZone _asbp_modulation)
      (GameplayEffects|ApplyGameplayEffectToTarget (Ability|TargetData|AbilityTargetDatafromActor (Class|PlayerCharacter|GetCustomPlayerState _array_element_2)) "/Game/Blueprints/GAS/GameplayEffects/GE_Health_AoeDamageOverTime.GE_Health_AoeDamageOverTime_C" 1 1)
      (Ability|EndAbility))
    (Ability|EndAbility)))

(event EventOnTargetPlayer
  (params (Player :type BP%20First%20Person%20Character%20Object%20Reference))
  (GameplayEffects|ApplyGameplayEffectToTarget (Ability|TargetData|AbilityTargetDatafromActor (Class|PlayerCharacter|GetCustomPlayerState Player)) "/Game/Blueprints/GAS/GameplayEffects/GE_Health_AoeDamageOverTime.GE_Health_AoeDamageOverTime_C" 1 1)
  (Ability|EndAbility))