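; GA_TP is a gameplay ability that teleports the owning player's first-person character to their teammate's location.
; Its target-player, target-modulation and free-placement events all share one path, which gets the pawn through the owning player state.
; If the teammate is waiting to respawn the ability ends without moving; otherwise it teleports with zero rotation, then ends.
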(event EventOnTargetPlayer
  (params (Player :type BP%20First%20Person%20Character%20Object%20Reference) (Point :type Vector :default "0, 0, 0"))
  (bind _asbp_custom_player_state (Utilities|Casting|CastToBP_CustomPlayerState (Ability|GetOwningActorfromActorInfo)))
  (bind _asbp_first_person_character (Utilities|Casting|CastToBP_FirstPersonCharacter (PlayerState|GetPawn _asbp_custom_player_state)))
  (if (Variables|/Game/Blueprints/Player/BP_FirstPersonCharacter.BP_FirstPersonCharacter_C|GetWaitingForRespawn (Variables|/Game/Blueprints/Player/BP_FirstPersonCharacter.BP_FirstPersonCharacter_C|GetTeamMateRef _asbp_first_person_character))
    (Ability|EndAbility)
    (else
      (Transformation|Teleport _asbp_first_person_character (Transformation|GetActorLocation (Variables|/Game/Blueprints/Player/BP_FirstPersonCharacter.BP_FirstPersonCharacter_C|GetTeamMateRef _asbp_first_person_character)) "0, 0, 0")
      (Ability|EndAbility))))

(event EventOnTargetModulation
  (params (Modulations :type BP%20Modulation%20Object%20Reference%20%28by%20ref%29) (Point :type Vector :default "0, 0, 0"))
  (bind _asbp_custom_player_state (Utilities|Casting|CastToBP_CustomPlayerState (Ability|GetOwningActorfromActorInfo)))
  (bind _asbp_first_person_character (Utilities|Casting|CastToBP_FirstPersonCharacter (PlayerState|GetPawn _asbp_custom_player_state)))
  (if (Variables|/Game/Blueprints/Player/BP_FirstPersonCharacter.BP_FirstPersonCharacter_C|GetWaitingForRespawn (Variables|/Game/Blueprints/Player/BP_FirstPersonCharacter.BP_FirstPersonCharacter_C|GetTeamMateRef _asbp_first_person_character))
    (Ability|EndAbility)
    (else
      (Transformation|Teleport _asbp_first_person_character (Transformation|GetActorLocation (Variables|/Game/Blueprints/Player/BP_FirstPersonCharacter.BP_FirstPersonCharacter_C|GetTeamMateRef _asbp_first_person_character)) "0, 0, 0")
      (Ability|EndAbility))))

(event EventOnFreePlacement
  (params (Point :type Vector :default "0, 0, 0"))
  (bind _asbp_custom_player_state (Utilities|Casting|CastToBP_CustomPlayerState (Ability|GetOwningActorfromActorInfo)))
  (bind _asbp_first_person_character (Utilities|Casting|CastToBP_FirstPersonCharacter (PlayerState|GetPawn _asbp_custom_player_state)))
  (if (Variables|/Game/Blueprints/Player/BP_FirstPersonCharacter.BP_FirstPersonCharacter_C|GetWaitingForRespawn (Variables|/Game/Blueprints/Player/BP_FirstPersonCharacter.BP_FirstPersonCharacter_C|GetTeamMateRef _asbp_first_person_character))
    (Ability|EndAbility)
    (else
      (Transformation|Teleport _asbp_first_person_character (Transformation|GetActorLocation (Variables|/Game/Blueprints/Player/BP_FirstPersonCharacter.BP_FirstPersonCharacter_C|GetTeamMateRef _asbp_first_person_character)) "0, 0, 0")
      (Ability|EndAbility))))