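; GA_Impulse is a gameplay ability that knocks first-person characters away from a target point, with optional area damage.
; Free-placement, target-modulation and target-player events all set the origin and share one path.
; That path spawns a translucent red sphere scaled to the radius, then sphere-overlaps for targets.
; On authority, it applies a damage GameplayEffect via each character's player state and launches them radially outward.
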(event EventOnFreePlacement
  (params (Point :type Vector :default "0, 0, 0"))
  (Variables|Default|SetOrigin Point)
  (bind _returnvalue (Game|SpawnActorfromClass "/Game/Blueprints/GAS/Debug/UnitSphere.UnitSphere_C" (Math|Transform|MakeTransform (Variables|Default|GetOrigin) "0, 0, 0" (Math|Conversions|ToVector(Float) (/ (Variables|Default|GetAoe%20Radius) 5e+01))) "Undefined" "MultiplyWithRoot" 0 0))
  (Default|SetMat _returnvalue "/Game/Art/Materials/Inst/Diorama/MI_T_RedTranslucent.MI_T_RedTranslucent")
  (bind _outactors (Collision|SphereOverlapActors (Variables|Default|GetOrigin) (Variables|Default|GetAoe%20Radius) (Utilities|Array|MakeArray "ObjectTypeQuery7") 0))
  (for _array_element _outactors
    (Ability|HasAuthority
      (:True
        (bind _asbp_first_person_character (Utilities|Casting|CastToBP_FirstPersonCharacter _array_element))
        (Utilities|FlowControl|Sequence
          (:then_0
            ;[0.15 0.15 0.15 0.5] Damage
            (if (Variables|Default|GetApplyDamage)
              (GameplayEffects|ApplyGameplayEffectToTarget (Ability|TargetData|AbilityTargetDatafromActor (Class|PlayerCharacter|GetCustomPlayerState _asbp_first_person_character)) "/Game/Blueprints/GAS/GameplayEffects/GE_Health_AoeDamage.GE_Health_AoeDamage_C" 1 1)))
          (:then_1
            ;[0.15 0.15 0.15 0.5] Impulse
            (Character|LaunchCharacter _asbp_first_person_character (* (Math|Vector|Normalize (- (Transformation|GetActorLocation _asbp_first_person_character) (Variables|Default|GetOrigin))) (Variables|Default|GetImpulse%20Force)) true true))))))
  (Ability|EndAbility))

(event EventOnTargetModulation
  (params (Modulations :type BP%20Modulation%20Object%20Reference%20%28by%20ref%29) (Point :type Vector :default "0, 0, 0"))
  (Variables|Default|SetOrigin Point)
  (bind _returnvalue (Game|SpawnActorfromClass "/Game/Blueprints/GAS/Debug/UnitSphere.UnitSphere_C" (Math|Transform|MakeTransform (Variables|Default|GetOrigin) "0, 0, 0" (Math|Conversions|ToVector(Float) (/ (Variables|Default|GetAoe%20Radius) 5e+01))) "Undefined" "MultiplyWithRoot" 0 0))
  (Default|SetMat _returnvalue "/Game/Art/Materials/Inst/Diorama/MI_T_RedTranslucent.MI_T_RedTranslucent")
  (bind _outactors (Collision|SphereOverlapActors (Variables|Default|GetOrigin) (Variables|Default|GetAoe%20Radius) (Utilities|Array|MakeArray "ObjectTypeQuery7") 0))
  (for _array_element _outactors
    (Ability|HasAuthority
      (:True
        (bind _asbp_first_person_character (Utilities|Casting|CastToBP_FirstPersonCharacter _array_element))
        (Utilities|FlowControl|Sequence
          (:then_0
            ;[0.15 0.15 0.15 0.5] Damage
            (if (Variables|Default|GetApplyDamage)
              (GameplayEffects|ApplyGameplayEffectToTarget (Ability|TargetData|AbilityTargetDatafromActor (Class|PlayerCharacter|GetCustomPlayerState _asbp_first_person_character)) "/Game/Blueprints/GAS/GameplayEffects/GE_Health_AoeDamage.GE_Health_AoeDamage_C" 1 1)))
          (:then_1
            ;[0.15 0.15 0.15 0.5] Impulse
            (Character|LaunchCharacter _asbp_first_person_character (* (Math|Vector|Normalize (- (Transformation|GetActorLocation _asbp_first_person_character) (Variables|Default|GetOrigin))) (Variables|Default|GetImpulse%20Force)) true true))))))
  (Ability|EndAbility))

(event EventOnTargetPlayer
  (params (Player :type BP%20First%20Person%20Character%20Object%20Reference) (Point :type Vector :default "0, 0, 0"))
  (Variables|Default|SetOrigin Point)
  (bind _returnvalue (Game|SpawnActorfromClass "/Game/Blueprints/GAS/Debug/UnitSphere.UnitSphere_C" (Math|Transform|MakeTransform (Variables|Default|GetOrigin) "0, 0, 0" (Math|Conversions|ToVector(Float) (/ (Variables|Default|GetAoe%20Radius) 5e+01))) "Undefined" "MultiplyWithRoot" 0 0))
  (Default|SetMat _returnvalue "/Game/Art/Materials/Inst/Diorama/MI_T_RedTranslucent.MI_T_RedTranslucent")
  (bind _outactors (Collision|SphereOverlapActors (Variables|Default|GetOrigin) (Variables|Default|GetAoe%20Radius) (Utilities|Array|MakeArray "ObjectTypeQuery7") 0))
  (for _array_element _outactors
    (Ability|HasAuthority
      (:True
        (bind _asbp_first_person_character (Utilities|Casting|CastToBP_FirstPersonCharacter _array_element))
        (Utilities|FlowControl|Sequence
          (:then_0
            ;[0.15 0.15 0.15 0.5] Damage
            (if (Variables|Default|GetApplyDamage)
              (GameplayEffects|ApplyGameplayEffectToTarget (Ability|TargetData|AbilityTargetDatafromActor (Class|PlayerCharacter|GetCustomPlayerState _asbp_first_person_character)) "/Game/Blueprints/GAS/GameplayEffects/GE_Health_AoeDamage.GE_Health_AoeDamage_C" 1 1)))
          (:then_1
            ;[0.15 0.15 0.15 0.5] Impulse
            (Character|LaunchCharacter _asbp_first_person_character (* (Math|Vector|Normalize (- (Transformation|GetActorLocation _asbp_first_person_character) (Variables|Default|GetOrigin))) (Variables|Default|GetImpulse%20Force)) true true))))))
  (Ability|EndAbility))