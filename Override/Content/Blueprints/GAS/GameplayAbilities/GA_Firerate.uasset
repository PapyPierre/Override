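; GA_Firerate is a gameplay ability that temporarily raises the weapon RPM of the owning player and, when close enough, their teammate.
; All three targeting events run the same logic, resolving the pawn from the owning PlayerState.
; A respawning or distant teammate means a solo bonus; otherwise both players get the ally bonus.
; After a delay it restores the owner's RPM, copies that value onto any boosted teammate, and ends.
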(event EventOnTargetPlayer
  (params (Player :type BP%20First%20Person%20Character%20Object%20Reference) (Point :type Vector :default "0, 0, 0"))
  (bind _asbp_custom_player_state (Utilities|Casting|CastToBP_CustomPlayerState (Ability|GetOwningActorfromActorInfo)))
  (bind _asbp_first_person_character (Utilities|Casting|CastToBP_FirstPersonCharacter (PlayerState|GetPawn _asbp_custom_player_state)))
  (Variables|Default|SetOriginRPM (Variables|/Game/Blueprints/Component/AC_Weapon.AC_Weapon_C|GetRPM (Variables|/Game/Blueprints/Player/BP_FirstPersonCharacter.BP_FirstPersonCharacter_C|GetAC_WeaponComponent _asbp_first_person_character)))
  (if (or (Variables|/Game/Blueprints/Player/BP_FirstPersonCharacter.BP_FirstPersonCharacter_C|GetWaitingForRespawn (Variables|/Game/Blueprints/Player/BP_FirstPersonCharacter.BP_FirstPersonCharacter_C|GetTeamMateRef _asbp_first_person_character)) (> (Math|Vector|Distance(Vector) (Transformation|GetActorLocation (Variables|/Game/Blueprints/Player/BP_FirstPersonCharacter.BP_FirstPersonCharacter_C|GetTeamMateRef _asbp_first_person_character)) (Transformation|GetActorLocation _asbp_first_person_character)) (Variables|Default|GetDistToAlly)))
    (Variables|/Game/Blueprints/Component/AC_Weapon.AC_Weapon_C|SetRPM (Variables|/Game/Blueprints/Player/BP_FirstPersonCharacter.BP_FirstPersonCharacter_C|GetAC_WeaponComponent _asbp_first_person_character) (+ (Variables|Default|GetOriginRPM) (Variables|Default|GetSoloBonus)))
    (Utilities|FlowControl|Delay (Variables|Default|GetEffectDuration))
    (Variables|/Game/Blueprints/Component/AC_Weapon.AC_Weapon_C|SetRPM (Variables|/Game/Blueprints/Player/BP_FirstPersonCharacter.BP_FirstPersonCharacter_C|GetAC_WeaponComponent _asbp_first_person_character) (Variables|Default|GetOriginRPM))
    (else
      (bind _output_get (Variables|/Game/Blueprints/Component/AC_Weapon.AC_Weapon_C|SetRPM (Variables|/Game/Blueprints/Player/BP_FirstPersonCharacter.BP_FirstPersonCharacter_C|GetAC_WeaponComponent _asbp_first_person_character) (+ (Variables|Default|GetOriginRPM) (Variables|Default|GetWithAllyBonus))))
      (Variables|/Game/Blueprints/Component/AC_Weapon.AC_Weapon_C|SetRPM (Variables|/Game/Blueprints/Player/BP_FirstPersonCharacter.BP_FirstPersonCharacter_C|GetAC_WeaponComponent (Variables|/Game/Blueprints/Player/BP_FirstPersonCharacter.BP_FirstPersonCharacter_C|GetTeamMateRef _asbp_first_person_character)) _output_get)
      (Utilities|FlowControl|Delay (Variables|Default|GetEffectDuration))
      (bind _output_get_2 (Variables|/Game/Blueprints/Component/AC_Weapon.AC_Weapon_C|SetRPM (Variables|/Game/Blueprints/Player/BP_FirstPersonCharacter.BP_FirstPersonCharacter_C|GetAC_WeaponComponent _asbp_first_person_character) (Variables|Default|GetOriginRPM)))
      (Variables|/Game/Blueprints/Component/AC_Weapon.AC_Weapon_C|SetRPM (Variables|/Game/Blueprints/Player/BP_FirstPersonCharacter.BP_FirstPersonCharacter_C|GetAC_WeaponComponent (Variables|/Game/Blueprints/Player/BP_FirstPersonCharacter.BP_FirstPersonCharacter_C|GetTeamMateRef _asbp_first_person_character)) _output_get_2)))
  (Ability|EndAbility))

(event EventOnTargetModulation
  (params (Modulations :type BP%20Modulation%20Object%20Reference%20%28by%20ref%29) (Point :type Vector :default "0, 0, 0"))
  (bind _asbp_custom_player_state (Utilities|Casting|CastToBP_CustomPlayerState (Ability|GetOwningActorfromActorInfo)))
  (bind _asbp_first_person_character (Utilities|Casting|CastToBP_FirstPersonCharacter (PlayerState|GetPawn _asbp_custom_player_state)))
  (Variables|Default|SetOriginRPM (Variables|/Game/Blueprints/Component/AC_Weapon.AC_Weapon_C|GetRPM (Variables|/Game/Blueprints/Player/BP_FirstPersonCharacter.BP_FirstPersonCharacter_C|GetAC_WeaponComponent _asbp_first_person_character)))
  (if (or (Variables|/Game/Blueprints/Player/BP_FirstPersonCharacter.BP_FirstPersonCharacter_C|GetWaitingForRespawn (Variables|/Game/Blueprints/Player/BP_FirstPersonCharacter.BP_FirstPersonCharacter_C|GetTeamMateRef _asbp_first_person_character)) (> (Math|Vector|Distance(Vector) (Transformation|GetActorLocation (Variables|/Game/Blueprints/Player/BP_FirstPersonCharacter.BP_FirstPersonCharacter_C|GetTeamMateRef _asbp_first_person_character)) (Transformation|GetActorLocation _asbp_first_person_character)) (Variables|Default|GetDistToAlly)))
    (Variables|/Game/Blueprints/Component/AC_Weapon.AC_Weapon_C|SetRPM (Variables|/Game/Blueprints/Player/BP_FirstPersonCharacter.BP_FirstPersonCharacter_C|GetAC_WeaponComponent _asbp_first_person_character) (+ (Variables|Default|GetOriginRPM) (Variables|Default|GetSoloBonus)))
    (Utilities|FlowControl|Delay (Variables|Default|GetEffectDuration))
    (Variables|/Game/Blueprints/Component/AC_Weapon.AC_Weapon_C|SetRPM (Variables|/Game/Blueprints/Player/BP_FirstPersonCharacter.BP_FirstPersonCharacter_C|GetAC_WeaponComponent _asbp_first_person_character) (Variables|Default|GetOriginRPM))
    (else
      (bind _output_get (Variables|/Game/Blueprints/Component/AC_Weapon.AC_Weapon_C|SetRPM (Variables|/Game/Blueprints/Player/BP_FirstPersonCharacter.BP_FirstPersonCharacter_C|GetAC_WeaponComponent _asbp_first_person_character) (+ (Variables|Default|GetOriginRPM) (Variables|Default|GetWithAllyBonus))))
      (Variables|/Game/Blueprints/Component/AC_Weapon.AC_Weapon_C|SetRPM (Variables|/Game/Blueprints/Player/BP_FirstPersonCharacter.BP_FirstPersonCharacter_C|GetAC_WeaponComponent (Variables|/Game/Blueprints/Player/BP_FirstPersonCharacter.BP_FirstPersonCharacter_C|GetTeamMateRef _asbp_first_person_character)) _output_get)
      (Utilities|FlowControl|Delay (Variables|Default|GetEffectDuration))
      (bind _output_get_2 (Variables|/Game/Blueprints/Component/AC_Weapon.AC_Weapon_C|SetRPM (Variables|/Game/Blueprints/Player/BP_FirstPersonCharacter.BP_FirstPersonCharacter_C|GetAC_WeaponComponent _asbp_first_person_character) (Variables|Default|GetOriginRPM)))
      (Variables|/Game/Blueprints/Component/AC_Weapon.AC_Weapon_C|SetRPM (Variables|/Game/Blueprints/Player/BP_FirstPersonCharacter.BP_FirstPersonCharacter_C|GetAC_WeaponComponent (Variables|/Game/Blueprints/Player/BP_FirstPersonCharacter.BP_FirstPersonCharacter_C|GetTeamMateRef _asbp_first_person_character)) _output_get_2)))
  (Ability|EndAbility))

(event EventOnFreePlacement
  (params (Point :type Vector :default "0, 0, 0"))
  (bind _asbp_custom_player_state (Utilities|Casting|CastToBP_CustomPlayerState (Ability|GetOwningActorfromActorInfo)))
  (bind _asbp_first_person_character (Utilities|Casting|CastToBP_FirstPersonCharacter (PlayerState|GetPawn _asbp_custom_player_state)))
  (Variables|Default|SetOriginRPM (Variables|/Game/Blueprints/Component/AC_Weapon.AC_Weapon_C|GetRPM (Variables|/Game/Blueprints/Player/BP_FirstPersonCharacter.BP_FirstPersonCharacter_C|GetAC_WeaponComponent _asbp_first_person_character)))
  (if (or (Variables|/Game/Blueprints/Player/BP_FirstPersonCharacter.BP_FirstPersonCharacter_C|GetWaitingForRespawn (Variables|/Game/Blueprints/Player/BP_FirstPersonCharacter.BP_FirstPersonCharacter_C|GetTeamMateRef _asbp_first_person_character)) (> (Math|Vector|Distance(Vector) (Transformation|GetActorLocation (Variables|/Game/Blueprints/Player/BP_FirstPersonCharacter.BP_FirstPersonCharacter_C|GetTeamMateRef _asbp_first_person_character)) (Transformation|GetActorLocation _asbp_first_person_character)) (Variables|Default|GetDistToAlly)))
    (Variables|/Game/Blueprints/Component/AC_Weapon.AC_Weapon_C|SetRPM (Variables|/Game/Blueprints/Player/BP_FirstPersonCharacter.BP_FirstPersonCharacter_C|GetAC_WeaponComponent _asbp_first_person_character) (+ (Variables|Default|GetOriginRPM) (Variables|Default|GetSoloBonus)))
    (Utilities|FlowControl|Delay (Variables|Default|GetEffectDuration))
    (Variables|/Game/Blueprints/Component/AC_Weapon.AC_Weapon_C|SetRPM (Variables|/Game/Blueprints/Player/BP_FirstPersonCharacter.BP_FirstPersonCharacter_C|GetAC_WeaponComponent _asbp_first_person_character) (Variables|Default|GetOriginRPM))
    (else
      (bind _output_get (Variables|/Game/Blueprints/Component/AC_Weapon.AC_Weapon_C|SetRPM (Variables|/Game/Blueprints/Player/BP_FirstPersonCharacter.BP_FirstPersonCharacter_C|GetAC_WeaponComponent _asbp_first_person_character) (+ (Variables|Default|GetOriginRPM) (Variables|Default|GetWithAllyBonus))))
      (Variables|/Game/Blueprints/Component/AC_Weapon.AC_Weapon_C|SetRPM (Variables|/Game/Blueprints/Player/BP_FirstPersonCharacter.BP_FirstPersonCharacter_C|GetAC_WeaponComponent (Variables|/Game/Blueprints/Player/BP_FirstPersonCharacter.BP_FirstPersonCharacter_C|GetTeamMateRef _asbp_first_person_character)) _output_get)
      (Utilities|FlowControl|Delay (Variables|Default|GetEffectDuration))
      (bind _output_get_2 (Variables|/Game/Blueprints/Component/AC_Weapon.AC_Weapon_C|SetRPM (Variables|/Game/Blueprints/Player/BP_FirstPersonCharacter.BP_FirstPersonCharacter_C|GetAC_WeaponComponent _asbp_first_person_character) (Variables|Default|GetOriginRPM)))
      (Variables|/Game/Blueprints/Component/AC_Weapon.AC_Weapon_C|SetRPM (Variables|/Game/Blueprints/Player/BP_FirstPersonCharacter.BP_FirstPersonCharacter_C|GetAC_WeaponComponent (Variables|/Game/Blueprints/Player/BP_FirstPersonCharacter.BP_FirstPersonCharacter_C|GetTeamMateRef _asbp_first_person_character)) _output_get_2)))
  (Ability|EndAbility))