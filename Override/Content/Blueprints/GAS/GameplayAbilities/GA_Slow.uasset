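; GA_Slow is a gameplay ability that places a slow sphere at a targeted point.
; Free placement, player targeting and modulation targeting events all call CastSlowSphere, then end the ability.
; CastSlowSphere reaches the character through the owning PlayerState, spawns a BP_SlowSphere scaled by SphereScale, excludes the caster and teammate, and starts its life for EffectDuration.
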(event EventOnFreePlacement
  (params (Point :type Vector :default "0, 0, 0"))
  (CallFunction|CastSlowSphere Point)
  (Ability|EndAbility))

(event EventOnTargetPlayer
  (params (Player :type BP%20First%20Person%20Character%20Object%20Reference) (Point :type Vector :default "0, 0, 0"))
  (CallFunction|CastSlowSphere Point)
  (Ability|EndAbility))

(event EventOnTargetModulation
  (params (Modulations :type BP%20Modulation%20Object%20Reference%20%28by%20ref%29) (Point :type Vector :default "0, 0, 0"))
  (CallFunction|CastSlowSphere Point)
  (Ability|EndAbility))

(fn CastSlowSphere
  (params (Origin :type Vector))
  (bind _asbp_custom_player_state (Utilities|Casting|CastToBP_CustomPlayerState (Ability|GetOwningActorfromActorInfo)))
  (bind _asbp_first_person_character (Utilities|Casting|CastToBP_FirstPersonCharacter (PlayerState|GetPawn _asbp_custom_player_state)))
  (bind _returnvalue (Game|SpawnActorfromClass "/Game/Blueprints/Other/BP_SlowSphere.BP_SlowSphere_C" (Math|Transform|MakeTransform Origin "0, 0, 0" (Math|Conversions|ToVector(Float) (Variables|Default|GetSphere%20Scale))) "Undefined" "MultiplyWithRoot" 0 0))
  (Variables|/Game/Blueprints/Other/BP_SlowSphere.BP_SlowSphere_C|SetIgnoredActors _returnvalue (Utilities|Array|MakeArray _asbp_first_person_character (Variables|/Game/Blueprints/Player/BP_FirstPersonCharacter.BP_FirstPersonCharacter_C|GetTeamMateRef _asbp_first_person_character)))
  (Default|StartLife _returnvalue (Variables|Default|GetEffect%20Duration)))