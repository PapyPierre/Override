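; GA_BP_Base_Ability is a base gameplay ability that routes an activation by what was targeted.
; On activation it gets the owning player's first-person character via the player state and calls CallAbility with SelfCast.
; With no targets it fires the Aoe gameplay cue and calls OnFreePlacement.
; Otherwise it calls OnTargetPlayer for a first-target player, or OnTargetModulation per Modulation target; all three hooks are empty.
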(event Custom|OnFreePlacement
  (params (Point :type Vector)))

(event Custom|OnTargetPlayer
  (params (Player :type BP%20First%20Person%20Character%20Object%20Reference) (Point :type Vector)))

(event Custom|OnTargetModulation
  (params (Modulations :type BP%20Modulation%20Object%20Reference%20%28by%20ref%29) (Point :type Vector)))

(event EventOnAbilityActivated
  (params (Location :type Vector :default "0, 0, 0") (Targets :type Array%20of%20Actor%20Object%20References))
  (bind _asbp_custom_player_state (Utilities|Casting|CastToBP_CustomPlayerState (Ability|GetOwningActorfromActorInfo)))
  (bind _asbp_first_person_character (Utilities|Casting|CastToBP_FirstPersonCharacter (PlayerState|GetPawn _asbp_custom_player_state)))
  (Default|CallAbility _asbp_first_person_character (Variables|Default|GetSelfCast))
  (if (Utilities|Array|IsEmpty Targets)
    (Class|GameplayAbility|ExecuteGameplayCuewithParams "(TagName=\"GameplayCue.Aoe\")" (Ability|GameplayCue|MakeGameplayCueParameters :Location Location))
    (CallFunction|OnFreePlacement Location)
    (else
      (bind _asbp_first_person_character_2 (Utilities|Casting|CastToBP_FirstPersonCharacter (Utilities|Array|Get(acopy) Targets))
        (:then
          (CallFunction|OnTargetPlayer _asbp_first_person_character_2 Location))
        (:CastFailed
          (for _array_element Targets
            (bind _asbp_modulation (Utilities|Casting|CastToBP_Modulation _array_element))
            (CallFunction|OnTargetModulation _asbp_modulation Location)))))))