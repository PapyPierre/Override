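; GA_Camouflage is a gameplay ability that puts the owning player's first-person character into camouflage for a limited time.
; The free placement, player target and modulation target events all run the same logic, reaching the pawn through the owning custom PlayerState.
; It starts camouflage, waits for the effect duration, stops camouflage if still active, then ends the ability.
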(event EventOnFreePlacement
  (params (Point :type Vector :default "0, 0, 0"))
  (bind _asbp_custom_player_state (Utilities|Casting|CastToBP_CustomPlayerState (Ability|GetOwningActorfromActorInfo)))
  (bind _asbp_first_person_character (Utilities|Casting|CastToBP_FirstPersonCharacter (PlayerState|GetPawn _asbp_custom_player_state)))
  (Default|StartCamouflage _asbp_first_person_character)
  (Utilities|FlowControl|Delay (Variables|Default|GetEffectDuration))
  (if (Variables|/Game/Blueprints/Player/BP_FirstPersonCharacter.BP_FirstPersonCharacter_C|GetInCamouflage _asbp_first_person_character)
    (Default|StopCamouflage _asbp_first_person_character))
  (Ability|EndAbility))

(event EventOnTargetPlayer
  (params (Player :type BP%20First%20Person%20Character%20Object%20Reference) (Point :type Vector :default "0, 0, 0"))
  (bind _asbp_custom_player_state (Utilities|Casting|CastToBP_CustomPlayerState (Ability|GetOwningActorfromActorInfo)))
  (bind _asbp_first_person_character (Utilities|Casting|CastToBP_FirstPersonCharacter (PlayerState|GetPawn _asbp_custom_player_state)))
  (Default|StartCamouflage _asbp_first_person_character)
  (Utilities|FlowControl|Delay (Variables|Default|GetEffectDuration))
  (if (Variables|/Game/Blueprints/Player/BP_FirstPersonCharacter.BP_FirstPersonCharacter_C|GetInCamouflage _asbp_first_person_character)
    (Default|StopCamouflage _asbp_first_person_character))
  (Ability|EndAbility))

(event EventOnTargetModulation
  (params (Modulations :type BP%20Modulation%20Object%20Reference%20%28by%20ref%29) (Point :type Vector :default "0, 0, 0"))
  (bind _asbp_custom_player_state (Utilities|Casting|CastToBP_CustomPlayerState (Ability|GetOwningActorfromActorInfo)))
  (bind _asbp_first_person_character (Utilities|Casting|CastToBP_FirstPersonCharacter (PlayerState|GetPawn _asbp_custom_player_state)))
  (Default|StartCamouflage _asbp_first_person_character)
  (Utilities|FlowControl|Delay (Variables|Default|GetEffectDuration))
  (if (Variables|/Game/Blueprints/Player/BP_FirstPersonCharacter.BP_FirstPersonCharacter_C|GetInCamouflage _asbp_first_person_character)
    (Default|StopCamouflage _asbp_first_person_character))
  (Ability|EndAbility))