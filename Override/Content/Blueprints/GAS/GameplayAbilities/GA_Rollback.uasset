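; Gameplay ability that triggers a rollback on the owning player's first-person character.
; Free placement, player target and modulation target events share one path, reaching the pawn through the player state to start its RollbackComponent.
; A timer set to the component's max history duration divided by rollback speed stops the rollback and ends the ability.
; The ability ends immediately if the component is missing.
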(event Custom|OnRollbackEnd
  (Class|RollbackComponent|StopRollback (Variables|Default|GetRollback%20Component))
  (Ability|EndAbility))

(event EventOnFreePlacement
  (params (Point :type Vector :default "0, 0, 0"))
  (bind _asbp_custom_player_state (Utilities|Casting|CastToBP_CustomPlayerState (Ability|GetOwningActorfromActorInfo)))
  (bind _asbp_first_person_character (Utilities|Casting|CastToBP_FirstPersonCharacter (PlayerState|GetPawn _asbp_custom_player_state)))
  (bind _output_get (Variables|Default|SetRollback%20Component (Actor|GetComponentbyClass _asbp_first_person_character "/Script/Override.RollbackComponent")))
  (Utilities|IsValid _output_get
    (:Is%20Valid
      (Class|RollbackComponent|StartRollback (Variables|Default|GetRollback%20Component))
      (bind _output_get_2 (Variables|Default|SetEffect%20Duration (/ (Variables|/Script/Override.RollbackComponent|GetMaxHistoryDuration (Variables|Default|GetRollback%20Component)) (Variables|/Script/Override.RollbackComponent|GetRollbackSpeed (Variables|Default|GetRollback%20Component)))))
      (Utilities|Time|SetTimerbyEvent (delegate Custom|OnRollbackEnd) _output_get_2))
    (:Is%20Not%20Valid
      (Ability|EndAbility))))

(event EventOnTargetPlayer
  (params (Player :type BP%20First%20Person%20Character%20Object%20Reference) (Point :type Vector :default "0, 0, 0"))
  (bind _asbp_custom_player_state (Utilities|Casting|CastToBP_CustomPlayerState (Ability|GetOwningActorfromActorInfo)))
  (bind _asbp_first_person_character (Utilities|Casting|CastToBP_FirstPersonCharacter (PlayerState|GetPawn _asbp_custom_player_state)))
  (bind _output_get (Variables|Default|SetRollback%20Component (Actor|GetComponentbyClass _asbp_first_person_character "/Script/Override.RollbackComponent")))
  (Utilities|IsValid _output_get
    (:Is%20Valid
      (Class|RollbackComponent|StartRollback (Variables|Default|GetRollback%20Component))
      (bind _output_get_2 (Variables|Default|SetEffect%20Duration (/ (Variables|/Script/Override.RollbackComponent|GetMaxHistoryDuration (Variables|Default|GetRollback%20Component)) (Variables|/Script/Override.RollbackComponent|GetRollbackSpeed (Variables|Default|GetRollback%20Component)))))
      (Utilities|Time|SetTimerbyEvent (delegate Custom|OnRollbackEnd) _output_get_2))
    (:Is%20Not%20Valid
      (Ability|EndAbility))))

(event EventOnTargetModulation
  (params (Modulations :type BP%20Modulation%20Object%20Reference%20%28by%20ref%29) (Point :type Vector :default "0, 0, 0"))
  (bind _asbp_custom_player_state (Utilities|Casting|CastToBP_CustomPlayerState (Ability|GetOwningActorfromActorInfo)))
  (bind _asbp_first_person_character (Utilities|Casting|CastToBP_FirstPersonCharacter (PlayerState|GetPawn _asbp_custom_player_state)))
  (bind _output_get (Variables|Default|SetRollback%20Component (Actor|GetComponentbyClass _asbp_first_person_character "/Script/Override.RollbackComponent")))
  (Utilities|IsValid _output_get
    (:Is%20Valid
      (Class|RollbackComponent|StartRollback (Variables|Default|GetRollback%20Component))
      (bind _output_get_2 (Variables|Default|SetEffect%20Duration (/ (Variables|/Script/Override.RollbackComponent|GetMaxHistoryDuration (Variables|Default|GetRollback%20Component)) (Variables|/Script/Override.RollbackComponent|GetRollbackSpeed (Variables|Default|GetRollback%20Component)))))
      (Utilities|Time|SetTimerbyEvent (delegate Custom|OnRollbackEnd) _output_get_2))
    (:Is%20Not%20Valid
      (Ability|EndAbility))))