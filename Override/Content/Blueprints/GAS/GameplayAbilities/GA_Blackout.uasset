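; GA_Blackout is a gameplay ability that fires an EMP-style area disruption centred on the owning player's pawn.
; All three targeting events run the same logic: multicast the VFX, then sphere-overlap within the effect radius, ignoring the caster and teammate.
; Overlapped modulations are locked, while other characters get timed HUD interference and lose active camouflage, before the ability ends.
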(event EventOnFreePlacement
  (params (Point :type Vector :default "0, 0, 0"))
  (bind _asbp_custom_player_state (Utilities|Casting|CastToBP_CustomPlayerState (Ability|GetOwningActorfromActorInfo)))
  (bind _asbp_first_person_character (Utilities|Casting|CastToBP_FirstPersonCharacter (PlayerState|GetPawn _asbp_custom_player_state)))
  (Default|MulticastVFXIEM _asbp_first_person_character (Transformation|GetActorLocation (PlayerState|GetPawn _asbp_custom_player_state)))
  (bind _outactors (Collision|SphereOverlapActors (Transformation|GetActorLocation (PlayerState|GetPawn _asbp_custom_player_state)) (Variables|Default|GetEffect%20Radius) (Utilities|Array|MakeArray "ObjectTypeQuery7") "/Script/Engine.Actor" (Utilities|Array|MakeArray (PlayerState|GetPawn _asbp_custom_player_state) (Variables|/Game/Blueprints/Player/BP_FirstPersonCharacter.BP_FirstPersonCharacter_C|GetTeamMateRef _asbp_first_person_character))))
  (for _array_element _outactors
    (bind _asbp_modulation (Utilities|Casting|CastToBP_Modulation _array_element)
      (:then
        (Class|Modulation|Lock _asbp_modulation true))
      (:CastFailed
        (bind _asbp_first_person_character_2 (Utilities|Casting|CastToBP_FirstPersonCharacter _array_element))
        (Default|HUDInterference _asbp_first_person_character_2 (Variables|Default|GetEffect%20Duration))
        (Variables|/Game/Blueprints/Player/BP_FirstPersonCharacter.BP_FirstPersonCharacter_C|GetInCamouflage _asbp_first_person_character_2
          (:then
            (Default|StopCamouflage _asbp_first_person_character_2))
          (:else)))))
  (Ability|EndAbility))

(event EventOnTargetPlayer
  (params (Player :type BP%20First%20Person%20Character%20Object%20Reference) (Point :type Vector :default "0, 0, 0"))
  (bind _asbp_custom_player_state (Utilities|Casting|CastToBP_CustomPlayerState (Ability|GetOwningActorfromActorInfo)))
  (bind _asbp_first_person_character (Utilities|Casting|CastToBP_FirstPersonCharacter (PlayerState|GetPawn _asbp_custom_player_state)))
  (Default|MulticastVFXIEM _asbp_first_person_character (Transformation|GetActorLocation (PlayerState|GetPawn _asbp_custom_player_state)))
  (bind _outactors (Collision|SphereOverlapActors (Transformation|GetActorLocation (PlayerState|GetPawn _asbp_custom_player_state)) (Variables|Default|GetEffect%20Radius) (Utilities|Array|MakeArray "ObjectTypeQuery7") "/Script/Engine.Actor" (Utilities|Array|MakeArray (PlayerState|GetPawn _asbp_custom_player_state) (Variables|/Game/Blueprints/Player/BP_FirstPersonCharacter.BP_FirstPersonCharacter_C|GetTeamMateRef _asbp_first_person_character))))
  (for _array_element _outactors
    (bind _asbp_modulation (Utilities|Casting|CastToBP_Modulation _array_element)
      (:then
        (Class|Modulation|Lock _asbp_modulation true))
      (:CastFailed
        (bind _asbp_first_person_character_2 (Utilities|Casting|CastToBP_FirstPersonCharacter _array_element))
        (Default|HUDInterference _asbp_first_person_character_2 (Variables|Default|GetEffect%20Duration))
        (Variables|/Game/Blueprints/Player/BP_FirstPersonCharacter.BP_FirstPersonCharacter_C|GetInCamouflage _asbp_first_person_character_2
          (:then
            (Default|StopCamouflage _asbp_first_person_character_2))
          (:else)))))
  (Ability|EndAbility))

(event EventOnTargetModulation
  (params (Modulations :type BP%20Modulation%20Object%20Reference%20%28by%20ref%29) (Point :type Vector :default "0, 0, 0"))
  (bind _asbp_custom_player_state (Utilities|Casting|CastToBP_CustomPlayerState (Ability|GetOwningActorfromActorInfo)))
  (bind _asbp_first_person_character (Utilities|Casting|CastToBP_FirstPersonCharacter (PlayerState|GetPawn _asbp_custom_player_state)))
  (Default|MulticastVFXIEM _asbp_first_person_character (Transformation|GetActorLocation (PlayerState|GetPawn _asbp_custom_player_state)))
  (bind _outactors (Collision|SphereOverlapActors (Transformation|GetActorLocation (PlayerState|GetPawn _asbp_custom_player_state)) (Variables|Default|GetEffect%20Radius) (Utilities|Array|MakeArray "ObjectTypeQuery7") "/Script/Engine.Actor" (Utilities|Array|MakeArray (PlayerState|GetPawn _asbp_custom_player_state) (Variables|/Game/Blueprints/Player/BP_FirstPersonCharacter.BP_FirstPersonCharacter_C|GetTeamMateRef _asbp_first_person_character))))
  (for _array_element _outactors
    (bind _asbp_modulation (Utilities|Casting|CastToBP_Modulation _array_element)
      (:then
        (Class|Modulation|Lock _asbp_modulation true))
      (:CastFailed
        (bind _asbp_first_person_character_2 (Utilities|Casting|CastToBP_FirstPersonCharacter _array_element))
        (Default|HUDInterference _asbp_first_person_character_2 (Variables|Default|GetEffect%20Duration))
        (Variables|/Game/Blueprints/Player/BP_FirstPersonCharacter.BP_FirstPersonCharacter_C|GetInCamouflage _asbp_first_person_character_2
          (:then
            (Default|StopCamouflage _asbp_first_person_character_2))
          (:else)))))
  (Ability|EndAbility))