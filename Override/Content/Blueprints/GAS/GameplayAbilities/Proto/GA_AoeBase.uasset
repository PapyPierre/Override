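; Prototype base gameplay ability for area-of-effect abilities, triggered by an event carrying target data.
; For each target actor it commits the ability, draws a debug sphere and overlaps WorldDynamic actors within Radius plus the target's largest bounds extent, optionally excluding the avatar.
; On authority, overlapped actors go to ApplyEffectsToTarget, an empty hook here; without authority the ability ends.
; CommitAbility runs inside the target loop, and a failed commit cancels the ability.
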(event Ability|EventActivateAbility
  (for _array_element (Ability|TargetData|GetActorsfromTargetData (.TargetData (Utilities|Struct|BreakGameplayEventData (Class|GABaseHack|GetEventData))))
    (bind _returnvalue (Ability|CommitAbility))
    (if _returnvalue
      (Rendering|Debug|DrawDebugSphere (.Origin (Collision|GetActorBounds _array_element false false)) (+ (Math|Float|Max(Float) (.x (.BoxExtent (Collision|GetActorBounds _array_element false false))) (.y (.BoxExtent (Collision|GetActorBounds _array_element false false))) (.z (.BoxExtent (Collision|GetActorBounds _array_element false false)))) (Variables|Default|GetRadius)) 24 (Variables|Default|GetDebug%20Color) 2.0 3.0)
      (bind _outactors (Collision|SphereOverlapActors (.Origin (Collision|GetActorBounds _array_element false false)) (+ (Math|Float|Max(Float) (.x (.BoxExtent (Collision|GetActorBounds _array_element false false))) (.y (.BoxExtent (Collision|GetActorBounds _array_element false false))) (.z (.BoxExtent (Collision|GetActorBounds _array_element false false)))) (Variables|Default|GetRadius)) (Utilities|Array|MakeArray "ObjectTypeQuery2") 0 (select (Variables|Default|GetCanTargetSelf) 0 (Utilities|Array|MakeArray (Ability|GetAvatarActorfromActorInfo)))))
      (for _array_element_2 _outactors
        (Ability|HasAuthority
          (:True
            (CallFunction|ApplyEffectstoTarget _array_element_2))
          (:False
            (Ability|EndAbility))))
      (else
        (Ability|CancelAbility))))
  (Ability|EndAbility))

(fn ApplyEffectstoTarget
  (params (Target%20Actor :type Actor%20Object%20Reference)))