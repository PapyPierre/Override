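; BP_Ping is a short-lived world ping marker that shows its distance from a character.
; SetDistance stores the character, caches the WBP_Ping widget from its widget component and writes the initial distance.
; Tick then refreshes that text from the gap between character and marker, dividing by 100 to convert to meters.
; The actor destroys itself on a timer set at BeginPlay, or earlier when StopPing is called.
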(event Custom|AutoDestroy
  (Actor|DestroyActor))

(event Custom|SetDistance
  (params (Distance :type Integer) (Character :type Actor%20Object%20Reference))
  (Variables|Default|SetCharacter Character)
  (bind _aswbp_ping (Utilities|Casting|CastToWBP_Ping (UserInterface|GetWidget (Variables|Default|GetWidget))))
  (Variables|Default|SetAs%20WBP%20Ping _aswbp_ping)
  (Rendering|Components|TextRender|SetText (Variables|/Game/Blueprints/Widget/World/WBP_Ping.WBP_Ping_C|GetDistance _aswbp_ping) (Utilities|Text|ToText(Integer) (/ Distance 100))))

(event EventBeginPlay
  (Utilities|Time|SetTimerbyEvent (delegate Custom|AutoDestroy) 5.0))

(event EventStopPing
  (Actor|DestroyActor))

(event EventTick
  (params (DeltaSeconds :type Float%20%28single-precision%29))
  (Utilities|IsValid (Variables|Default|GetAs%20WBP%20Ping)
    (:Is%20Valid
      (Utilities|IsValid (Variables|Default|GetCharacter)
        (:Is%20Valid
          (Rendering|Components|TextRender|SetText (Variables|/Game/Blueprints/Widget/World/WBP_Ping.WBP_Ping_C|GetDistance (Variables|Default|GetAs%20WBP%20Ping)) (Utilities|Text|ToText(Integer) (/ (Math|Float|Truncate (Math|Vector|Distance(Vector) (Transformation|GetWorldLocation (Variables|/Script/Engine.Actor|GetRootComponent (Variables|Default|GetCharacter))) (Transformation|GetWorldLocation (Variables|Default|GetDefaultSceneRoot)))) 100))))))))

(fn ConstructionScript)