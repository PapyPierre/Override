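; Capture point actor holding a depletable pool of data that player characters collect by standing inside it.
; Overlap events track occupants, and a server-side Tick runs a looping timer that drains the pool into each occupant, mirroring their total to their teammate.
; Tick also tells the GameMode whether the point is occupied and the GameState when it empties.
; CurrentData's OnRep refreshes the widget text; the Old event retains earlier delta-time scoring.
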(event Custom|SetCurrentData
  (params (Data :type Float%20%28double-precision%29))
  ;[0.15 0.15 0.15 0.5] Set Data At Spawn
  (bind _output_get (Variables|Default|SetInitialData Data))
  (Variables|Default|SetCurrentData _output_get))

(event Custom|Add%20Date%20Per%20Second
  (bind _datapertime (Variables|Default|GetDataPerTime))
  ;[0.15 0.15 0.15 0.5] Logic For Adding Point Each Tick
  (for _array_element (Variables|Default|GetCharacterCurrentlyIn%20)
    (bind _output_get (Variables|/Game/Blueprints/Player/BP_FirstPersonCharacter.BP_FirstPersonCharacter_C|SetDataPossesed _array_element (+ (Variables|/Game/Blueprints/Player/BP_FirstPersonCharacter.BP_FirstPersonCharacter_C|GetDataPossesed _array_element) _datapertime)))
    (Utilities|IsValid (Variables|/Game/Blueprints/Player/BP_FirstPersonCharacter.BP_FirstPersonCharacter_C|GetTeamMateRef _array_element)
      (:Is%20Valid
        (Variables|/Game/Blueprints/Player/BP_FirstPersonCharacter.BP_FirstPersonCharacter_C|SetDataPossesed (Variables|/Game/Blueprints/Player/BP_FirstPersonCharacter.BP_FirstPersonCharacter_C|GetTeamMateRef _array_element) _output_get))
      (:Is%20Not%20Valid
        _))
    (Variables|Default|SetCurrentData (- (Variables|Default|GetCurrentData) _datapertime))))

(event Custom|SetDataUI
  (Utilities|IsValid (Variables|Default|GetWidgetRef)
    (:Is%20Valid
      _)
    (:Is%20Not%20Valid
      (bind _aswbp_data_text (Utilities|Casting|CastToWBP_DataText (UserInterface|GetWidget (Variables|Default|GetWidget))))
      (Variables|Default|SetWidgetRef _aswbp_data_text)))
  (Rendering|Components|TextRender|SetText (Variables|/Game/Blueprints/Widget/WBP_DataText.WBP_DataText_C|GetTextBlock_56 (Variables|Default|GetWidgetRef)) (Utilities|Text|ToText(Float) (Variables|Default|GetCurrentData) "HalfToEven")))

(event Custom|Old
  (params (DeltaSeconds :type Float%20%28single-precision%29))
  ;[0.15 0.000664 0 0.5] OLD Logic For Adding Point Each Tick
  (Networking|SwitchHasAuthority
    (:Authority
      (if (<= (Variables|Default|GetCurrentData) 0.0)
        (Default|DataPointEmpty (Variables|Default|GetGameState))
        (elif (> (Utilities|Array|Length (Variables|Default|GetCharacterCurrentlyIn%20)) 0)
          (bind _output_get (Variables|Default|SetCurrentData (- (Variables|Default|GetCurrentData) (+ (* DeltaSeconds (Variables|Default|GetDataPerTime)) (Variables|Default|GetScoreAccumulator)))))
          (if (< _output_get 0.0)
            (Variables|Default|SetScoreAccumulator (/ (- (+ (* DeltaSeconds (Variables|Default|GetDataPerTime)) (Variables|Default|GetScoreAccumulator)) (Math|Float|Absolute(Float) _output_get)) (Utilities|Array|Length (Variables|Default|GetCharacterCurrentlyIn%20))))
            (else
              (Variables|Default|SetScoreAccumulator (/ (+ (* DeltaSeconds (Variables|Default|GetDataPerTime)) (Variables|Default|GetScoreAccumulator)) (Utilities|Array|Length (Variables|Default|GetCharacterCurrentlyIn%20))))))
          (for _array_element (Variables|Default|GetCharacterCurrentlyIn%20)
            (bind _output_get_2 (Variables|/Game/Blueprints/Player/BP_FirstPersonCharacter.BP_FirstPersonCharacter_C|SetDataPossesed _array_element (* (+ (Variables|Default|GetScoreAccumulator) (Variables|/Game/Blueprints/Player/BP_FirstPersonCharacter.BP_FirstPersonCharacter_C|GetDataPossesed _array_element)) (Variables|Default|GetRoundMultiplier))))
            (Variables|/Game/Blueprints/Player/BP_FirstPersonCharacter.BP_FirstPersonCharacter_C|SetDataPossesed (Variables|/Game/Blueprints/Player/BP_FirstPersonCharacter.BP_FirstPersonCharacter_C|GetTeamMateRef _array_element) _output_get_2))
          (Variables|Default|SetScoreAccumulator 0.0))))))

(event EventTick
  (params (DeltaSeconds :type Float%20%28single-precision%29))
  (bind _gamestate (Variables|Default|GetGameState))
  (bind _gamemode (Variables|/Game/Blueprints/GameMode/BP_GameState.BP_GameState_C|GetGameMode _gamestate))
  ;[0.15 0.15 0.15 0.5] Logic For Adding Point Each Tick
  (Networking|SwitchHasAuthority
    (:Authority
      (if (<= (Variables|Default|GetCurrentData) 0.0)
        (Default|DataPointEmpty (Variables|Default|GetGameState))
        (Utilities|Time|ClearandInvalidateTimerbyHandle (Variables|Default|GetTimer))
        (elif (> (Utilities|Array|Length (Variables|Default|GetCharacterCurrentlyIn%20)) 0)
          (Default|CallCancelDataPointDestruction _gamemode)
          (if (not (Utilities|Time|IsValidTimerHandle (Variables|Default|GetTimer)))
            (bind _returnvalue (Utilities|Time|SetTimerbyEvent (delegate Custom|Add%20Date%20Per%20Second) (Variables|Default|GetDataCooldown) true))
            (Variables|Default|SetTimer _returnvalue))
          (else
            (Utilities|Time|ClearandInvalidateTimerbyHandle (Variables|Default|GetTimer))
            (Default|CallDataPointUnoccupied _gamemode)))))))

(event Collision|EventActorBeginOverlap
  (params (OtherActor :type Actor%20Object%20Reference))
  ;[0.15 0.15 0.15 0.5] Add Character To List When Overlap
  (if (== (Utilities|GetClass OtherActor) "/Game/Blueprints/Player/BP_FirstPersonCharacter.BP_FirstPersonCharacter_C")
    (Utilities|Array|Add (Variables|Default|GetCharacterCurrentlyIn%20) (.AsBP%20First%20Person%20Character (Utilities|Casting|CastToBP_FirstPersonCharacter OtherActor)))))

(event Collision|EventActorEndOverlap
  (params (OtherActor :type Actor%20Object%20Reference))
  ;[0.15 0.15 0.15 0.5] Remove Character To List When End Of Overlap
  (if (== (Utilities|GetClass OtherActor) "/Game/Blueprints/Player/BP_FirstPersonCharacter.BP_FirstPersonCharacter_C")
    (Utilities|Array|RemoveItem (Variables|Default|GetCharacterCurrentlyIn%20) (.AsBP%20First%20Person%20Character (Utilities|Casting|CastToBP_FirstPersonCharacter OtherActor)))))

(fn ConstructionScript)

(fn OnRepCurrentData
  (CallFunction|SetDataUI))