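; Cash-out point where players standing in its cone bank carried data into their team's score.
; On server Tick, occupants holding data get per-player cash-out timers, gated by a busy flag, while the point's expiry timer pauses.
; Completion zeroes the player's and teammate's data and updates GameState; leaving cancels the timer and resumes expiry.
; GameState is notified that extraction finished when expiry fires or banked total equals the round's cash value.
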(event OnComponentBeginOverlap(Cone)
  (params (OverlappedComponent :type Primitive%20Component%20Object%20Reference) (OtherActor :type Actor%20Object%20Reference) (OtherComp :type Primitive%20Component%20Object%20Reference) (OtherBodyIndex :type Integer) (bFromSweep :type Boolean) (SweepResult :type Hit%20Result%20Structure%20%28by%20ref%29))
  (bind _asbp_first_person_character (Utilities|Casting|CastToBP_FirstPersonCharacter OtherActor))
  ;[0.15 0.15 0.15 0.5] Add Character To List When Overlap
  (if (== (Utilities|GetClass OtherActor) "/Game/Blueprints/Player/BP_FirstPersonCharacter.BP_FirstPersonCharacter_C")
    (Utilities|Array|AddUnique (Variables|Default|GetCharacterCurrentlyIn%20) _asbp_first_person_character)
    (Utilities|Map|Add :TargetMap (Variables|Default|GetCooldownAndPlayer) :Key _asbp_first_person_character)))

(event OnComponentEndOverlap(Cone)
  (params (OverlappedComponent :type Primitive%20Component%20Object%20Reference) (OtherActor :type Actor%20Object%20Reference) (OtherComp :type Primitive%20Component%20Object%20Reference) (OtherBodyIndex :type Integer))
  (bind _asbp_first_person_character (Utilities|Casting|CastToBP_FirstPersonCharacter OtherActor))
  ;[0.15 0.15 0.15 0.5] Remove Character To List When End Of Overlap
  (if (== (Utilities|GetClass OtherActor) "/Game/Blueprints/Player/BP_FirstPersonCharacter.BP_FirstPersonCharacter_C")
    (Utilities|Array|RemoveItem (Variables|Default|GetCharacterCurrentlyIn%20) _asbp_first_person_character)
    (Utilities|Time|ClearandInvalidateTimerbyHandle (.Value (Utilities|Map|Find (Variables|Default|GetCooldownAndPlayer) _asbp_first_person_character)))
    (Utilities|Time|UnpauseTimerbyHandle (Variables|Default|GetDestroyTimerHandle))))

(event Custom|SetTimer
  (params (TimeBeforeEnd :type Float%20%28double-precision%29))
  (bind _returnvalue (Utilities|Time|SetTimerbyEvent (delegate Custom|DestroyExtraction) TimeBeforeEnd))
  (Variables|Default|SetDestroyTimerHandle _returnvalue))

(event Custom|DestroyExtraction
  (Default|CallFinishedExtraction (Variables|Default|GetGameState)))

(event Custom|StartExtraction
  ;[0.15 0.15 0.15 0.5] Logic For Adding Point Each Tick
  (CallFunction|StartExtractionFunction (stale EventTick _array_element)))

(event EventTick
  (params (DeltaSeconds :type Float%20%28single-precision%29))
  ;[0.15 0.15 0.15 0.5] Logic For Adding Point Each Tick
  (Networking|SwitchHasAuthority
    (:Authority
      (if (== (Variables|Default|GetRoundCashValue) (Variables|Default|GetTotalBanked))
        (Utilities|Time|ClearandInvalidateTimerbyHandle (Variables|Default|GetDestroyTimerHandle))
        (CallFunction|DestroyExtraction)
        (elif (> (Utilities|Array|Length (Variables|Default|GetCharacterCurrentlyIn%20)) 0)
          (if (not (Variables|Default|GetBusyRn))
            (for _array_element (Variables|Default|GetCharacterCurrentlyIn%20)
              (if (> (Variables|/Game/Blueprints/Player/BP_FirstPersonCharacter.BP_FirstPersonCharacter_C|GetDataPossesed _array_element) 0.0)
                (if (not (Utilities|Time|IsValidTimerHandle (.Value (Utilities|Map|Find (Variables|Default|GetCooldownAndPlayer) _array_element))))
                  (bind _returnvalue (Utilities|Time|SetTimerbyEvent (delegate Custom|StartExtraction) (Variables|Default|GetTimeForCashout)))
                  (Utilities|Map|Add (Variables|Default|GetCooldownAndPlayer) _array_element _returnvalue)
                  (Variables|Default|SetBusyRn true)
                  (Utilities|Time|PauseTimerbyHandle (Variables|Default|GetDestroyTimerHandle))))))
          (else
            (Variables|Default|SetBusyRn false)))))))

(fn ConstructionScript)

(fn StartExtractionFunction
  (params (Player :type BP%20First%20Person%20Character%20Object%20Reference))
  (bind _gamestate (Variables|Default|GetGameState))
  (bind _teammateref (Variables|/Game/Blueprints/Player/BP_FirstPersonCharacter.BP_FirstPersonCharacter_C|GetTeamMateRef Player))
  (bind _playerandcontroller (Variables|/Game/Blueprints/GameMode/BP_GameState.BP_GameState_C|GetPlayerAndController _gamestate))
  (bind _teams (Variables|/Game/Blueprints/GameMode/BP_GameState.BP_GameState_C|GetTeams _gamestate))
  (bind _value (Utilities|Map|Find _playerandcontroller Player))
  (bind _teamindex (Variables|/Game/Blueprints/Player/BP_FirstPersonPlayerController.BP_FirstPersonPlayerController_C|GetTeamIndex _value))
  (bind _output (Utilities|Array|Get(acopy) _teams _teamindex))
  (if (> (Variables|/Game/Blueprints/Player/BP_FirstPersonCharacter.BP_FirstPersonCharacter_C|GetDataPossesed Player) 0.0)
    (Variables|Default|SetDataBanked (+ (.DataBanked (Utilities|Struct|BreakPlayerArray _output)) (Variables|/Game/Blueprints/Player/BP_FirstPersonCharacter.BP_FirstPersonCharacter_C|GetDataPossesed Player)))
    (Variables|Default|SetTotalBanked (+ (Variables|Default|GetTotalBanked) (Variables|/Game/Blueprints/Player/BP_FirstPersonCharacter.BP_FirstPersonCharacter_C|GetDataPossesed Player)))
    (Variables|/Game/Blueprints/Player/BP_FirstPersonCharacter.BP_FirstPersonCharacter_C|SetDataPossesed Player 0.0)
    (Utilities|IsValid _teammateref
      (:Is%20Valid
        (Variables|/Game/Blueprints/Player/BP_FirstPersonCharacter.BP_FirstPersonCharacter_C|SetDataPossesed _teammateref 0.0))
      (:Is%20Not%20Valid
        _))
    (bind _structout (Utilities|Struct|SetmembersinPlayerArray _output (Variables|Default|GetDataBanked)))
    (Utilities|Array|SetArrayElem _teams _teamindex _structout)
    (Default|UpdateScore (Variables|Default|GetGameState) _output)
    (Utilities|Time|ClearandInvalidateTimerbyHandle (.Value (Utilities|Map|Find (Variables|Default|GetCooldownAndPlayer) Player)))
    (Variables|Default|SetBusyRn false)
    (Utilities|Time|UnpauseTimerbyHandle (Variables|Default|GetDestroyTimerHandle))))