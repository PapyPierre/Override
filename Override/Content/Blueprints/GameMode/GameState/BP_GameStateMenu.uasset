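; Menu GameState that runs the multiplayer lobby: team and spectator slots, ready states and the timed pre-match selection phase.
; RPC events update the open lobby widget on remote machines, while the authority counts team players into BP_GameInstance.
; OnRep handlers toggle the host's play button from ready and player counts.
; StartSelection shows each controller's selection with teammate names, ability picks are relayed to teammates, and timer expiry calls GameMode.CallNewMap.
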(event Custom|OnTimerEnd
  (Default|CallNewMap (Variables|Default|GetGameMode)))

(event Custom|StartSelection
  (bind _new_player (Variables|Default|GetNew%20Player))
  (bind _returnvalue (Utilities|Time|SetTimerbyEvent (delegate Custom|OnTimerEnd) (Variables|Default|GetSelectionTime)))
  (Variables|Default|SetTimer%20Handle _returnvalue)
  (for _array_element _new_player
    (Default|ShowSelection _array_element)
    (for _array_element_2 _new_player
      (if (and (== (Variables|/Game/Blueprints/Controller/BP_ControllerMenu.BP_ControllerMenu_C|GetSelectedTeam _array_element) (Variables|/Game/Blueprints/Controller/BP_ControllerMenu.BP_ControllerMenu_C|GetSelectedTeam _array_element_2)) (!= _array_element_2 _array_element))
        (Default|SetTextTeammate _array_element (Utilities|Text|ToText(String) (Variables|/Game/Blueprints/Controller/BP_FirstPersonPlayerController.BP_FirstPersonPlayerController_C|GetUserName _array_element_2)))))))

(event Custom|WidgetText
  (params (Controllers :type String) (Index :type Integer) (Player :type Integer) (Target :type BP%20Controller%20Menu%20Object%20Reference))
  (Default|RPCUpdateTextLobby Target Index Controllers Player))

(event Custom|Multicast_ReadyUpUI
  (params (TeamIndex :type Integer) (PlayerPosition :type Integer) (Ready :type Boolean))
  (Networking|SwitchHasAuthority
    (:Remote
      (bind _asbp_controller_menu (Utilities|Casting|CastToBP_ControllerMenu (Game|GetPlayerController 0)))
      (bind _openedlobby (Variables|/Game/Blueprints/Controller/BP_ControllerMenu.BP_ControllerMenu_C|GetOpenedLobby _asbp_controller_menu)
        (:then
          (Default|UpdateLobbyStatusPreview _openedlobby TeamIndex PlayerPosition (Math|Integer|SelectInt 2 1 Ready))
          (Variables|/Script/UMG.Widget|SetRenderOpacity (Utilities|Select :Index PlayerPosition :Option%200 (Variables|/Game/Blueprints/Widget/Menu/WBP_UserBox.WBP_UserBox_C|GetReadyState1 (Utilities|Select :Index TeamIndex :Option%200 (Variables|/Game/Blueprints/Widget/Menu/WBP_Lobby.WBP_Lobby_C|GetTeam1 _openedlobby) :Option%201 (Variables|/Game/Blueprints/Widget/Menu/WBP_Lobby.WBP_Lobby_C|GetTeam2 _openedlobby) :Option%202 (Variables|/Game/Blueprints/Widget/Menu/WBP_Lobby.WBP_Lobby_C|GetTeam3 _openedlobby))) :Option%201 (Variables|/Game/Blueprints/Widget/Menu/WBP_UserBox.WBP_UserBox_C|GetReadyState2 (Utilities|Select :Index TeamIndex :Option%200 (Variables|/Game/Blueprints/Widget/Menu/WBP_Lobby.WBP_Lobby_C|GetTeam1 _openedlobby) :Option%201 (Variables|/Game/Blueprints/Widget/Menu/WBP_Lobby.WBP_Lobby_C|GetTeam2 _openedlobby) :Option%202 (Variables|/Game/Blueprints/Widget/Menu/WBP_Lobby.WBP_Lobby_C|GetTeam3 _openedlobby)))) (Math|Float|SelectFloat 1.0 0.0 Ready)))
        (:else)))))

(event Custom|RPC_CleanOldTeam
  (params (OldTeam :type Integer) (Index :type Integer))
  (bind _color (Math|Color|MakeColor 255 255 255 102))
  (bind _slatecolor (Utilities|Struct|MakeSlateColor "(R=0.035601,G=0.056128,B=0.097587,A=0.400000)"))
  (bind _asbp_controller_menu (Utilities|Casting|CastToBP_ControllerMenu (Game|GetPlayerController 0)))
  (bind _openedlobby (Variables|/Game/Blueprints/Controller/BP_ControllerMenu.BP_ControllerMenu_C|GetOpenedLobby _asbp_controller_menu)
    (:then
      (Networking|SwitchHasAuthority
        (:Remote
          (if (!= OldTeam -1)
            (if (== OldTeam 3)
              (Rendering|Components|TextRender|SetText (Variables|/Game/Blueprints/Widget/Menu/WBP_Spec.WBP_Spec_C|GetPlayer1 (Variables|/Game/Blueprints/Widget/Menu/WBP_Lobby.WBP_Lobby_C|GetWBP_Spec _openedlobby)) "SPECTATE")
              (Default|SetBackgroundColor (Variables|/Game/Blueprints/Widget/Menu/WBP_Spec.WBP_Spec_C|GetSlot1Background (Variables|/Game/Blueprints/Widget/Menu/WBP_Lobby.WBP_Lobby_C|GetWBP_Spec _openedlobby)) _color)
              (Appearance|SetColorandOpacity (Variables|/Game/Blueprints/Widget/Menu/WBP_Spec.WBP_Spec_C|GetPlayer1 (Variables|/Game/Blueprints/Widget/Menu/WBP_Lobby.WBP_Lobby_C|GetWBP_Spec _openedlobby)) _slatecolor :!class /Script/UMG.TextBlock)
              (Widget|SetRenderOpacity (Variables|/Game/Blueprints/Widget/Menu/WBP_Spec.WBP_Spec_C|GetJoin1LeftArrow (Variables|/Game/Blueprints/Widget/Menu/WBP_Lobby.WBP_Lobby_C|GetWBP_Spec _openedlobby)) 1.0)
              (Widget|SetRenderOpacity (Variables|/Game/Blueprints/Widget/Menu/WBP_Spec.WBP_Spec_C|GetJoin1RightArrow (Variables|/Game/Blueprints/Widget/Menu/WBP_Lobby.WBP_Lobby_C|GetWBP_Spec _openedlobby)) 1.0)
              (else
                (Rendering|Components|TextRender|SetText (Utilities|Select :Index Index :Option%200 (Variables|/Game/Blueprints/Widget/Menu/WBP_UserBox.WBP_UserBox_C|GetPlayer1 (Utilities|Select :Index OldTeam :Option%200 (Variables|/Game/Blueprints/Widget/Menu/WBP_Lobby.WBP_Lobby_C|GetTeam1 _openedlobby) :Option%201 (Variables|/Game/Blueprints/Widget/Menu/WBP_Lobby.WBP_Lobby_C|GetTeam2 _openedlobby) :Option%202 (Variables|/Game/Blueprints/Widget/Menu/WBP_Lobby.WBP_Lobby_C|GetTeam3 _openedlobby))) :Option%201 (Variables|/Game/Blueprints/Widget/Menu/WBP_UserBox.WBP_UserBox_C|GetPlayer2 (Utilities|Select :Index OldTeam :Option%200 (Variables|/Game/Blueprints/Widget/Menu/WBP_Lobby.WBP_Lobby_C|GetTeam1 _openedlobby) :Option%201 (Variables|/Game/Blueprints/Widget/Menu/WBP_Lobby.WBP_Lobby_C|GetTeam2 _openedlobby) :Option%202 (Variables|/Game/Blueprints/Widget/Menu/WBP_Lobby.WBP_Lobby_C|GetTeam3 _openedlobby)))) "JOIN")
                (Default|SetBackgroundColor (Utilities|Select :Index Index :Option%200 (Variables|/Game/Blueprints/Widget/Menu/WBP_UserBox.WBP_UserBox_C|GetSlot1Background (Utilities|Select :Index OldTeam :Option%200 (Variables|/Game/Blueprints/Widget/Menu/WBP_Lobby.WBP_Lobby_C|GetTeam1 _openedlobby) :Option%201 (Variables|/Game/Blueprints/Widget/Menu/WBP_Lobby.WBP_Lobby_C|GetTeam2 _openedlobby) :Option%202 (Variables|/Game/Blueprints/Widget/Menu/WBP_Lobby.WBP_Lobby_C|GetTeam3 _openedlobby))) :Option%201 (Variables|/Game/Blueprints/Widget/Menu/WBP_UserBox.WBP_UserBox_C|GetSlot2Background (Utilities|Select :Index OldTeam :Option%200 (Variables|/Game/Blueprints/Widget/Menu/WBP_Lobby.WBP_Lobby_C|GetTeam1 _openedlobby) :Option%201 (Variables|/Game/Blueprints/Widget/Menu/WBP_Lobby.WBP_Lobby_C|GetTeam2 _openedlobby) :Option%202 (Variables|/Game/Blueprints/Widget/Menu/WBP_Lobby.WBP_Lobby_C|GetTeam3 _openedlobby)))) _color)
                (Appearance|SetColorandOpacity (Utilities|Select :Index Index :Option%200 (Variables|/Game/Blueprints/Widget/Menu/WBP_UserBox.WBP_UserBox_C|GetPlayer1 (Utilities|Select :Index OldTeam :Option%200 (Variables|/Game/Blueprints/Widget/Menu/WBP_Lobby.WBP_Lobby_C|GetTeam1 _openedlobby) :Option%201 (Variables|/Game/Blueprints/Widget/Menu/WBP_Lobby.WBP_Lobby_C|GetTeam2 _openedlobby) :Option%202 (Variables|/Game/Blueprints/Widget/Menu/WBP_Lobby.WBP_Lobby_C|GetTeam3 _openedlobby))) :Option%201 (Variables|/Game/Blueprints/Widget/Menu/WBP_UserBox.WBP_UserBox_C|GetPlayer2 (Utilities|Select :Index OldTeam :Option%200 (Variables|/Game/Blueprints/Widget/Menu/WBP_Lobby.WBP_Lobby_C|GetTeam1 _openedlobby) :Option%201 (Variables|/Game/Blueprints/Widget/Menu/WBP_Lobby.WBP_Lobby_C|GetTeam2 _openedlobby) :Option%202 (Variables|/Game/Blueprints/Widget/Menu/WBP_Lobby.WBP_Lobby_C|GetTeam3 _openedlobby)))) _slatecolor :!class /Script/UMG.TextBlock)
                (Widget|SetRenderOpacity (Utilities|Select :Index Index :Option%200 (Variables|/Game/Blueprints/Widget/Menu/WBP_UserBox.WBP_UserBox_C|GetJoin1LeftArrow (Utilities|Select :Index OldTeam :Option%200 (Variables|/Game/Blueprints/Widget/Menu/WBP_Lobby.WBP_Lobby_C|GetTeam1 _openedlobby) :Option%201 (Variables|/Game/Blueprints/Widget/Menu/WBP_Lobby.WBP_Lobby_C|GetTeam2 _openedlobby) :Option%202 (Variables|/Game/Blueprints/Widget/Menu/WBP_Lobby.WBP_Lobby_C|GetTeam3 _openedlobby))) :Option%201 (Variables|/Game/Blueprints/Widget/Menu/WBP_UserBox.WBP_UserBox_C|GetJoin2LeftArrow (Utilities|Select :Index OldTeam :Option%200 (Variables|/Game/Blueprints/Widget/Menu/WBP_Lobby.WBP_Lobby_C|GetTeam1 _openedlobby) :Option%201 (Variables|/Game/Blueprints/Widget/Menu/WBP_Lobby.WBP_Lobby_C|GetTeam2 _openedlobby) :Option%202 (Variables|/Game/Blueprints/Widget/Menu/WBP_Lobby.WBP_Lobby_C|GetTeam3 _openedlobby)))) 1.0)
                (Widget|SetRenderOpacity (Utilities|Select :Index Index :Option%200 (Variables|/Game/Blueprints/Widget/Menu/WBP_UserBox.WBP_UserBox_C|GetJoin1RightArrow (Utilities|Select :Index OldTeam :Option%200 (Variables|/Game/Blueprints/Widget/Menu/WBP_Lobby.WBP_Lobby_C|GetTeam1 _openedlobby) :Option%201 (Variables|/Game/Blueprints/Widget/Menu/WBP_Lobby.WBP_Lobby_C|GetTeam2 _openedlobby) :Option%202 (Variables|/Game/Blueprints/Widget/Menu/WBP_Lobby.WBP_Lobby_C|GetTeam3 _openedlobby))) :Option%201 (Variables|/Game/Blueprints/Widget/Menu/WBP_UserBox.WBP_UserBox_C|GetJoin2RightArrow (Utilities|Select :Index OldTeam :Option%200 (Variables|/Game/Blueprints/Widget/Menu/WBP_Lobby.WBP_Lobby_C|GetTeam1 _openedlobby) :Option%201 (Variables|/Game/Blueprints/Widget/Menu/WBP_Lobby.WBP_Lobby_C|GetTeam2 _openedlobby) :Option%202 (Variables|/Game/Blueprints/Widget/Menu/WBP_Lobby.WBP_Lobby_C|GetTeam3 _openedlobby)))) 1.0)
                (Default|UpdateLobbyStatusPreview _openedlobby OldTeam Index)))))))
    (:else)))

(event Custom|RPC_SetPlayerInNewTeam
  (params (Controllers :type String) (Index :type Integer) (OldTeam :type Integer) (Player :type Integer))
  (bind _asbp_controller_menu (Utilities|Casting|CastToBP_ControllerMenu (Game|GetPlayerController 0)))
  (Networking|SwitchHasAuthority
    (:Authority
      (if (== OldTeam -1)
        (Networking|SwitchHasAuthority
          (:Authority
            (if (!= Index 3)
              (bind _asbp_game_instance (Utilities|Casting|CastToBP_GameInstance (Game|GetGameInstance)))
              (Variables|/Game/Blueprints/GameMode/GameInstance/BP_GameInstance.BP_GameInstance_C|SetPlayerNumber _asbp_game_instance (+ (Variables|Default|GetPlayerInTeam) 1))
              (Variables|Default|SetPlayerInTeam (+ (Variables|Default|GetPlayerInTeam) 1)))))))
    (:Remote
      (CallFunction|SetPlayerinNewTeam Controllers Index Player _asbp_controller_menu))))

(event Custom|UpdateTeam
  (params (Target :type BP%20Controller%20Menu%20Object%20Reference))
  (for _array_element (Variables|Default|GetNew%20Player)
    (if (!= (Variables|/Game/Blueprints/Controller/BP_ControllerMenu.BP_ControllerMenu_C|GetSelectedTeam _array_element) -1)
      (CallFunction|WidgetText (Variables|/Game/Blueprints/Controller/BP_FirstPersonPlayerController.BP_FirstPersonPlayerController_C|GetUserName _array_element) (Variables|/Game/Blueprints/Controller/BP_ControllerMenu.BP_ControllerMenu_C|GetSelectedTeam _array_element) (Variables|/Game/Blueprints/Controller/BP_ControllerMenu.BP_ControllerMenu_C|GetOldSlot _array_element) Target))))

(event Custom|Debug%20Load%20New%20Map
  (Default|CallNewMap (Variables|Default|GetGameMode)))

(event Custom|AbilitySelectNotify
  (params (TeamIndex :type Integer) (Controller :type BP%20Controller%20Menu%20Object%20Reference) (Slot%20Index :type Integer) (Ability :type GA%20Base%20Ability%20Class%20Reference) (SkillSelected :type Integer))
  (for _array_element (Variables|Default|GetNew%20Player)
    (if (not (== _array_element Controller))
      (if (== (Variables|/Game/Blueprints/Controller/BP_ControllerMenu.BP_ControllerMenu_C|GetSelectedTeam _array_element) TeamIndex)
        (Default|TeammateAbilitySelectNotify _array_element Slot%20Index Ability SkillSelected)))))

(event EventTick
  (params (DeltaSeconds :type Float%20%28single-precision%29))
  (bind _timer_handle (Variables|Default|GetTimer%20Handle))
  (Networking|SwitchHasAuthority
    (:Authority
      (if (Utilities|Time|IsValidTimerHandle _timer_handle)
        (Variables|Default|SetSelectionRemainingTime (Utilities|Time|GetTimerRemainingTimebyHandle _timer_handle))))))

(event EventBeginPlay
  (Networking|SwitchHasAuthority
    (:Authority
      (bind _asbp_game_instance (Utilities|Casting|CastToBP_GameInstance (Game|GetGameInstance)))
      (Variables|Default|SetAs%20BP%20Game%20Instance _asbp_game_instance))))

(fn ConstructionScript)

(fn SetPlayerinNewTeam
  (params (Username :type String) (Previous%20Team%20Index :type Integer) (Player%20Index :type Integer) (Controller :type BP%20Controller%20Menu%20Object%20Reference))
  (bind _returnvalue (Utilities|String|Append "- " Username))
  (bind _color (Math|Color|MakeColor 255 255 255 255))
  (bind _returnvalue_2 (Utilities|Text|ToText(String) _returnvalue))
  (bind _openedlobby (Variables|/Game/Blueprints/Controller/BP_ControllerMenu.BP_ControllerMenu_C|GetOpenedLobby Controller)
    (:then
      (if (== Previous%20Team%20Index 3)
        (Rendering|Components|TextRender|SetText (Variables|/Game/Blueprints/Widget/Menu/WBP_Spec.WBP_Spec_C|GetPlayer1 (Variables|/Game/Blueprints/Widget/Menu/WBP_Lobby.WBP_Lobby_C|GetWBP_Spec _openedlobby)) _returnvalue_2)
        (Default|SetBackgroundColor (Variables|/Game/Blueprints/Widget/Menu/WBP_Spec.WBP_Spec_C|GetSlot1Background (Variables|/Game/Blueprints/Widget/Menu/WBP_Lobby.WBP_Lobby_C|GetWBP_Spec _openedlobby)) _color)
        (Appearance|SetColorandOpacity (Variables|/Game/Blueprints/Widget/Menu/WBP_Spec.WBP_Spec_C|GetPlayer1 (Variables|/Game/Blueprints/Widget/Menu/WBP_Lobby.WBP_Lobby_C|GetWBP_Spec _openedlobby)) (Utilities|Struct|MakeSlateColor "(R=0.035601,G=0.056128,B=0.097587,A=1.000000)") :!class /Script/UMG.TextBlock)
        (Widget|SetRenderOpacity (Variables|/Game/Blueprints/Widget/Menu/WBP_Spec.WBP_Spec_C|GetJoin1LeftArrow (Variables|/Game/Blueprints/Widget/Menu/WBP_Lobby.WBP_Lobby_C|GetWBP_Spec _openedlobby)) 0.0)
        (Widget|SetRenderOpacity (Variables|/Game/Blueprints/Widget/Menu/WBP_Spec.WBP_Spec_C|GetJoin1RightArrow (Variables|/Game/Blueprints/Widget/Menu/WBP_Lobby.WBP_Lobby_C|GetWBP_Spec _openedlobby)) 0.0)
        (else
          (Rendering|Components|TextRender|SetText (Utilities|Select :Index Player%20Index :Option%200 (Variables|/Game/Blueprints/Widget/Menu/WBP_UserBox.WBP_UserBox_C|GetPlayer1 (Utilities|Select :Index Previous%20Team%20Index :Option%200 (Variables|/Game/Blueprints/Widget/Menu/WBP_Lobby.WBP_Lobby_C|GetTeam1 _openedlobby) :Option%201 (Variables|/Game/Blueprints/Widget/Menu/WBP_Lobby.WBP_Lobby_C|GetTeam2 _openedlobby) :Option%202 (Variables|/Game/Blueprints/Widget/Menu/WBP_Lobby.WBP_Lobby_C|GetTeam3 _openedlobby))) :Option%201 (Variables|/Game/Blueprints/Widget/Menu/WBP_UserBox.WBP_UserBox_C|GetPlayer2 (Utilities|Select :Index Previous%20Team%20Index :Option%200 (Variables|/Game/Blueprints/Widget/Menu/WBP_Lobby.WBP_Lobby_C|GetTeam1 _openedlobby) :Option%201 (Variables|/Game/Blueprints/Widget/Menu/WBP_Lobby.WBP_Lobby_C|GetTeam2 _openedlobby) :Option%202 (Variables|/Game/Blueprints/Widget/Menu/WBP_Lobby.WBP_Lobby_C|GetTeam3 _openedlobby)))) _returnvalue_2)
          (Default|UpdateLobbyStatusPreview _openedlobby Previous%20Team%20Index Player%20Index 1)
          (Default|SetBackgroundColor (Utilities|Select :Index Player%20Index :Option%200 (Variables|/Game/Blueprints/Widget/Menu/WBP_UserBox.WBP_UserBox_C|GetSlot1Background (Utilities|Select :Index Previous%20Team%20Index :Option%200 (Variables|/Game/Blueprints/Widget/Menu/WBP_Lobby.WBP_Lobby_C|GetTeam1 _openedlobby) :Option%201 (Variables|/Game/Blueprints/Widget/Menu/WBP_Lobby.WBP_Lobby_C|GetTeam2 _openedlobby) :Option%202 (Variables|/Game/Blueprints/Widget/Menu/WBP_Lobby.WBP_Lobby_C|GetTeam3 _openedlobby))) :Option%201 (Variables|/Game/Blueprints/Widget/Menu/WBP_UserBox.WBP_UserBox_C|GetSlot2Background (Utilities|Select :Index Previous%20Team%20Index :Option%200 (Variables|/Game/Blueprints/Widget/Menu/WBP_Lobby.WBP_Lobby_C|GetTeam1 _openedlobby) :Option%201 (Variables|/Game/Blueprints/Widget/Menu/WBP_Lobby.WBP_Lobby_C|GetTeam2 _openedlobby) :Option%202 (Variables|/Game/Blueprints/Widget/Menu/WBP_Lobby.WBP_Lobby_C|GetTeam3 _openedlobby)))) _color)
          (Appearance|SetColorandOpacity (Utilities|Select :Index Player%20Index :Option%200 (Variables|/Game/Blueprints/Widget/Menu/WBP_UserBox.WBP_UserBox_C|GetPlayer1 (Utilities|Select :Index Previous%20Team%20Index :Option%200 (Variables|/Game/Blueprints/Widget/Menu/WBP_Lobby.WBP_Lobby_C|GetTeam1 _openedlobby) :Option%201 (Variables|/Game/Blueprints/Widget/Menu/WBP_Lobby.WBP_Lobby_C|GetTeam2 _openedlobby) :Option%202 (Variables|/Game/Blueprints/Widget/Menu/WBP_Lobby.WBP_Lobby_C|GetTeam3 _openedlobby))) :Option%201 (Variables|/Game/Blueprints/Widget/Menu/WBP_UserBox.WBP_UserBox_C|GetPlayer2 (Utilities|Select :Index Previous%20Team%20Index :Option%200 (Variables|/Game/Blueprints/Widget/Menu/WBP_Lobby.WBP_Lobby_C|GetTeam1 _openedlobby) :Option%201 (Variables|/Game/Blueprints/Widget/Menu/WBP_Lobby.WBP_Lobby_C|GetTeam2 _openedlobby) :Option%202 (Variables|/Game/Blueprints/Widget/Menu/WBP_Lobby.WBP_Lobby_C|GetTeam3 _openedlobby)))) (Utilities|Struct|MakeSlateColor "(R=0.035601,G=0.056128,B=0.097587,A=1.000000)") :!class /Script/UMG.TextBlock)
          (Widget|SetRenderOpacity (Utilities|Select :Index Player%20Index :Option%200 (Variables|/Game/Blueprints/Widget/Menu/WBP_UserBox.WBP_UserBox_C|GetJoin1LeftArrow (Utilities|Select :Index Previous%20Team%20Index :Option%200 (Variables|/Game/Blueprints/Widget/Menu/WBP_Lobby.WBP_Lobby_C|GetTeam1 _openedlobby) :Option%201 (Variables|/Game/Blueprints/Widget/Menu/WBP_Lobby.WBP_Lobby_C|GetTeam2 _openedlobby) :Option%202 (Variables|/Game/Blueprints/Widget/Menu/WBP_Lobby.WBP_Lobby_C|GetTeam3 _openedlobby))) :Option%201 (Variables|/Game/Blueprints/Widget/Menu/WBP_UserBox.WBP_UserBox_C|GetJoin2LeftArrow (Utilities|Select :Index Previous%20Team%20Index :Option%200 (Variables|/Game/Blueprints/Widget/Menu/WBP_Lobby.WBP_Lobby_C|GetTeam1 _openedlobby) :Option%201 (Variables|/Game/Blueprints/Widget/Menu/WBP_Lobby.WBP_Lobby_C|GetTeam2 _openedlobby) :Option%202 (Variables|/Game/Blueprints/Widget/Menu/WBP_Lobby.WBP_Lobby_C|GetTeam3 _openedlobby)))) 0.0)
          (Widget|SetRenderOpacity (Utilities|Select :Index Player%20Index :Option%200 (Variables|/Game/Blueprints/Widget/Menu/WBP_UserBox.WBP_UserBox_C|GetJoin1RightArrow (Utilities|Select :Index Previous%20Team%20Index :Option%200 (Variables|/Game/Blueprints/Widget/Menu/WBP_Lobby.WBP_Lobby_C|GetTeam1 _openedlobby) :Option%201 (Variables|/Game/Blueprints/Widget/Menu/WBP_Lobby.WBP_Lobby_C|GetTeam2 _openedlobby) :Option%202 (Variables|/Game/Blueprints/Widget/Menu/WBP_Lobby.WBP_Lobby_C|GetTeam3 _openedlobby))) :Option%201 (Variables|/Game/Blueprints/Widget/Menu/WBP_UserBox.WBP_UserBox_C|GetJoin2RightArrow (Utilities|Select :Index Previous%20Team%20Index :Option%200 (Variables|/Game/Blueprints/Widget/Menu/WBP_Lobby.WBP_Lobby_C|GetTeam1 _openedlobby) :Option%201 (Variables|/Game/Blueprints/Widget/Menu/WBP_Lobby.WBP_Lobby_C|GetTeam2 _openedlobby) :Option%202 (Variables|/Game/Blueprints/Widget/Menu/WBP_Lobby.WBP_Lobby_C|GetTeam3 _openedlobby)))) 0.0))))
    (:else)))

(fn OnRepPlayerReady
  (Networking|SwitchHasAuthority
    (:Authority
      (Default|AddorRemovePlayButton (Variables|Default|GetHost) (or (and (>= (Variables|Default|GetPlayerReady) (Variables|/Game/Blueprints/GameMode/GameInstance/BP_GameInstance.BP_GameInstance_C|GetPlayerNumber (Variables|Default|GetAs%20BP%20Game%20Instance))) (!= (Variables|Default|GetPlayerReady) 0)) (== (Variables|/Game/Blueprints/GameMode/GameInstance/BP_GameInstance.BP_GameInstance_C|GetPlayerNumber (Variables|Default|GetAs%20BP%20Game%20Instance)) 1))))))

(fn OnRepPlayerinTeam
  (Networking|SwitchHasAuthority
    (:Authority
      (Default|AddorRemovePlayButton (Variables|Default|GetHost) (or (and (>= (Variables|Default|GetPlayerReady) (Variables|/Game/Blueprints/GameMode/GameInstance/BP_GameInstance.BP_GameInstance_C|GetPlayerNumber (Variables|Default|GetAs%20BP%20Game%20Instance))) (!= (Variables|Default|GetPlayerReady) 0)) (== (Variables|Default|GetPlayerInTeam) 1))))))