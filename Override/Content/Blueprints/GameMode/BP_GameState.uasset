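; Game state for a team data-banking mode: it tracks the active collect point, cash-out point and team scores.
; It relays emptied points and finished extractions to the GameMode, and flags game over when a team banks enough data.
; Round data removed before a cash-out point exists is held until one arrives.
; It also handles team switching with teammate links and delayed recoloring, death data-pack drops and respawn calls.
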(event Custom|RemoveRoundData
  (params (Data :type Integer))
  (bind _currentcashoutpoint (Variables|Default|GetCurrentCashOutPoint))
  (Utilities|IsValid _currentcashoutpoint
    (:Is%20Valid
      (Variables|/Game/Blueprints/GameMode/BP_CashOutPoint.BP_CashOutPoint_C|SetRoundCashValue _currentcashoutpoint (- (Variables|/Game/Blueprints/GameMode/BP_CashOutPoint.BP_CashOutPoint_C|GetRoundCashValue _currentcashoutpoint) Data)))
    (:Is%20Not%20Valid
      (Variables|Default|SetDataToRemove Data))))

(event Custom|Extraction%20Finished
  (Actor|DestroyActor (Variables|Default|GetCurrentCashOutPoint))
  (Default|CallExtractionFinished (Variables|Default|GetGameMode)))

(event Custom|ShareScore
  (params (Key :type BP%20First%20Person%20Character%20Object%20Reference%20%28by%20ref%29) (Data :type Integer))
  (Default|SetHUDScore Key (Variables|/Game/Blueprints/Player/BP_FirstPersonPlayerController.BP_FirstPersonPlayerController_C|GetTeamIndex (.Value (Utilities|Map|Find (Variables|Default|GetPlayerAndController) Key))) self Data))

(event Custom|Multicast%20Spawn%20DataPack
  (params (Data :type Float%20%28double-precision%29) (Transform :type Transform))
  ;[0.15 0.15 0.15 0.5] Data Pack Drop When Player Die
  (bind _returnvalue (Game|SpawnActorfromClass "/Game/Blueprints/Collectible/BP_DataPack.BP_DataPack_C" Transform "Undefined" "MultiplyWithRoot" 0 0))
  (Default|SetData _returnvalue Data))

(event Custom|ReplicateCollectPoint
  (params (Actor :type Actor%20Object%20Reference))
  ;[0.15 0.15 0.15 0.5] Replication Collect Point
  (bind _asbp_collect_point (Utilities|Casting|CastToBP_CollectPoint Actor))
  (bind _output_get (Variables|Default|SetCurrentDataPoint _asbp_collect_point))
  (Variables|/Game/Blueprints/GameMode/BP_CollectPoint.BP_CollectPoint_C|SetGameState _output_get self)
  (EventDispatchers|BindEventtoEmptyDataPoint (delegate Custom|Data%20Point%20Empty)))

(event Custom|ReplicateCashOut
  (params (ExtractPoint :type Actor%20Object%20Reference) (MaxRoundValue :type Integer))
  (bind _asbp_cash_out_point (Utilities|Casting|CastToBP_CashOutPoint ExtractPoint))
  (bind _output_get (Variables|Default|SetCurrentCashOutPoint _asbp_cash_out_point))
  (Variables|/Game/Blueprints/GameMode/BP_CashOutPoint.BP_CashOutPoint_C|SetGameState _output_get self)
  (Variables|/Game/Blueprints/GameMode/BP_CashOutPoint.BP_CashOutPoint_C|SetRoundCashValue _asbp_cash_out_point (- MaxRoundValue (Variables|Default|GetDataToRemove)))
  (EventDispatchers|BindEventtoFinishedExtraction (delegate Custom|Extraction%20Finished))
  (Variables|Default|SetDataToRemove 0))

(event Custom|DisableCollisionActor
  (params (Actor :type BP%20First%20Person%20Character%20Object%20Reference))
  (Collision|SetActorEnableCollision Actor false))

(event Custom|Data%20Point%20Empty
  ;[0.15 0.15 0.15 0.5] Replication Collect Point
  (Actor|DestroyActor (Variables|Default|GetCurrentDataPoint))
  (Default|CallDataPointEmpty (Variables|Default|GetGameMode)))

(event Custom|UpdateScore
  (params (Team :type Player%20Array%20Structure))
  (bind (_player _databanked) (Utilities|Struct|BreakPlayerArray Team))
  ;[0.15 0.15 0.15 0.5] Update UI Team Score
  (for _array_element _player
    (Default|UpdateOwnScore (Variables|/Game/Blueprints/Player/BP_FirstPersonPlayerController.BP_FirstPersonPlayerController_C|GetPlayerOwning _array_element) _databanked (Variables|/Game/Blueprints/Player/BP_FirstPersonPlayerController.BP_FirstPersonPlayerController_C|GetTeamIndex _array_element)))
  (if (>= _databanked (Variables|Default|GetMaxData))
    (Variables|/Game/Blueprints/GameMode/BP_FirstPersonGameMode.BP_FirstPersonGameMode_C|SetGameOver (Variables|Default|GetGameMode) true)))

(event Custom|RemoveOrAddInput
  (params (PlayerController :type BP%20First%20Person%20Player%20Controller%20Object%20Reference) (Condition :type Boolean))
  (Default|OwningRemoveorAddInput PlayerController Condition))

(event Custom|ChangeTeam
  (params (Character :type BP%20First%20Person%20Character%20Object%20Reference) (NewTeam :type Integer))
  (bind _playerandcontroller (Variables|Default|GetPlayerAndController))
  (bind _teams (Variables|Default|GetTeams))
  (bind _value (Utilities|Map|Find _playerandcontroller Character))
  (bind _output (Utilities|Array|Get(acopy) _teams NewTeam))
  (bind _player (Utilities|Struct|BreakPlayerArray _output))
  (if (!= NewTeam (Variables|/Game/Blueprints/Player/BP_FirstPersonPlayerController.BP_FirstPersonPlayerController_C|GetTeamIndex _value))
    (Utilities|Array|RemoveItem (.Player (Utilities|Struct|BreakPlayerArray (Utilities|Array|Get(acopy) (Variables|Default|GetTeams) (Variables|/Game/Blueprints/Player/BP_FirstPersonPlayerController.BP_FirstPersonPlayerController_C|GetTeamIndex _value)))) _value)
    (Utilities|Array|Resize (.Player (Utilities|Struct|BreakPlayerArray (Utilities|Array|Get(acopy) (Variables|Default|GetTeams) (Variables|/Game/Blueprints/Player/BP_FirstPersonPlayerController.BP_FirstPersonPlayerController_C|GetTeamIndex _value)))) (Utilities|Array|Length (.Player (Utilities|Struct|BreakPlayerArray (Utilities|Array|Get(acopy) (Variables|Default|GetTeams) (Variables|/Game/Blueprints/Player/BP_FirstPersonPlayerController.BP_FirstPersonPlayerController_C|GetTeamIndex _value))))))
    (Variables|/Game/Blueprints/Player/BP_FirstPersonPlayerController.BP_FirstPersonPlayerController_C|SetTeamIndex _value NewTeam)
    (CallFunction|CallChangeColorTeam)
    (bind _teammateref (Variables|/Game/Blueprints/Player/BP_FirstPersonCharacter.BP_FirstPersonCharacter_C|GetTeamMateRef Character)
      (:then
        (Variables|/Game/Blueprints/Player/BP_FirstPersonCharacter.BP_FirstPersonCharacter_C|SetTeamMateRef _teammateref 0))
      (:else
        _))
    (for _array_element _player
      (if (!= _array_element _value)
        (Variables|/Game/Blueprints/Player/BP_FirstPersonCharacter.BP_FirstPersonCharacter_C|SetTeamMateRef Character (Variables|/Game/Blueprints/Player/BP_FirstPersonPlayerController.BP_FirstPersonPlayerController_C|GetPlayerOwning _array_element))
        (Variables|/Game/Blueprints/Player/BP_FirstPersonCharacter.BP_FirstPersonCharacter_C|SetTeamMateRef (Variables|/Game/Blueprints/Player/BP_FirstPersonPlayerController.BP_FirstPersonPlayerController_C|GetPlayerOwning _array_element) Character)
        (Utilities|Array|Add _player _value)))))

(event Custom|CallChangeColorTeam
  (Utilities|FlowControl|Delay 1.0)
  (Networking|SwitchHasAuthority
    (:Authority
      (bind (_keypin _valuepin) (Utilities|Map|ForEachLoop(Map) (Variables|Default|GetPlayerAndController))
        (:then
          (Default|ChangeTeamMaterial _keypin (Variables|/Game/Blueprints/Player/BP_FirstPersonPlayerController.BP_FirstPersonPlayerController_C|GetTeamIndex _valuepin)))))))

(event Custom|CallRespawnTime
  (params (Time :type Float%20%28single-precision%29) (Position :type Transform) (Data :type Integer) (Player :type BP%20First%20Person%20Character%20Object%20Reference))
  (Default|CallRespawn Player Time Position Data)
  (Default|MaxHealthonRespawn Player))

(fn ConstructionScript)

(fn IsontheSameTeam?
  (params (Player1 :type BP%20First%20Person%20Character%20Object%20Reference) (Player2 :type BP%20First%20Person%20Character%20Object%20Reference))
  (return (== (Variables|/Game/Blueprints/Player/BP_FirstPersonPlayerController.BP_FirstPersonPlayerController_C|GetTeamIndex (.Value (Utilities|Map|Find (Variables|Default|GetPlayerAndController) Player1))) (Variables|/Game/Blueprints/Player/BP_FirstPersonPlayerController.BP_FirstPersonPlayerController_C|GetTeamIndex (.Value (Utilities|Map|Find (Variables|Default|GetPlayerAndController) Player2))))))