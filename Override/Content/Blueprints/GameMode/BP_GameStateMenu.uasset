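; Menu game state that keeps the multiplayer lobby's team and spectator slot labels in sync and relays play-button calls to tracked players.
; RPC_MulticastWidgetText and RPC_CleanOldPlace write or reset a slot's name through the local BP_ControllerMenu's lobby widget, only on the Remote authority branch.
; Test replays every assigned player's name and slot to one target via WidgetText.
; RPC_CallWidget triggers RPCPlayButton on each NewPlayer entry.
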(event Custom|RPC_CallWidget
  (for _array_element (Variables|Default|GetNew%20Player)
    (Default|RPCPlayButton _array_element)))

(event Custom|WidgetText
  (params (Controllers :type String) (Index :type Integer) (Player :type Integer) (Target :type BP%20Controller%20Menu%20Object%20Reference))
  (Default|RPCUpdateTextLobby Target Index Controllers Player))

(event Custom|RPC_CleanOldPlace
  (params (OldTeam :type Integer) (Index :type Integer))
  (bind _asbp_controller_menu (Utilities|Casting|CastToBP_ControllerMenu (Game|GetPlayerController 0)))
  (Networking|SwitchHasAuthority
    (:Remote
      (if (!= OldTeam -1)
        (Rendering|Components|TextRender|SetText (Utilities|Select :Index Index :Option%200 (Variables|/Game/Blueprints/Widget/Menu/WBP_UserBox.WBP_UserBox_C|GetPlayer1 (Utilities|Select :Index OldTeam :Option%200 (Variables|/Game/Blueprints/Widget/Menu/WBP_Lobby.WBP_Lobby_C|GetTeam1 (Variables|/Game/Blueprints/Widget/Menu/WBP_Menu.WBP_Menu_C|GetWBP_Lobby (Variables|/Game/Blueprints/Player/BP_ControllerMenu.BP_ControllerMenu_C|GetUI _asbp_controller_menu))) :Option%201 (Variables|/Game/Blueprints/Widget/Menu/WBP_Lobby.WBP_Lobby_C|GetTeam2 (Variables|/Game/Blueprints/Widget/Menu/WBP_Menu.WBP_Menu_C|GetWBP_Lobby (Variables|/Game/Blueprints/Player/BP_ControllerMenu.BP_ControllerMenu_C|GetUI _asbp_controller_menu))) :Option%202 (Variables|/Game/Blueprints/Widget/Menu/WBP_Lobby.WBP_Lobby_C|GetTeam3 (Variables|/Game/Blueprints/Widget/Menu/WBP_Menu.WBP_Menu_C|GetWBP_Lobby (Variables|/Game/Blueprints/Player/BP_ControllerMenu.BP_ControllerMenu_C|GetUI _asbp_controller_menu))) :Option%203 (Variables|/Game/Blueprints/Widget/Menu/WBP_Lobby.WBP_Lobby_C|GetSpec (Variables|/Game/Blueprints/Widget/Menu/WBP_Menu.WBP_Menu_C|GetWBP_Lobby (Variables|/Game/Blueprints/Player/BP_ControllerMenu.BP_ControllerMenu_C|GetUI _asbp_controller_menu))))) :Option%201 (Variables|/Game/Blueprints/Widget/Menu/WBP_UserBox.WBP_UserBox_C|GetPlayer2 (Utilities|Select :Index OldTeam :Option%200 (Variables|/Game/Blueprints/Widget/Menu/WBP_Lobby.WBP_Lobby_C|GetTeam1 (Variables|/Game/Blueprints/Widget/Menu/WBP_Menu.WBP_Menu_C|GetWBP_Lobby (Variables|/Game/Blueprints/Player/BP_ControllerMenu.BP_ControllerMenu_C|GetUI _asbp_controller_menu))) :Option%201 (Variables|/Game/Blueprints/Widget/Menu/WBP_Lobby.WBP_Lobby_C|GetTeam2 (Variables|/Game/Blueprints/Widget/Menu/WBP_Menu.WBP_Menu_C|GetWBP_Lobby (Variables|/Game/Blueprints/Player/BP_ControllerMenu.BP_ControllerMenu_C|GetUI _asbp_controller_menu))) :Option%202 (Variables|/Game/Blueprints/Widget/Menu/WBP_Lobby.WBP_Lobby_C|GetTeam3 (Variables|/Game/Blueprints/Widget/Menu/WBP_Menu.WBP_Menu_C|GetWBP_Lobby (Variables|/Game/Blueprints/Player/BP_ControllerMenu.BP_ControllerMenu_C|GetUI _asbp_controller_menu))) :Option%203 (Variables|/Game/Blueprints/Widget/Menu/WBP_Lobby.WBP_Lobby_C|GetSpec (Variables|/Game/Blueprints/Widget/Menu/WBP_Menu.WBP_Menu_C|GetWBP_Lobby (Variables|/Game/Blueprints/Player/BP_ControllerMenu.BP_ControllerMenu_C|GetUI _asbp_controller_menu)))))) "- ")))))

(event Custom|RPC_MulticastWidgetText
  (params (Controllers :type String) (Index :type Integer) (OldTeam :type Integer) (Player :type Integer))
  (bind _asbp_controller_menu (Utilities|Casting|CastToBP_ControllerMenu (Game|GetPlayerController 0)))
  (Networking|SwitchHasAuthority
    (:Remote
      (Rendering|Components|TextRender|SetText (Utilities|Select :Index Player :Option%200 (Variables|/Game/Blueprints/Widget/Menu/WBP_UserBox.WBP_UserBox_C|GetPlayer1 (Utilities|Select :Index Index :Option%200 (Variables|/Game/Blueprints/Widget/Menu/WBP_Lobby.WBP_Lobby_C|GetTeam1 (Variables|/Game/Blueprints/Widget/Menu/WBP_Menu.WBP_Menu_C|GetWBP_Lobby (Variables|/Game/Blueprints/Player/BP_ControllerMenu.BP_ControllerMenu_C|GetUI _asbp_controller_menu))) :Option%201 (Variables|/Game/Blueprints/Widget/Menu/WBP_Lobby.WBP_Lobby_C|GetTeam2 (Variables|/Game/Blueprints/Widget/Menu/WBP_Menu.WBP_Menu_C|GetWBP_Lobby (Variables|/Game/Blueprints/Player/BP_ControllerMenu.BP_ControllerMenu_C|GetUI _asbp_controller_menu))) :Option%202 (Variables|/Game/Blueprints/Widget/Menu/WBP_Lobby.WBP_Lobby_C|GetTeam3 (Variables|/Game/Blueprints/Widget/Menu/WBP_Menu.WBP_Menu_C|GetWBP_Lobby (Variables|/Game/Blueprints/Player/BP_ControllerMenu.BP_ControllerMenu_C|GetUI _asbp_controller_menu))) :Option%203 (Variables|/Game/Blueprints/Widget/Menu/WBP_Lobby.WBP_Lobby_C|GetSpec (Variables|/Game/Blueprints/Widget/Menu/WBP_Menu.WBP_Menu_C|GetWBP_Lobby (Variables|/Game/Blueprints/Player/BP_ControllerMenu.BP_ControllerMenu_C|GetUI _asbp_controller_menu))))) :Option%201 (Variables|/Game/Blueprints/Widget/Menu/WBP_UserBox.WBP_UserBox_C|GetPlayer2 (Utilities|Select :Index Index :Option%200 (Variables|/Game/Blueprints/Widget/Menu/WBP_Lobby.WBP_Lobby_C|GetTeam1 (Variables|/Game/Blueprints/Widget/Menu/WBP_Menu.WBP_Menu_C|GetWBP_Lobby (Variables|/Game/Blueprints/Player/BP_ControllerMenu.BP_ControllerMenu_C|GetUI _asbp_controller_menu))) :Option%201 (Variables|/Game/Blueprints/Widget/Menu/WBP_Lobby.WBP_Lobby_C|GetTeam2 (Variables|/Game/Blueprints/Widget/Menu/WBP_Menu.WBP_Menu_C|GetWBP_Lobby (Variables|/Game/Blueprints/Player/BP_ControllerMenu.BP_ControllerMenu_C|GetUI _asbp_controller_menu))) :Option%202 (Variables|/Game/Blueprints/Widget/Menu/WBP_Lobby.WBP_Lobby_C|GetTeam3 (Variables|/Game/Blueprints/Widget/Menu/WBP_Menu.WBP_Menu_C|GetWBP_Lobby (Variables|/Game/Blueprints/Player/BP_ControllerMenu.BP_ControllerMenu_C|GetUI _asbp_controller_menu))) :Option%203 (Variables|/Game/Blueprints/Widget/Menu/WBP_Lobby.WBP_Lobby_C|GetSpec (Variables|/Game/Blueprints/Widget/Menu/WBP_Menu.WBP_Menu_C|GetWBP_Lobby (Variables|/Game/Blueprints/Player/BP_ControllerMenu.BP_ControllerMenu_C|GetUI _asbp_controller_menu)))))) (Utilities|Text|ToText(String) (Utilities|String|Append "- " Controllers))))))

(event Custom|Test
  (params (Target :type BP%20Controller%20Menu%20Object%20Reference))
  (for _array_element (Variables|Default|GetNew%20Player)
    (if (!= (Variables|/Game/Blueprints/Player/BP_ControllerMenu.BP_ControllerMenu_C|GetSelectedTeam _array_element) -1)
      (CallFunction|WidgetText (Variables|/Game/Blueprints/Player/BP_FirstPersonPlayerController.BP_FirstPersonPlayerController_C|GetUserName _array_element) (Variables|/Game/Blueprints/Player/BP_ControllerMenu.BP_ControllerMenu_C|GetSelectedTeam _array_element) (Variables|/Game/Blueprints/Player/BP_ControllerMenu.BP_ControllerMenu_C|GetOldSlot _array_element) Target))))

(event EventBeginPlay)

(fn ConstructionScript)