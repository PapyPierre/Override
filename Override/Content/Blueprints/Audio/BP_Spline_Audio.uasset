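; BP_Spline_Audio is an actor that makes a water wall sound follow the player along a spline.
; It starts WaterWallSFX on BeginPlay, then each Tick moves it to the spline point closest to player pawn 0, so one emitter covers the spline's length.
; Tick also draws a debug sphere at that point and ends in a short Delay with nothing after it, which does not throttle the updates.
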(event EventBeginPlay
  (Class|FMODAudioComponent|Play (Variables|Default|GetWaterWallSFX)))

(event EventTick
  (params (DeltaSeconds :type Float%20%28single-precision%29))
  (bind _returnvalue (Game|Player|GetPlayerPawn 0))
  (bind _spline (Variables|Default|GetSpline))
  (bind _returnvalue_2 (Transformation|GetActorLocation _returnvalue))
  (bind _returnvalue_3 (Spline|FindLocationClosesttoWorldLocation _spline _returnvalue_2 "World"))
  (Rendering|Debug|DrawDebugSphere _returnvalue_3 1e+01 12 "(R=1.000000,G=1.000000,B=1.000000,A=1.000000)" 1.0)
  (Transformation|SetWorldLocation (Variables|Default|GetWaterWallSFX) _returnvalue_3 false false)
  (Utilities|FlowControl|Delay 0.05))

(fn ConstructionScript)