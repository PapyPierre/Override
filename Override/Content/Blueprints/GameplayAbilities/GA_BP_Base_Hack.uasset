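; Base gameplay ability for hacks, routing an activation to one of three empty hook events by what was targeted.
; After committing, it reads the event's target data: a first actor that is a player fires OnTargetPlayer; otherwise actors cast to BP_Modulation fire OnTargetModulation.
; With no targets, it draws a debug sphere at the effect context origin and calls OnFreePlacement there after a delay.
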(event Custom|OnFreePlacement
  (params (Point :type Vector)))

(event Custom|OnTargetPlayer
  (params (Player :type BP%20First%20Person%20Character%20Object%20Reference)))

(event Custom|OnTargetModulation
  (params (Modulations :type BP%20Modulation%20Object%20Reference%20%28by%20ref%29)))

(event Ability|EventActivateAbility
  (bind _returnvalue (Class|GABaseHack|GetEventData))
  (bind _freeplacementdelay (Variables|Default|GetFreePlacementDelay))
  (bind (_eventtag _instigator _target _optionalobject _optionalobject2 _contexthandle _instigatortags _targettags _eventmagnitude _targetdata) (Utilities|Struct|BreakGameplayEventData _returnvalue))
  (bind _returnvalue_2 (Class|AbilitySystemBlueprintLibrary|EffectContextGetOrigin _contexthandle))
  (bind _returnvalue_3 (Ability|TargetData|GetActorsfromTargetData _targetdata))
  (bind _returnvalue_4 (Ability|CommitAbility))
  (if _returnvalue_4
    (if (Utilities|Array|IsEmpty _returnvalue_3)
      (Rendering|Debug|DrawDebugSphere _returnvalue_2 1e+01 12 "(R=1.000000,G=1.000000,B=1.000000,A=1.000000)" _freeplacementdelay 1.0)
      (Utilities|FlowControl|Delay _freeplacementdelay)
      (CallFunction|OnFreePlacement _returnvalue_2)
      (else
        (bind _asbp_first_person_character (Utilities|Casting|CastToBP_FirstPersonCharacter (Utilities|Array|Get(acopy) _returnvalue_3))
          (:then
            (CallFunction|OnTargetPlayer _asbp_first_person_character))
          (:CastFailed
            (for _array_element _returnvalue_3
              (bind _asbp_modulation (Utilities|Casting|CastToBP_Modulation _array_element))
              (CallFunction|OnTargetModulation _asbp_modulation))))))
    (else
      (Ability|CancelAbility))))