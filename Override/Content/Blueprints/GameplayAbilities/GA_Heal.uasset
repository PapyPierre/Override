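; GA_Heal is a gameplay ability that heals through three targeting modes: free placement, modulation zone or single player.
; Free placement draws a debug sphere and, with authority, burst-heals overlapped characters except the caster's avatar.
; Modulation applies heal-over-time to players in its zone, then starts casting that effect on it for the applied duration.
; Player targeting applies a burst heal; effects target player states, and each mode ends the ability.
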(event EventOnFreePlacement
  (params (Point :type Vector :default "0, 0, 0"))
  (bind _free_placement_aoe_radius (Variables|Default|GetFree%20Placement%20Aoe%20Radius))
  (Rendering|Debug|DrawDebugSphere Point _free_placement_aoe_radius 24 "(R=0.017098,G=1.000000,B=0.288824,A=1.000000)" 1.0 3.0)
  (bind _outactors (Collision|SphereOverlapActors Point _free_placement_aoe_radius (Utilities|Array|MakeArray "ObjectTypeQuery7") 0 (Utilities|Array|MakeArray (Ability|GetAvatarActorfromActorInfo))))
  (for _array_element _outactors
    (Ability|HasAuthority
      (:True
        (bind _asbp_first_person_character (Utilities|Casting|CastToBP_FirstPersonCharacter _array_element))
        (GameplayEffects|ApplyGameplayEffectToTarget (Ability|TargetData|AbilityTargetDatafromActor (Class|PlayerCharacter|GetCustomPlayerState _asbp_first_person_character)) "/Game/Blueprints/GameplayEffects/GE_Health_HealBurst.GE_Health_HealBurst_C" 1 1))))
  (Ability|EndAbility))

(event EventOnTargetModulation
  (params (Modulations :type BP%20Modulation%20Object%20Reference%20%28by%20ref%29))
  (for _array_element (Variables|/Game/Blueprints/Interactable/BP_Modulation.BP_Modulation_C|GetPlayerInZone Modulations)
    (bind _returnvalue (GameplayEffects|ApplyGameplayEffectToTarget (Ability|TargetData|AbilityTargetDatafromActor (Class|PlayerCharacter|GetCustomPlayerState _array_element)) "/Game/Blueprints/GameplayEffects/GE_Health_HealOverTime.GE_Health_HealOverTime_C" 1 1)))
  (bind _returnvalue_2 (Class|AbilitySystemBlueprintLibrary|GetActiveGameplayEffectTotalDuration (Utilities|Array|Get(acopy) _returnvalue)))
  (Class|Modulation|StartCastingGE Modulations "/Game/Blueprints/GameplayEffects/GE_Health_HealOverTime.GE_Health_HealOverTime_C" _returnvalue_2)
  (Ability|EndAbility))

(event EventOnTargetPlayer
  (params (Player :type BP%20First%20Person%20Character%20Object%20Reference))
  (GameplayEffects|ApplyGameplayEffectToTarget (Ability|TargetData|AbilityTargetDatafromActor (Class|PlayerCharacter|GetCustomPlayerState Player)) "/Game/Blueprints/GameplayEffects/GE_Health_HealBurst.GE_Health_HealBurst_C" 1 1)
  (Ability|EndAbility))