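; GA_AoeBase is a base area-of-effect Gameplay Ability with an empty ApplyEffectsToTarget hook.
; Activation reads actors from the event's target data, commits per actor, and cancels if a commit fails.
; A debug-drawn sphere overlap around each actor gathers pawns, excluding the avatar unless CanTargetSelf is set.
; Authority passes each pawn to the hook, while non-authority ends the ability.
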(event Ability|EventActivateAbility
  (bind _radius (Variables|Default|GetRadius))
  (for _array_element (Ability|TargetData|GetActorsfromTargetData (.TargetData (Utilities|Struct|BreakGameplayEventData (Class|BaseHack|GetEventData))))
    (bind _returnvalue (Ability|CommitAbility))
    (if _returnvalue
      (Rendering|Debug|DrawDebugSphere (Transformation|GetActorLocation _array_element) _radius 12 "(R=1.000000,G=1.000000,B=1.000000,A=1.000000)" 1.0 1.0)
      (bind _outactors (Collision|SphereOverlapActors (Transformation|GetActorLocation _array_element) _radius (Utilities|Array|MakeArray "ObjectTypeQuery3") 0 (select (Variables|Default|GetCanTargetSelf) 0 (Utilities|Array|MakeArray (Ability|GetAvatarActorfromActorInfo)))))
      (for _array_element_2 _outactors
        (Ability|HasAuthority
          (:True
            (CallFunction|ApplyEffectstoTarget _array_element_2))
          (:False
            (Ability|EndAbility))))
      (else
        (Ability|CancelAbility)
        (Development|PrintString "Hello"))))
  (Ability|EndAbility))

(fn ApplyEffectstoTarget
  (params (Target%20Actor :type Actor%20Object%20Reference)))