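; Demat gameplay ability with three targeting modes: free placement, modulations and player.
; Free placement sphere-overlaps an area and applies a damage-over-time effect to characters on authority; modulations apply it to players in their zones.
; Player targeting changes the mesh collision type and disables shooting until AfterCooldown restores both.
; Effects target each character's player state, and EndAbility is called inside the area loops.
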(event Custom|AfterCooldown
  (bind _player (Variables|Default|GetPlayer))
  (Collision|SetCollisionObjectType (Variables|/Script/Engine.Character|GetMesh _player) "ECC_GameTraceChannel1")
  (Variables|/Game/Blueprints/Component/AC_Weapon.AC_Weapon_C|SetCanShoot (Variables|/Game/Blueprints/Player/BP_FirstPersonCharacter.BP_FirstPersonCharacter_C|GetAC_WeaponComponent _player) true)
  (Ability|EndAbility))

(event EventOnFreePlacement
  (params (Point :type Vector :default "0, 0, 0"))
  (bind _free_placement_aoe_radius (Variables|Default|GetFree%20Placement%20Aoe%20Radius))
  (Development|PrintString "Demat free placement")
  (Rendering|Debug|DrawDebugSphere Point _free_placement_aoe_radius 24 "(R=0.017098,G=1.000000,B=0.288824,A=1.000000)" 1.0 3.0)
  (bind _outactors (Collision|SphereOverlapActors Point _free_placement_aoe_radius (Utilities|Array|MakeArray "ObjectTypeQuery7") 0 (Utilities|Array|MakeArray (Ability|GetAvatarActorfromActorInfo))))
  (for _array_element _outactors
    (Ability|HasAuthority
      (:True
        (bind _asbp_first_person_character (Utilities|Casting|CastToBP_FirstPersonCharacter _array_element))
        (GameplayEffects|ApplyGameplayEffectToTarget (Ability|TargetData|AbilityTargetDatafromActor (Class|PlayerCharacter|GetCustomPlayerState _asbp_first_person_character)) "/Game/Blueprints/GameplayEffects/GE_Health_AoeDamageOverTime.GE_Health_AoeDamageOverTime_C" 1 1)
        (Ability|EndAbility))
      (:False
        (Ability|EndAbility))))
  (Ability|EndAbility))

(event EventOnTargetModulations
  (params (Modulations :type Array%20of%20Actor%20Object%20References))
  (for _array_element Modulations
    (bind _asbp_modulation (Utilities|Casting|CastToBP_Modulation _array_element))
    (for _array_element_2 (Variables|/Game/Blueprints/Interactable/BP_Modulation.BP_Modulation_C|GetPlayerInZone _asbp_modulation)
      (GameplayEffects|ApplyGameplayEffectToTarget (Ability|TargetData|AbilityTargetDatafromActor (Class|PlayerCharacter|GetCustomPlayerState _array_element_2)) "/Game/Blueprints/GameplayEffects/GE_Health_AoeDamageOverTime.GE_Health_AoeDamageOverTime_C" 1 1)
      (Ability|EndAbility))
    (Ability|EndAbility)))

(event EventOnTargetPlayer
  (params (Player :type BP%20First%20Person%20Character%20Object%20Reference))
  (Development|PrintString "Demat on player")
  (Collision|SetCollisionObjectType (Variables|/Script/Engine.Character|GetMesh Player) "ECC_Pawn")
  (Variables|/Game/Blueprints/Component/AC_Weapon.AC_Weapon_C|SetCanShoot (Variables|/Game/Blueprints/Player/BP_FirstPersonCharacter.BP_FirstPersonCharacter_C|GetAC_WeaponComponent Player) false)
  (Variables|Default|SetPlayer Player))