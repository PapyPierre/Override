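; Health pack pickup that heals an overlapping first-person character below max health through the Gameplay Ability System.
; It applies a SetByCaller heal effect via the player state's ability system component, then marks itself used and hides.
; Tick runs a cooldown that clears the used flag but does not unhide the actor.
; Ping temporarily outlines the sphere using custom depth stencil and a material parameter collection color.
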(event OnComponentBeginOverlap(Sphere)
  (params (OverlappedComponent :type Primitive%20Component%20Object%20Reference) (OtherActor :type Actor%20Object%20Reference) (OtherComp :type Primitive%20Component%20Object%20Reference) (OtherBodyIndex :type Integer) (bFromSweep :type Boolean) (SweepResult :type Hit%20Result%20Structure%20%28by%20ref%29))
  (bind _asbp_first_person_character (Utilities|Casting|CastToBP_FirstPersonCharacter OtherActor))
  (bind _returnvalue (Class|PlayerCharacter|GetCustomPlayerState _asbp_first_person_character))
  (bind _asc (Variables|/Script/Override.CustomPlayerState|GetAsc _returnvalue))
  (if (not (Variables|Default|GetUsed))
    (if (== "/Game/Blueprints/Player/BP_FirstPersonCharacter.BP_FirstPersonCharacter_C" (Utilities|GetClass OtherActor))
      (bind _asbp_custom_player_state (Utilities|Casting|CastToBP_CustomPlayerState (Variables|/Script/Engine.Pawn|GetPlayerState _asbp_first_person_character)))
      (bind _returnvalue_2 (GameplayAttributes|GetAttributeSet (Variables|/Script/Override.CustomPlayerState|GetAsc _asbp_custom_player_state) "/Script/Override.HealthAttributeSet"))
      (if (< (.currentvalue (Variables|/Script/Override.HealthAttributeSet|GetHealth _returnvalue_2)) (.currentvalue (Variables|/Script/Override.HealthAttributeSet|GetMaxHealth _returnvalue_2)))
        (bind _returnvalue_3 (Ability|GameplayEffect|AssignTagSetbyCallerMagnitude (GameplayEffects|MakeOutgoingSpec :self _asc :GameplayEffectClass "/Game/Blueprints/GAS/GameplayEffects/GE_Health_SetByCallerHeal.GE_Health_SetByCallerHeal_C" :Level 1.0) "(TagName=\"Data.Heal\")" (Variables|Default|GetHealth)))
        (GameplayEffects|ApplyGameplayEffectSpecToSelf _asc _returnvalue_3)
        (GameplayAttributes|GetAttributeSet _asc "/Script/Override.HealthAttributeSet")
        (Variables|Default|SetUsed true)
        (Rendering|SetActorHiddenInGame true)))))

(event Custom|CancelPing
  (bind _sphere (Variables|Default|GetSphere))
  (Rendering|SetRenderCustomDepth _sphere false)
  (Rendering|SetCustomDepthStencilValue _sphere 0))

(event EventStopPing
  (bind _sphere (Variables|Default|GetSphere))
  (Rendering|SetRenderCustomDepth _sphere false)
  (Rendering|SetCustomDepthStencilValue _sphere 0))

(event EventPing
  (params (LifeTime :type Float%20%28single-precision%29))
  (bind _sphere (Variables|Default|GetSphere))
  (Rendering|Material|SetVectorParameterValue "/Game/Art/Shader/Devs/PP_OutlineCollector.PP_OutlineCollector" "Color" (Math|Color|MakeColor 0.0 0.0 1.0) :!class /Script/Engine.KismetMaterialLibrary)
  (Rendering|SetRenderCustomDepth _sphere true)
  (Rendering|SetCustomDepthStencilValue _sphere 1)
  (Utilities|Time|SetTimerbyEvent (delegate Custom|CancelPing) LifeTime))

(event EventTick
  (params (DeltaSeconds :type Float%20%28single-precision%29))
  (if (Variables|Default|GetUsed)
    (bind _output_get (Variables|Default|SetCooldown (- (Variables|Default|GetCooldown) DeltaSeconds)))
    (if (<= _output_get 0.0)
      (Variables|Default|SetUsed false)
      (Variables|Default|SetCooldown (Variables|Default|GetInitialCooldown)))))

(event EventBeginPlay
  (Variables|Default|SetCooldown (Variables|Default|GetInitialCooldown)))

(fn ConstructionScript)

(fn OnRepUsed)